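; AI character that walks a path made of placed BP_PlaceableFlag actors and can die into a ragdoll.
; GetAIPathFlags gathers every flag in the level in returned order, then Move chains AI MoveTo calls, advancing the index on each success.
; The index has no wrap or bounds check, and failed moves are not handled.
; Death runs once, enabling mesh physics and disabling movement.
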(event Custom|GetAIPathFlags
  (bind _outactors (Actor|GetAllActorsOfClass "/Game/Tech/Blueprints/Placeables/BP_PlaceableFlag.BP_PlaceableFlag_C"))
  (for _array_element _outactors
    (Utilities|Array|Add (Variables|Default|GetPathFlags) _array_element))
  (CallFunction|Move))

(event Custom|Move
  (AI|AIMoveTo self "0, 0, 0" (Utilities|Array|Get(acopy) (Variables|Default|GetPathFlags) (Variables|Default|GetCurrentPoint)) 2e+01 false
    (:OnSuccess
      (Math|Integer|IncrementInt (Variables|Default|GetCurrentPoint)
        (:%20%20
          (CallFunction|Move))))))

(fn ConstructionScript)

(fn Death
  (if (not (Variables|Default|GetDead?))
    (Variables|Default|SetDead? true)
    (Physics|SetSimulatePhysics (Variables|Character|GetMesh) true)
    (Pawn|Components|CharacterMovement|DisableMovement (Variables|Character|GetCharacterMovement))))