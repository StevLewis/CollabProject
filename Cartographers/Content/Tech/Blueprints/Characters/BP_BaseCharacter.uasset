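; Base player character with camera-relative movement (inverted by SlimeOnHead), box-trace interaction, pushing, equipment cycling, help requests and flag placement.
; CanPerform gates most actions, while montages, delays and timers lock and release movement or action state.
; Damage triggers ragdoll death, hold-to-restart flickers the mesh material, and walking off ledges plays a cartoon hover before falling.
; Empty equipment hooks suggest child classes supply specifics, and the GameMode receives respawn and character-switch messages.
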(event EventOnWalkingOffLedge
  (params (PreviousFloorImpactNormal :type Vector%20%28by%20ref%29 :default "0, 0, 0") (PreviousFloorContactNormal :type Vector%20%28by%20ref%29 :default "0, 0, 0") (PreviousLocation :type Vector%20%28by%20ref%29 :default "0, 0, 0") (TimeDelta :type Float%20%28single-precision%29))
  ;[1 1 1] Special Fall
  (bind _floorhit_ (CallFunction|FloorTrace))
  (if (not _floorhit_)
    (if (not (Variables|Status|GetSpecialFalling?))
      (Pawn|Components|CharacterMovement|SetMovementMode (Variables|Character|GetCharacterMovement) "MOVE_Flying" 0)
      (Variables|Status|SetSpecialFalling? true)
      (Variables|Default|SetPerformingAction? true)
      (bind _returnvalue (Animation|PlayAnimMontage "/Game/Tech/Blueprints/Animation/Fall/AM_ToonFall.AM_ToonFall" 1.0 "None"))
      (Utilities|FlowControl|Delay 0.2)
      (Pawn|Components|CharacterMovement|DisableMovement (Variables|Character|GetCharacterMovement))
      (Utilities|FlowControl|Delay (* _returnvalue 0.8))
      (Pawn|Components|CharacterMovement|SetMovementMode (Variables|Character|GetCharacterMovement) "MOVE_Walking" 0)
      (Variables|Default|SetPerformingAction? false))))

(event Game|Damage|EventAnyDamage
  (params (Damage :type Float%20%28single-precision%29) (DamageType :type Damage%20Type%20Object%20Reference) (InstigatedBy :type Controller%20Object%20Reference) (DamageCauser :type Actor%20Object%20Reference))
  ;[1 1 1] Damage
  (if (not (Variables|Stats|Damage|GetCanTakeDamage?))
    (Stats|Death)))

(event EventTick
  (params (DeltaSeconds :type Float%20%28single-precision%29))
  ;[1 1 1] Event Tick
)

(event EventOnLanded
  (params (Hit :type Hit%20Result%20Structure%20%28by%20ref%29))
  ;[1 1 1] Special Fall
  (if (Variables|Status|GetSpecialFalling?)
    (Variables|Status|SetSpecialFalling? false)))

(event EventStopHold
  (bind _charactermovement (Variables|Character|GetCharacterMovement))
  (Variables|Default|SetIsPushing? false)
  (Variables|/Script/Engine.CharacterMovementComponent|SetMaxWalkSpeed _charactermovement (Variables|Stats|GetMoveSpeed))
  (Variables|/Script/Engine.CharacterMovementComponent|SetRotationRate _charactermovement (Variables|Default|GetPlayerRotationRate)))

(event EventHold
  (params (Held%20Object :type Actor%20Object%20Reference))
  (bind _returnvalue (Transformation|GetActorLocation))
  (bind _charactermovement (Variables|Character|GetCharacterMovement))
  (Variables|Default|SetIsPushing? true)
  (Variables|/Script/Engine.CharacterMovementComponent|SetMaxWalkSpeed _charactermovement (Variables|Default|GetPlayerPushingSpeed))
  (Variables|/Script/Engine.CharacterMovementComponent|SetRotationRate _charactermovement (Variables|Default|GetPlayerPushingRotation))
  (Transformation|SetActorRotation (Math|Conversions|RotationFromXVector (Math|Vector|MakeVector (.x _returnvalue) (.y _returnvalue) 0.0))))

(event EventInit
  ;[1 1 1] Init
  ;;[1 1 1] Save current material
  (Variables|Components|SetMeshMaterialRef (Utilities|Array|Get(acopy) (Rendering|Material|GetMaterials (Variables|Character|GetMesh))))
  (Stats|SeupStats)
  (bind _asbp_game_instance (Utilities|Casting|CastToBP_GameInstance (Game|GetGameInstance)))
  (Variables|Components|SetGameInstanceRef _asbp_game_instance))

(event Input|AxisEvents|InputAxisMoveForwardBack
  (params (AxisValue :type Float%20%28single-precision%29))
  ;[1 1 1] Movement
  (Pawn|Input|AddMovementInput (Math|Vector|GetForwardVector (Utilities|GetCameraRotation)) (select (Variables|Status|GetSlimeOnHead?) (* AxisValue -1.0) AxisValue) false))

(event Input|AxisEvents|InputAxisMoveRightLeft
  (params (AxisValue :type Float%20%28single-precision%29))
  ;[1 1 1] Movement
  (Pawn|Input|AddMovementInput (Math|Vector|GetRightVector (Utilities|GetCameraRotation)) (select (Variables|Status|GetSlimeOnHead?) (* AxisValue -1.0) AxisValue) false))

(event Custom|RetryEquipment
  ;[1 1 1] Equipment
)

(event Custom|Speak
  (params (SpeechType :type E_Speech%20Enum :default "NewEnumerator0"))
  ;[1 1 1] Speak
  (Class|BPIPopup|Speak(Message) (UserInterface|GetWidget (Variables|Default|GetSpeechWidget)) SpeechType))

(event Custom|UpdateEquipment
  ;[1 1 1] Equipment
  (bind _returnvalue (Animation|PlayAnimMontage "/Game/Tech/Blueprints/Animation/Actions/AM_Equip.AM_Equip" 1.0 "None"))
  (Variables|Default|SetPerformingAction? true)
  (Variables|Default|SetSwitchingEquipment? true)
  (Utilities|FlowControl|Delay _returnvalue)
  (Variables|Default|SetPerformingAction? false)
  (Variables|Default|SetSwitchingEquipment? false))

(event EventLevitatefor
  (params (LevitationTime :type Float%20%28single-precision%29))
  ;[1 1 1] Levitation
  (Physics|AddForce (Variables|Character|GetCharacterMovement) "0, 0,100.000000")
  (Variables|/Script/Engine.CharacterMovementComponent|SetGravityScale (Variables|Character|GetCharacterMovement) 0.0)
  (Utilities|FlowControl|Delay LevitationTime)
  (Variables|/Script/Engine.CharacterMovementComponent|SetGravityScale (Variables|Character|GetCharacterMovement) 1.0))

(event Input|ActionEvents|InputActionInteract
  (params (Key :type Key%20Structure :default "None"))
  ;[1 1 1] Interact
  (:Pressed
    (Actions|Interact|StartInteract)))

(event Input|ActionEvents|InputActionSwitchEquipment
  (params (Key :type Key%20Structure :default "None"))
  ;[1 1 1] Equipment
  (:Pressed
    (if (Checks|CanPerform?)
      (Actions|Equipment|SwitchEquipment))))

(event Input|ActionEvents|InputActionHelp
  (params (Key :type Key%20Structure :default "None"))
  ;[1 1 1] Help
  (:Pressed
    (Variables|Default|SetHelpHeldDown? true)
    (Actions|Help|StartAskingforHelp))
  (:Released
    (Variables|Default|SetHelpHeldDown? false)
    (if (Class|KismetSystemLibrary|TimerExistsHandle (Variables|Default|GetHelpTH))
      (Utilities|Time|SetTimerbyEvent (EventDispatchers|CreateEvent :!event StopAskingforHelp) (Utilities|Time|GetTimerRemainingTimebyHandle (Variables|Default|GetHelpTH))))))

(event Input|ActionEvents|InputActionRestart
  (params (Key :type Key%20Structure :default "None"))
  ;[1 1 1] Restart
  (:Pressed
    (Actions|Restart|StartRestarting))
  (:Released
    (Actions|Restart|StopRestarting)))

(event Input|KeyboardEvents|1
  (params (Key :type Key%20Structure :default "None"))
  ;[1 0 0] Debug
  (:Pressed
    (Class|BPISwitch|SwitchCharacters(Message) (Game|GetGameMode))))

(fn ConstructionScript)

(fn SeupStats
  (Variables|/Script/Engine.CharacterMovementComponent|SetMaxWalkSpeed (Variables|Character|GetCharacterMovement) (Variables|Stats|GetMoveSpeed))
  (Variables|Default|SetPlayerRotationRate (Variables|/Script/Engine.CharacterMovementComponent|GetRotationRate (Variables|Character|GetCharacterMovement))))

(fn Death
  (if (not (Variables|Stats|Damage|GetDead?))
    (Variables|Stats|Damage|SetDead? true)
    (Physics|SetSimulatePhysics (Variables|Character|GetMesh) true)
    (Pawn|Components|CharacterMovement|DisableMovement (Variables|Character|GetCharacterMovement))
    (Utilities|Time|SetTimerbyEvent (EventDispatchers|CreateEvent :!event Respawn) (Variables|Stats|Spawn|GetRespawnTime))))

(fn SetInvincible
  (params (InvicibilityDuration :type Float%20%28single-precision%29))
  (Utilities|Time|SetTimerbyEvent (EventDispatchers|CreateEvent :!event UnsetInvincible) InvicibilityDuration)
  (Variables|Stats|Damage|SetCanTakeDamage? true)
  (Variables|Components|SetMeshMaterialRef (Utilities|Array|Get(acopy) (Rendering|Material|GetMaterials (Variables|Character|GetMesh))))
  (bind _returnvalue (Utilities|Time|SetTimerbyEvent (EventDispatchers|CreateEvent :!event InvinciblityFlicker) 0.1 true))
  (Variables|Stats|Damage|SetInvincibilityFlickerTH _returnvalue))

(fn UnsetInvincible
  (Variables|Stats|Damage|SetCanTakeDamage? false)
  (Utilities|Time|ClearandInvalidateTimerbyHandle (Variables|Stats|Damage|GetInvincibilityFlickerTH))
  (Rendering|Material|SetMaterial (Variables|Character|GetMesh) 0 (Variables|Components|GetMeshMaterialRef)))

(fn InvinciblityFlicker
  (if (== (Utilities|Array|Get(acopy) (Rendering|Material|GetMaterials (Variables|Character|GetMesh))) (Variables|Components|GetMeshMaterialRef))
    (Rendering|Material|SetMaterial (Variables|Character|GetMesh) 0 "/Game/Tech/BasicMaterials/M_Grey.M_Grey")
    (else
      (Rendering|Material|SetMaterial (Variables|Character|GetMesh) 0 (Variables|Components|GetMeshMaterialRef)))))

(fn RestartFlicker
  (if (== (Utilities|Array|Get(acopy) (Rendering|Material|GetMaterials (Variables|Character|GetMesh))) (Variables|Components|GetMeshMaterialRef))
    (Rendering|Material|SetMaterial (Variables|Character|GetMesh) 0 "/Game/Tech/BasicMaterials/M_Green.M_Green")
    (else
      (Rendering|Material|SetMaterial (Variables|Character|GetMesh) 0 (Variables|Components|GetMeshMaterialRef)))))

(fn Respawn
  (Class|BPIRespawn|RespawnPlayers(Message) (Game|GetGameMode)))

(fn SetWalking
  (Pawn|Components|CharacterMovement|SetMovementMode (Variables|Character|GetCharacterMovement) "MOVE_Walking" 0))

(fn StartInteract
  (if (Checks|CanPerform?)
    (Class|BPIInteract|Interact(Message) (Actions|Interact|InteractBoxTrace 1e+02) self)
    (bind _returnvalue (Animation|PlayAnimMontage "/Game/Tech/Blueprints/Animation/Actions/AM_Push.AM_Push" 3.0 "None"))
    (Variables|Default|SetPerformingAction? true)
    (Pawn|Components|CharacterMovement|DisableMovement (Variables|Character|GetCharacterMovement))
    (Utilities|Time|SetTimerbyEvent (EventDispatchers|CreateEvent :!event StopInteract) (/ _returnvalue 3.0))))

(fn InteractBoxTrace
  (params (Range :type Float%20%28single-precision%29))
  (bind _returnvalue (Transformation|GetActorLocation))
  (LocalVariables|SetTempRange Range)
  (bind (_outhits _returnvalue_2) (Class|KismetSystemLibrary|BoxTraceMultiforObjects _returnvalue (+ _returnvalue (* (Transformation|GetActorForwardVector) (LocalVariables|GetTempRange))) "10.000000,10.000000,10.000000" "0, 0, 0" (Utilities|Array|MakeArray "ObjectTypeQuery1" "ObjectTypeQuery2" "ObjectTypeQuery3" "ObjectTypeQuery4" "ObjectTypeQuery5" "ObjectTypeQuery6") false (Utilities|Array|MakeArray self) "None" true))
  (if _returnvalue_2
    (bind _array_element (Utilities|Array|ForEachLoopwithBreak _outhits :!label _label)
      (:LoopBody
        (if (Utilities|DoesObjectImplementInterface (.HitActor (Collision|BreakHitResult _array_element)) "/Game/Tech/Blueprints/Characters/BPI_Interact.BPI_Interact_C")
          (LocalVariables|SetTempInteractable (.HitActor (Collision|BreakHitResult _array_element)))
          (goto _label Break)))
      (:Completed
        (return (LocalVariables|GetTempInteractable))))
    (else
      (return 0))))

(fn StartRestarting
  (if (not (Variables|Stats|Damage|GetDead?))
    (Variables|Actions|Restart|SetRestarting? true)
    (bind _returnvalue (Utilities|Time|SetTimerbyEvent (EventDispatchers|CreateEvent :!event RestartFlicker) 0.1 true))
    (Variables|Default|SetRestartFlickerTH _returnvalue)
    (bind _returnvalue_2 (Utilities|Time|SetTimerbyEvent (EventDispatchers|CreateEvent :!event Respawn) (Variables|Stats|Spawn|GetRespawnTime)))
    (Variables|Actions|Restart|SetRestartingTH _returnvalue_2)))

(fn StopRestarting
  (if (Variables|Actions|Restart|GetRestarting?)
    (Variables|Actions|Restart|SetRestarting? false)
    (Utilities|Time|ClearandInvalidateTimerbyHandle (Variables|Actions|Restart|GetRestartingTH))
    (Utilities|Time|ClearandInvalidateTimerbyHandle (Variables|Default|GetRestartFlickerTH))
    (Rendering|Material|SetMaterial (Variables|Character|GetMesh) 0 (Variables|Components|GetMeshMaterialRef))))

(fn InitHelpWidget
  (if (Variables|Default|GetHelpHeldDown?)
    (Class|BPIInit|Init(Message) (UserInterface|GetWidget (Variables|Default|GetHelpWidget)))
    (Default|CallCalledforHelp)))

(fn StartAskingforHelp
  (if (Checks|CanPerform?)
    (if (not (Class|KismetSystemLibrary|TimerExistsHandle (Variables|Default|GetHelpTH)))
      (Variables|Default|SetPerformingAction? true)
      (Variables|Actions|Help|SetRequestingHelp? true)
      (Pawn|Components|CharacterMovement|DisableMovement (Variables|Character|GetCharacterMovement))
      (Actions|Help|InitHelpWidget)
      (bind _returnvalue (Utilities|Time|SetTimerbyEvent (EventDispatchers|CreateEvent :!event InitHelpWidget) 1.0 true))
      (Variables|Default|SetHelpTH _returnvalue))))

(fn StopAskingforHelp
  (if (Variables|Actions|Help|GetRequestingHelp?)
    (Variables|Default|SetPerformingAction? false)
    (Variables|Actions|Help|SetRequestingHelp? false)
    (Utilities|Time|ClearandInvalidateTimerbyHandle (Variables|Default|GetHelpTH))
    (CallFunction|SetWalking)))

(fn SwitchEquipment
  (bind _result (Math|Integer|IncrementInt (Variables|Equipment|GetEquipmentIndex))
    (:%20%20
      (if (> _result (Variables|Equipment|GetMaxEquipment))
        (Variables|Equipment|SetEquipmentIndex 1))
      (CallFunction|UpdateEquipment))))

(fn SkipEquipment
  (bind _result (Math|Integer|IncrementInt (Variables|Equipment|GetEquipmentIndex))
    (:%20%20
      (if (> _result (Variables|Equipment|GetMaxEquipment))
        (Variables|Equipment|SetEquipmentIndex 1))
      (CallFunction|RetryEquipment))))

(fn Grounded?
  (return (and (not (AI|Components|NavMovement|IsFalling (Variables|Character|GetCharacterMovement))) (not (Class|NavMovementComponent|IsFlying (Variables|Character|GetCharacterMovement))))))

(fn CanPerform?
  (return (Math|Boolean|ANDBoolean (Checks|Grounded?) (not (Variables|Default|GetPerformingAction?)) (not (Variables|Stats|Damage|GetDead?)))))

(fn StartPlacingFlag
  (bind _returnvalue (Animation|PlayAnimMontage "/Game/Tech/Blueprints/Animation/Actions/AM_PlaceFlag.AM_PlaceFlag" 2.0 "None"))
  (Variables|Default|SetPerformingAction? true)
  (Pawn|Components|CharacterMovement|DisableMovement (Variables|Character|GetCharacterMovement))
  (Utilities|Time|SetTimerbyEvent (EventDispatchers|CreateEvent :!event SpawnFlag) (* (/ _returnvalue 2.0) 0.5))
  (Utilities|Time|SetTimerbyEvent (EventDispatchers|CreateEvent :!event FinishPlacingFlag) (/ _returnvalue 2.0)))

(fn FinishPlacingFlag
  (Variables|Default|SetPerformingAction? false)
  (CallFunction|SetWalking)
  (Rendering|SetVisibility (Variables|Default|GetFlagMesh) true true))

(fn SpawnFlag
  (bind _mesh (Variables|Character|GetMesh))
  (bind _mesh_2 (Variables|Character|GetMesh))
  (bind _returnvalue (Transformation|GetSocketLocation _mesh "hand_r"))
  (bind _returnvalue_2 (Transformation|GetSocketLocation _mesh_2 "hand_r"))
  (bind (_outhit _returnvalue_3) (Collision|LineTraceByChannel (Math|Vector|MakeVector (.x _returnvalue_2) (.y _returnvalue_2) (.z _returnvalue_2)) (Math|Vector|MakeVector (.x _returnvalue_2) (.y _returnvalue_2) (- (.z (- (Transformation|GetActorLocation) (Math|Vector|MakeVector 0.0 0.0 (Components|Capsule|GetScaledCapsuleHalfHeight (Variables|Collision|GetCapsuleComponent))))) 1e+01)) "TraceTypeQuery1" false (Utilities|Array|MakeArray self) "None"))
  (if _returnvalue_3
    (if (not (== "/Game/Tech/Blueprints/Placeables/Traps/BP_BaseTrap.BP_BaseTrap_C" (Utilities|GetClass (.HitActor (Collision|BreakHitResult _outhit)))))
      (bind (_outhits _returnvalue_4) (Collision|MultiSphereTraceForObjects (.Location (Collision|BreakHitResult _outhit)) (.Location (Collision|BreakHitResult _outhit)) 2e+02 (Utilities|Array|MakeArray "ObjectTypeQuery1" "ObjectTypeQuery2" "ObjectTypeQuery3" "ObjectTypeQuery4" "ObjectTypeQuery5" "ObjectTypeQuery6") false (Utilities|Array|MakeArray self) "None"))
      (if _returnvalue_4
        (bind _array_element (Utilities|Array|ForEachLoopwithBreak _outhits :!label _label)
          (:LoopBody
            (if (or (== "/Game/Tech/Blueprints/Placeables/BP_PlaceableFlag.BP_PlaceableFlag_C" (Utilities|GetClass (.HitActor (Collision|BreakHitResult _array_element)))) (Utilities|ClassIsChildOf (Utilities|GetClass (.HitActor (Collision|BreakHitResult _array_element))) "/Game/Tech/Blueprints/Placeables/Traps/BP_BaseTrap.BP_BaseTrap_C"))
              (LocalVariables|SetCanPlace? false)
              (goto _label Break)))
          (:Completed
            (if (LocalVariables|GetCanPlace?)
              (Game|SpawnActorfromClass "/Game/Tech/Blueprints/Placeables/BP_PlaceableFlag.BP_PlaceableFlag_C" (Math|Transform|MakeTransform (Math|Vector|MakeVector (.x _returnvalue) (.y _returnvalue) (.z (- (Transformation|GetActorLocation) (Math|Vector|MakeVector 0.0 0.0 (Components|Capsule|GetScaledCapsuleHalfHeight (Variables|Collision|GetCapsuleComponent)))))) "0, 0, 0" "1.250000,1.250000,1.250000") "Undefined" 0 0)
              (CallFunction|HideAllEquipment)
              (else
                (CallFunction|Speak "NewEnumerator3"))))))
      (else
        (CallFunction|Speak "NewEnumerator3")))
    (else
      (CallFunction|Speak "NewEnumerator3"))))

(fn HideAllEquipment)

(fn StopInteract
  (Variables|Default|SetPerformingAction? false)
  (CallFunction|SetWalking))

(fn FloorTrace
  (bind _returnvalue (Transformation|GetActorLocation))
  (bind _capsulecomponent (Variables|Collision|GetCapsuleComponent))
  (bind _returnvalue_2 (Components|Capsule|GetScaledCapsuleHalfHeight _capsulecomponent))
  (bind _returnvalue_3 (- _returnvalue (Math|Vector|MakeVector 0.0 0.0 _returnvalue_2)))
  (bind _returnvalue_4 (Class|KismetSystemLibrary|CapsuleTraceMultiforObjects _returnvalue_3 _returnvalue_3 75.0 1e+02 (Utilities|Array|MakeArray "ObjectTypeQuery1" "ObjectTypeQuery2") false (Utilities|Array|MakeArray self) "None" true))
  (return _returnvalue_4))