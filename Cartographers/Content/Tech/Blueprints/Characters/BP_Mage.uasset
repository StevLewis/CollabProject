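; Mage player character, a child character Blueprint with four equipment slots: flag, staff, spell book and sleeping powder.
; Equipment updates show only the selected mesh, and the Action input starts the matching use.
; Staff, book and powder only play a montage and lock movement, with a montage-length timer and Finish functions that restore walking.
; An unwired tap-or-hold invincibility ability, for self or nearby characters, remains in the event graph.
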(event Custom|UseActionOnOther)

(event Custom|UpdateEquipment
  ;[1 1 1] Equipment
  (|CallParentFunction)
  (CallFunction|HideAllEquipment)
  (switch int (Variables|Default|GetEquipmentIndex)
    (:1
      (Rendering|SetVisibility (Variables|Default|GetFlagMesh) true true))
    (:2
      (Rendering|SetVisibility (Variables|Default|GetStaffMesh) true true))
    (:3
      (Rendering|SetVisibility (Variables|Default|GetSpellBookMesh) true true))
    (:4
      (Rendering|SetVisibility (Variables|Default|GetSleepingPowderMesh) true true))))

(event Custom|ActionCooldown
  (Variables|Default|SetActionOnCooldown? false)
  (Development|PrintString "Ability off cooldown"))

(event EventInit
  ;[1 1 1] Init
  (|CallParentFunction)
  (Variables|Default|SetMaxEquipment 4)
  (CallFunction|UpdateEquipment))

(event Input|ActionEvents|InputActionAction
  (params (Key :type Key%20Structure :default "None"))
  ;[1 1 1] Mage Actions
  (:Pressed
    (if (CallFunction|CanPerform?)
      (switch int (Variables|Default|GetEquipmentIndex)
        (:1
          (CallFunction|StartPlacingFlag))
        (:2
          (Actions|Staff|StartUsingStaff))
        (:3
          (Actions|Book|StartUsingBook))
        (:4
          (Actions|Powder|StartUsingPowder))))))

(fn ConstructionScript
  (|CallParentFunction))

(fn StartUsingStaff
  (bind _returnvalue (Animation|PlayAnimMontage "/Game/Tech/Blueprints/Animation/Actions/Mage/AM_StaffCast.AM_StaffCast" 1.0 "None"))
  (Variables|Default|SetPerformingAction? true)
  (Pawn|Components|CharacterMovement|DisableMovement (Variables|Character|GetCharacterMovement))
  (Utilities|Time|SetTimerbyEvent (EventDispatchers|CreateEvent :!event FinishUsingStaff) _returnvalue))

(fn FinishUsingStaff
  (Variables|Default|SetPerformingAction? false)
  (CallFunction|SetWalking))

(fn StartUsingBook
  (bind _returnvalue (Animation|PlayAnimMontage "/Game/Tech/Blueprints/Animation/Actions/Mage/AM_BookCast.AM_BookCast" 1.0 "None"))
  (Variables|Default|SetPerformingAction? true)
  (Pawn|Components|CharacterMovement|DisableMovement (Variables|Character|GetCharacterMovement))
  (Utilities|Time|SetTimerbyEvent (EventDispatchers|CreateEvent :!event FinishUsingStaff) _returnvalue))

(fn FinishUsingBook
  (Variables|Default|SetPerformingAction? false)
  (CallFunction|SetWalking))

(fn StartUsingPowder
  (bind _returnvalue (Animation|PlayAnimMontage "/Game/Tech/Blueprints/Animation/Actions/AM_throw.AM_Throw" 1.0 "None"))
  (Variables|Default|SetPerformingAction? true)
  (Pawn|Components|CharacterMovement|DisableMovement (Variables|Character|GetCharacterMovement))
  (Utilities|Time|SetTimerbyEvent (EventDispatchers|CreateEvent :!event FinishUsingPowder) _returnvalue))

(fn FinishUsingPowder
  (Variables|Default|SetPerformingAction? false)
  (CallFunction|SetWalking))

(fn HideAllEquipment
  (|CallParentFunction)
  (Rendering|SetVisibility (Variables|Default|GetStaffMesh) false true))