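; Player controller that handles pause menu toggling and a hold-to-fast-forward key.
; The Pause action lazily creates and caches WB_PauseMenu, then adds or removes it based on whether the game is paused.
; Each toggle also sets the paused state, switches input mode between game-only and game-and-UI, and updates cursor visibility.
; Holding Left Shift raises global time dilation to speed up the game, restoring normal speed on release.
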(event Input|ActionEvents|InputActionPause
  (params (Key :type Key%20Structure :default "None"))
  (bind _returnvalue (Game|GetPlayerController 0))
  (bind _returnvalue_2 (Game|GetPlayerController 0))
  ;[1 1 1] Pause
  (:Pressed
    (Utilities|IsValid (Variables|Default|GetPauseMenuRef)
      (:Is%20Valid
        _)
      (:Is%20Not%20Valid
        (bind _returnvalue_3 (UserInterface|CreateWidget "/Game/Tech/Blueprints/UI/WB_PauseMenu.WB_PauseMenu_C"))
        (Variables|Default|SetPauseMenuRef _returnvalue_3)))
    (if (Game|IsGamePaused)
      (Widget|RemovefromParent (Variables|Default|GetPauseMenuRef))
      (Game|SetGamePaused false)
      (Input|SetInputModeGameOnly _returnvalue_2)
      (Variables|/Script/Engine.PlayerController|SetbShowMouseCursor _returnvalue_2 false)
      (else
        (UserInterface|Viewport|AddtoViewport (Variables|Default|GetPauseMenuRef) 0)
        (Game|SetGamePaused true)
        (Input|SetInputModeGameandUI _returnvalue (Variables|Default|GetPauseMenuRef) "LockInFullscreen" false)
        (Variables|/Script/Engine.PlayerController|SetbShowMouseCursor _returnvalue true)))))

(event Input|KeyboardEvents|LeftShift
  (params (Key :type Key%20Structure :default "None"))
  (:Pressed
    (Utilities|Time|SetGlobalTimeDilation 5.0))
  (:Released
    (Utilities|Time|SetGlobalTimeDilation 1.0)))

(fn ConstructionScript)