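; BP_Scout is the Scout character, whose Action input performs a forward stick poke that can set off triggerable objects such as traps.
; A press plays the poke montage and immediately runs a multi-object box trace ahead, sending TriggerMessage to hit actors implementing BPI_Trigger.
; An ActionInUse flag blocks repeat presses until a delay matching the montage length ends.
; Debug prints and trace drawing are enabled.
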(event Input|ActionEvents|InputActionAction
  (params (Key :type Key%20Structure :default "None"))
  (bind _returnvalue (Transformation|GetActorLocation))
  (:Pressed
    (if (not (Variables|Default|GetActionInUse?))
      (Variables|Default|SetActionInUse? true)
      (Utilities|FlowControl|Sequence
        (:then_0
          (bind _returnvalue_2 (Animation|PlayAnimMontage "/Game/Tech/Blueprints/Animation/Floor_Trap_Poke_0_Anim_Montage.Floor_Trap_Poke_0_Anim_Montage" 1.0 "None"))
          (Utilities|FlowControl|Delay _returnvalue_2)
          (Variables|Default|SetActionInUse? false))
        (:then_1
          (Development|PrintString "stick poke")
          (bind (_outhits _returnvalue_3) (Class|KismetSystemLibrary|BoxTraceMultiforObjects _returnvalue (+ _returnvalue (* (Transformation|GetActorForwardVector) 2e+02)) "0.000000,50.000000,100.000000" "0, 0, 0" (Utilities|Array|MakeArray "ObjectTypeQuery1" "ObjectTypeQuery2" "ObjectTypeQuery3" "ObjectTypeQuery4" "ObjectTypeQuery5" "ObjectTypeQuery6") false (Utilities|Array|MakeArray self) "ForDuration" true))
          (if _returnvalue_3
            (bind _array_element (Utilities|Array|ForEachLoopwithBreak _outhits)
              (:LoopBody
                (if (Utilities|DoesObjectImplementInterface (.HitActor (Collision|BreakHitResult _array_element)) "/Game/Tech/Blueprints/Placeables/Triggers/BPI_Trigger.BPI_Trigger_C")
                  (Class|BPITrigger|Trigger(Message) (.HitActor (Collision|BreakHitResult _array_element)))))))))
      (else
        (Development|PrintString "action un use")))))

(fn ConstructionScript
  (|CallParentFunction))