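; Game mode for two-player local co-op levels with a switchable Mage and Scout, followed by an AI adventurer party run.
; Setup creates both local players, HUDs and a timer, reads GameInstance level data, finds spawn and goal actors, then walks characters in.
; The end scene returns characters to their AI controllers, drops player two and spawns randomly classed, named adventurers.
; It also handles respawns and score display.
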(event Custom|Setup
  ;[1 1 1] Setup
  (Setup|GetGameInstance)
  (Setup|SetupControllers)
  (Setup|SetupUI)
  (CallFunction|StartTimer)
  (Setup|GetSpawnPoints)
  (Setup|SetupCharacters)
  (Setup|SetupGoals)
  (Setup|SetupAISpawnPoint)
  (Setup|GetChests))

(event Custom|StartTimer
  ;[1 1 1] Timer
  (bind _returnvalue (Utilities|Time|SetTimerbyEvent (EventDispatchers|CreateEvent :!event UpdateTimer) 1.0 true))
  (Variables|Timer|SetTimerTH _returnvalue))

(event Custom|SpawnAIParty
  ;[1 1 1] AI
  (Variables|AI|SetTempAdventurerNames (Variables|AI|GetAdventurerNames))
  (for _index (range 0 (- (Variables|AI|GetAdventurePartyNumber) 1))
    (CallFunction|SpawnAICharacter _index))
  (for _array_element (Variables|AI|GetAICharacters)
    (EventDispatchers|BindEventtoOnDeath _array_element (EventDispatchers|CreateEvent :!event RemoveDeadAdventurer)))
  (Game|Player|SetViewTargetwithBlend (Variables|Player1|GetPlayer1Controller) (Utilities|Array|Get(acopy) (Variables|AI|GetAICharacters)) 5.0 "VTBlend_Linear" 0.0 false)
  (EventDispatchers|BindEventtoBossRoomReached (Utilities|Array|Get(acopy) (Variables|AI|GetAICharacters)) (EventDispatchers|CreateEvent :!event ShowScore))
  (Utilities|FlowControl|Delay 5.0)
  (for _array_element_2 (Variables|AI|GetAICharacters)
    (Default|Move _array_element_2)))

(event EventBeginPlay
  ;[1 1 1] Event Begin Play
  (CallFunction|Setup))

(event EventSwitchCharacters
  ;[1 1 1] Switch Characters
  (CallFunction|CharacterSwitch))

(event EventActivateEndStairs
  ;[1 1 1] Goal
  (Default|ActivateTrigger (Variables|Goal|GetEndStairsRef)))

(event EventSetupEndScene
  ;[1 1 1] AI
  (Default|QuickFade (Variables|Player1|GetPlayer1MainHudRef))
  (Utilities|FlowControl|Delay 0.2)
  (Pawn|Possess (Variables|Player1|GetPlayer1AIController) (Variables|Player1|GetPlayer1CharacterRef))
  (Pawn|Possess (Variables|Player2|GetPlayer2AIController) (Variables|Player2|GetPlayer2CharacterRef))
  (Utilities|FlowControl|Delay 0.1)
  (Game|Player|SetViewTargetwithBlend (Variables|Player1|GetPlayer1Controller) (Variables|Player1|GetPlayer1CharacterRef) 0.0 "VTBlend_Linear" 0.0 false)
  (Game|Player|SetViewTargetwithBlend (Variables|Player2|GetPlayer2Controller) (Variables|Player2|GetPlayer2CharacterRef) 0.0 "VTBlend_Linear" 0.0 false)
  (Default|Moveto (Variables|Player1|GetPlayer1CharacterRef) (Transformation|GetWorldLocation (Variables|/Game/Tech/Blueprints/Placeables/Goal/BP_EndStairs.BP_EndStairs_C|GetEndPoint (Variables|Goal|GetEndStairsRef))))
  (Default|Moveto (Variables|Player2|GetPlayer2CharacterRef) (Transformation|GetWorldLocation (Variables|/Game/Tech/Blueprints/Placeables/Goal/BP_EndStairs.BP_EndStairs_C|GetEndPoint (Variables|Goal|GetEndStairsRef))))
  (Utilities|FlowControl|Delay 1.0)
  (Default|QuickFade (Variables|Player1|GetPlayer1MainHudRef))
  (Utilities|FlowControl|Delay 0.2)
  (Class|GameplayStatics|RemovePlayer (Variables|Player2|GetPlayer2Controller) false)
  (Input|SetInputModeUIOnly (Variables|Player1|GetPlayer1Controller) 0 "DoNotLock")
  (CallFunction|SpawnAIParty))

(event EventRespawnPlayers
  ;[1 1 1] Respawn
  (Actor|DestroyActor (Variables|Player1|GetPlayer1CharacterRef))
  (CallFunction|SpawnCharacter (Variables|Player1|GetPlayer1Controller) "NewEnumerator1")
  (Actor|DestroyActor (Variables|Player2|GetPlayer2CharacterRef))
  (CallFunction|SpawnCharacter (Variables|Player2|GetPlayer2Controller) "NewEnumerator0"))

(event EventSetSpawnPoints
  (params (MageSpawnPoint :type Transform) (ScoutSpawnPoint :type Transform))
  ;[1 1 1] Set Spawn Points
  (Variables|Respawn|SetMageSpawnPoint MageSpawnPoint)
  (Variables|Respawn|SetScoutSpawnPoint ScoutSpawnPoint))

(event EventOnLogout
  (params (ExitingController :type Controller%20Object%20Reference))
  ;[1 1 1] Controller Login and Logout, stores spawned controllers
  (if (== ExitingController (Variables|Player1|GetPlayer1Controller))
    (Variables|Player1|SetPlayer1Controller 0)
    (elif (== ExitingController (Variables|Player2|GetPlayer2Controller))
      (Variables|Player2|SetPlayer2Controller 0))))

(event EventPostLogin
  (params (NewPlayer :type Player%20Controller%20Object%20Reference))
  ;[1 1 1] Controller Login and Logout, stores spawned controllers
  (Input|SetInputModeGameOnly NewPlayer)
  (Utilities|IsValid (Variables|Player1|GetPlayer1Controller)
    (:Is%20Valid
      (Utilities|IsValid (Variables|Player2|GetPlayer2Controller)
        (:Is%20Valid
          (Class|GameplayStatics|RemovePlayer NewPlayer false))
        (:Is%20Not%20Valid
          (Variables|Player2|SetPlayer2Controller NewPlayer))))
    (:Is%20Not%20Valid
      (Variables|Player1|SetPlayer1Controller NewPlayer))))

(fn ConstructionScript)

(fn GetSpawnPoints
  (bind _outactors (Actor|GetAllActorsOfClass "/Game/Tech/Blueprints/Placeables/BP_SpawnPoint.BP_SpawnPoint_C"))
  (LocalVariables|SetSpawnPoints _outactors)
  (Utilities|FlowControl|Sequence
    (:then_0
      ;[1 1 1] Get Mage SpawnPoint
      (bind _array_element (Utilities|Array|ForEachLoopwithBreak (LocalVariables|GetSpawnPoints) :!label _label)
        (:LoopBody
          (if (Utilities|Enum|Equal(Enum) (Variables|/Game/Tech/Blueprints/Placeables/BP_SpawnPoint.BP_SpawnPoint_C|GetCharacter _array_element) "NewEnumerator1")
            (Variables|Respawn|SetMageSpawnPoint (Transformation|GetWorldTransform (Variables|/Game/Tech/Blueprints/Placeables/BP_SpawnPoint.BP_SpawnPoint_C|GetSpawnPoint _array_element)))
            (Variables|Respawn|SetMageMovePoint (Transformation|GetWorldLocation (Variables|/Game/Tech/Blueprints/Placeables/BP_SpawnPoint.BP_SpawnPoint_C|GetStartSpawnPoint _array_element)))
            (Utilities|Array|RemoveItem (LocalVariables|GetSpawnPoints) _array_element)
            (goto _label Break)))))
    (:then_1
      ;[1 1 1] Get Scout SpawnPoint
      (bind _array_element_2 (Utilities|Array|ForEachLoopwithBreak (LocalVariables|GetSpawnPoints) :!label _label_2)
        (:LoopBody
          (if (Utilities|Enum|Equal(Enum) (Variables|/Game/Tech/Blueprints/Placeables/BP_SpawnPoint.BP_SpawnPoint_C|GetCharacter _array_element_2) "NewEnumerator0")
            (Variables|Respawn|SetScoutSpawnPoint (Transformation|GetWorldTransform (Variables|/Game/Tech/Blueprints/Placeables/BP_SpawnPoint.BP_SpawnPoint_C|GetSpawnPoint _array_element_2)))
            (Variables|Respawn|SetScoutMovePoint (Transformation|GetWorldLocation (Variables|/Game/Tech/Blueprints/Placeables/BP_SpawnPoint.BP_SpawnPoint_C|GetStartSpawnPoint _array_element_2)))
            (Utilities|Array|RemoveItem (LocalVariables|GetSpawnPoints) _array_element_2)
            (goto _label_2 Break)))))))

(fn GetGameInstance
  (bind _asbp_game_instance (Utilities|Casting|CastToBP_GameInstance (Game|GetGameInstance)))
  (bind _output_get (Variables|Default|SetGameInstanceRef _asbp_game_instance))
  (bind (_player1character _player2character) (Default|GetCharacters _output_get))
  (Variables|Player1|SetPlayer1Character _player1character)
  (Variables|Player2|SetPlayer2Character _player2character)
  (bind (_adventurepartynumber _leveldifficulty _levelflagpar) (Default|GetLevelDetails (Variables|Default|GetGameInstanceRef)))
  (Variables|AI|SetAdventurePartyNumber _adventurepartynumber)
  (Variables|Default|SetLevelDifficulty _leveldifficulty)
  (Variables|Default|SetLevelFlagPar _levelflagpar))

(fn SetupControllers
  ;[1 1 1] Get initial auto spawned controller and remove it
  (Class|GameplayStatics|RemovePlayer (Game|GetPlayerController -1) false)
  ;[1 1 1] Spawn new controller based on the one in class defaults, -1 to find next free controller index
  (Class|GameplayStatics|CreatePlayer -1)
  (Class|GameplayStatics|CreatePlayer -1))

(fn SetupUI
  (Utilities|FlowControl|Sequence
    (:then_0
      (bind _returnvalue (UserInterface|CreateWidget "/Game/Tech/Blueprints/UI/WB_MainHud.WB_MainHud_C" (Variables|Player1|GetPlayer1Controller)))
      (bind _output_get (Variables|Player1|SetPlayer1MainHudRef _returnvalue))
      (UserInterface|Viewport|AddtoPlayerScreen _output_get)
      (Default|Init _output_get "NewEnumerator1"))
    (:then_1
      (bind _returnvalue_2 (UserInterface|CreateWidget "/Game/Tech/Blueprints/UI/WB_MainHud.WB_MainHud_C" (Variables|Player2|GetPlayer2Controller)))
      (bind _output_get_2 (Variables|Player2|SetPlayer2MainHudRef _returnvalue_2))
      (UserInterface|Viewport|AddtoPlayerScreen _output_get_2)
      (Default|Init _output_get_2 "NewEnumerator0"))))

(fn SpawnCharacter
  (params (Controller :type Controller%20Object%20Reference) (Player :type E_Player%20Enum :default "NewEnumerator1"))
  (switch Utilities|FlowControl|Switch|SwitchonE_Player Player
    (:NewEnumerator1
      (bind _characterref (CallFunction|SpawnPlayerCharacter (Variables|Player1|GetPlayer1Character)))
      (bind _output_get (Variables|Player1|SetPlayer1CharacterRef _characterref))
      (Variables|Player1|SetPlayer1AIController (Pawn|GetController _characterref))
      (Pawn|Possess Controller _output_get)
      (Class|BPIInit|Init(Message) (Variables|Player1|GetPlayer1CharacterRef)))
    (:NewEnumerator0
      (bind _characterref_2 (CallFunction|SpawnPlayerCharacter (Variables|Player2|GetPlayer2Character)))
      (bind _output_get_2 (Variables|Player2|SetPlayer2CharacterRef _characterref_2))
      (Variables|Player2|SetPlayer2AIController (Pawn|GetController _characterref_2))
      (Pawn|Possess Controller _output_get_2)
      (Class|BPIInit|Init(Message) (Variables|Player2|GetPlayer2CharacterRef)))))

(fn UpdateTimer
  (Variables|Timer|SetTimerTimespan (Math|Timespan|MakeTimespan (.Days (Math|Timespan|BreakTimespan (Variables|Timer|GetTimerTimespan))) (.Hours (Math|Timespan|BreakTimespan (Variables|Timer|GetTimerTimespan))) (.Minutes (Math|Timespan|BreakTimespan (Variables|Timer|GetTimerTimespan))) (+ (.Seconds (Math|Timespan|BreakTimespan (Variables|Timer|GetTimerTimespan))) 1) (.Milliseconds (Math|Timespan|BreakTimespan (Variables|Timer|GetTimerTimespan)))))
  (Default|CallTimerModified))

(fn SetupCharacters
  (Setup|SpawnandMoveCharacter (Variables|Player1|GetPlayer1Controller) (Variables|Player1|GetPlayer1Character))
  (Setup|SpawnandMoveCharacter (Variables|Player2|GetPlayer2Controller) (Variables|Player2|GetPlayer2Character)))

(fn SpawnandMoveCharacter
  (params (Controller :type Player%20Controller%20Object%20Reference) (Character :type E_Characters%20Enum :default "NewEnumerator1"))
  (switch Utilities|FlowControl|Switch|SwitchonE_Characters Character
    (:NewEnumerator1
      (bind _returnvalue (Game|SpawnActorfromClass "/Game/Tech/Blueprints/Characters/BP_Mage.BP_Mage_C" (Variables|Respawn|GetMageSpawnPoint) "AdjustIfPossibleButAlwaysSpawn" 0 0))
      (Variables|Player1|SetPlayer1CharacterRef _returnvalue)
      (Variables|Player1|SetPlayer1AIController (Pawn|GetController _returnvalue))
      (Class|BPIInit|Init(Message) (Variables|Player1|GetPlayer1CharacterRef))
      (Game|Player|SetViewTargetwithBlend Controller (Variables|Player1|GetPlayer1CharacterRef) 0.0 "VTBlend_Linear" 0.0 false)
      (Default|Moveto (Variables|Player1|GetPlayer1CharacterRef) (Variables|Respawn|GetMageMovePoint) Controller)
      (Variables|Respawn|SetMageSpawnPoint (Math|Transform|MakeTransform (Variables|Respawn|GetMageMovePoint) (.rotation (Variables|Respawn|GetMageSpawnPoint)) (.scale (Variables|Respawn|GetMageSpawnPoint)))))
    (:NewEnumerator0
      (bind _returnvalue_2 (Game|SpawnActorfromClass "/Game/Tech/Blueprints/Characters/BP_Scout.BP_Scout_C" (Variables|Respawn|GetScoutSpawnPoint) "AdjustIfPossibleButAlwaysSpawn" 0 0))
      (Variables|Player2|SetPlayer2CharacterRef _returnvalue_2)
      (Variables|Player2|SetPlayer2AIController (Pawn|GetController _returnvalue_2))
      (Class|BPIInit|Init(Message) (Variables|Player2|GetPlayer2CharacterRef))
      (Game|Player|SetViewTargetwithBlend Controller (Variables|Player2|GetPlayer2CharacterRef) 0.0 "VTBlend_Linear" 0.0 false)
      (Default|Moveto (Variables|Player2|GetPlayer2CharacterRef) (Variables|Respawn|GetScoutMovePoint) Controller)
      (Variables|Respawn|SetScoutSpawnPoint (Math|Transform|MakeTransform (Variables|Respawn|GetScoutMovePoint) (.rotation (Variables|Respawn|GetScoutSpawnPoint)) (.scale (Variables|Respawn|GetScoutSpawnPoint)))))))

(fn CharacterSwitch
  (LocalVariables|SetTempCharacterRef (Variables|Player1|GetPlayer1CharacterRef))
  (LocalVariables|SetTempCharacter (Variables|Player1|GetPlayer1Character))
  (Utilities|FlowControl|Sequence
    (:then_0
      (Pawn|Possess (Variables|Player1|GetPlayer1Controller) (Variables|Player2|GetPlayer2CharacterRef))
      (Variables|Player1|SetPlayer1Character (Variables|Player2|GetPlayer2Character))
      (Variables|Player1|SetPlayer1CharacterRef (Variables|Player2|GetPlayer2CharacterRef)))
    (:then_1
      (Pawn|Possess (Variables|Player2|GetPlayer2Controller) (LocalVariables|GetTempCharacterRef))
      (Variables|Player2|SetPlayer2Character (LocalVariables|GetTempCharacter))
      (Variables|Player2|SetPlayer2CharacterRef (LocalVariables|GetTempCharacterRef)))))

(fn SetupGoals
  (bind _outactors (Actor|GetAllActorsOfClass "/Game/Tech/Blueprints/Placeables/Goal/BP_BossDoor.BP_BossDoor_C"))
  (Utilities|IsValid (Utilities|Array|Get(acopy) _outactors)
    (:Is%20Valid
      (Variables|Goal|SetBossDoorRef (Utilities|Array|Get(acopy) _outactors)))
    (:Is%20Not%20Valid
      _))
  (bind _outactors_2 (Actor|GetAllActorsOfClass "/Game/Tech/Blueprints/Placeables/Goal/BP_EndStairs.BP_EndStairs_C"))
  (Utilities|IsValid (Utilities|Array|Get(acopy) _outactors_2)
    (:Is%20Valid
      (bind _output_get (Variables|Goal|SetEndStairsRef (Utilities|Array|Get(acopy) _outactors_2)))
      (Variables|Goal|SetNextLevelName (Variables|/Game/Tech/Blueprints/Placeables/Goal/BP_EndStairs.BP_EndStairs_C|GetLevelName _output_get)))))

(fn SetupAISpawnPoint
  (bind _outactors (Actor|GetAllActorsOfClass "/Game/Tech/Blueprints/AI/BP_AISpawnPoint.BP_AISpawnPoint_C"))
  (Utilities|IsValid (Utilities|Array|Get(acopy) _outactors)
    (:Is%20Valid
      (Variables|AI|SetAISpawnPoint (Transformation|GetWorldTransform (Variables|/Game/Tech/Blueprints/AI/BP_AISpawnPoint.BP_AISpawnPoint_C|GetSpawnPoint (Utilities|Array|Get(acopy) _outactors)))))))

(fn SpawnPlayerCharacter
  (params (Character :type E_Characters%20Enum :default "NewEnumerator1"))
  (switch Utilities|FlowControl|Switch|SwitchonE_Characters Character
    (:NewEnumerator1
      (bind _returnvalue (Game|SpawnActorfromClass "/Game/Tech/Blueprints/Characters/BP_Mage.BP_Mage_C" (Variables|Respawn|GetMageSpawnPoint) "AdjustIfPossibleButAlwaysSpawn" 0 0))
      (return _returnvalue))
    (:NewEnumerator0
      (bind _returnvalue_2 (Game|SpawnActorfromClass "/Game/Tech/Blueprints/Characters/BP_Scout.BP_Scout_C" (Variables|Respawn|GetScoutSpawnPoint) "AdjustIfPossibleButAlwaysSpawn" 0 0))
      (return _returnvalue_2))))

(fn SpawnAICharacter
  (params (CurrentAdventurer :type Integer))
  (bind _aispawnpoint (Variables|AI|GetAISpawnPoint))
  (bind _location (Math|Transform|BreakTransform _aispawnpoint))
  (bind (_x _y _z) (Math|Vector|BreakVector _location))
  (bind _returnvalue (Game|SpawnActorfromClass (Utilities|Select :Index (Math|Random|RandomIntegerinRange 0 2) :Option%200 "/Game/Tech/Blueprints/AI/BP_AIKnight.BP_AIKnight_C" :Option%201 "/Game/Tech/Blueprints/AI/BP_AICleric.BP_AICleric_C" :Option%202 "/Game/Tech/Blueprints/AI/BP_AIArcher.BP_AIArcher_C") (Variables|AI|GetAISpawnPoint) "Undefined" 0 0))
  (Utilities|Array|Add (Variables|AI|GetAICharacters) (.AsBP%20AICharacter (Utilities|Casting|CastToBP_AICharacter _returnvalue)))
  (bind _output_get (Variables|/Game/Tech/Blueprints/AI/BP_AICharacter.BP_AICharacter_C|SetName (.AsBP%20AICharacter (Utilities|Casting|CastToBP_AICharacter _returnvalue)) (.OutItem (Utilities|Array|Random (Variables|AI|GetTempAdventurerNames)))))
  (Utilities|Array|RemoveItem (Variables|AI|GetTempAdventurerNames) _output_get)
  (Class|BPIInit|Init(Message) _returnvalue)
  (Default|Moveto (.AsBP%20AICharacter (Utilities|Casting|CastToBP_AICharacter _returnvalue)) (Math|Vector|MakeVector (+ _x (* CurrentAdventurer 1e+02)) _y _z))
  (Default|GetAIPathFlags (.AsBP%20AICharacter (Utilities|Casting|CastToBP_AICharacter _returnvalue)) (Variables|Goal|GetBossDoorRef)))

(fn ShowScore
  (bind _returnvalue (UserInterface|CreateWidget "/Game/Tech/Blueprints/UI/WB_ScoreMenu.WB_ScoreMenu_C" (Variables|Player1|GetPlayer1Controller)))
  (Default|Init _returnvalue (Variables|AI|GetAdventurePartyNumber) (Utilities|Array|Length (Variables|AI|GetAICharacters)) (Variables|Default|GetLevelDifficulty) (Variables|Default|GetLevelFlagPar) (+ (Variables|/Game/Tech/Blueprints/Characters/BP_BaseCharacter.BP_BaseCharacter_C|GetFlagCount (Variables|Player1|GetPlayer1CharacterRef)) (Variables|/Game/Tech/Blueprints/Characters/BP_BaseCharacter.BP_BaseCharacter_C|GetFlagCount (Variables|Player2|GetPlayer2CharacterRef))))
  (UserInterface|Viewport|AddtoViewport _returnvalue 0)
  (Variables|/Script/Engine.PlayerController|SetbShowMouseCursor (Variables|Player1|GetPlayer1Controller) true))

(fn RemoveDeadAdventurer
  (params (SelfRef :type BP%20AI%20Character%20Object%20Reference))
  (Utilities|Array|RemoveItem (Variables|AI|GetAICharacters) SelfRef))

(fn GetChests)