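; Game mode for local two-player gameplay, with each player controlling a Mage or Scout as chosen in the game instance.
; On BeginPlay it recreates both player controllers, adds per-player HUDs, starts a looping timer, then spawns and possesses characters at matching BP_SpawnPoints.
; PostLogin and OnLogout track the two controllers, removing any extra player.
; It also stores updatable respawn locations, respawns both players together, and can swap their possessed pawns.
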(event Custom|Setup
  ;[1 1 1] Setup
  (Setup|GetGameInstance)
  (Setup|SetupControllers)
  (Setup|SetupUI)
  (CallFunction|StartTimer)
  (Setup|GetSpawnPoints)
  (Setup|SetupCharacters)
  (CallFunction|SetRespawnPoints (Transformation|GetActorLocation (Variables|Setup|GetMageSpawnPoint)) (Transformation|GetActorLocation (Variables|Setup|GetScoutSpawnPoint))))

(event Custom|StartTimer
  ;[1 1 1] Timer
  (bind _returnvalue (Utilities|Time|SetTimerbyEvent (EventDispatchers|CreateEvent :!event UpdateTimer) 1.0 true))
  (Variables|Timer|SetTimerTH _returnvalue))

(event EventBeginPlay
  ;[1 1 1] Event Begin Play
  (CallFunction|Setup))

(event EventSwitchCharacters
  (CallFunction|CharacterSwitch))

(event EventSetRespawnPoints
  (params (MageLocation :type Vector :default "0, 0, 0") (ScoutLocation :type Vector :default "0, 0, 0"))
  (Variables|Respawn|SetMageRespawnLocation MageLocation)
  (Variables|Respawn|SetScoutRespawnLocation ScoutLocation))

(event EventOnLogout
  (params (ExitingController :type Controller%20Object%20Reference))
  ;[1 1 1] Controller Login and Logout, stores spawned controllers
  (if (== ExitingController (Variables|Default|GetPlayer1Controller))
    (Variables|Default|SetPlayer1Controller 0)
    (elif (== ExitingController (Variables|Default|GetPlayer2Controller))
      (Variables|Default|SetPlayer2Controller 0))))

(event EventPostLogin
  (params (NewPlayer :type Player%20Controller%20Object%20Reference))
  ;[1 1 1] Controller Login and Logout, stores spawned controllers
  (Utilities|IsValid (Variables|Default|GetPlayer1Controller)
    (:Is%20Valid
      (Utilities|IsValid (Variables|Default|GetPlayer2Controller)
        (:Is%20Valid
          (Class|GameplayStatics|RemovePlayer NewPlayer false))
        (:Is%20Not%20Valid
          (Variables|Default|SetPlayer2Controller NewPlayer))))
    (:Is%20Not%20Valid
      (Variables|Default|SetPlayer1Controller NewPlayer))))

(fn ConstructionScript)

(fn GetSpawnPoints
  (bind _outactors (Actor|GetAllActorsOfClass "/Game/Tech/Blueprints/Placeables/BP_SpawnPoint.BP_SpawnPoint_C"))
  (LocalVariables|SetSpawnPoints _outactors)
  (Utilities|FlowControl|Sequence
    (:then_0
      ;[1 1 1] Get Mage SpawnPoint
      (bind _array_element (Utilities|Array|ForEachLoopwithBreak (LocalVariables|GetSpawnPoints) :!label _label)
        (:LoopBody
          (if (Utilities|Enum|Equal(Enum) (Variables|/Game/Tech/Blueprints/Placeables/BP_SpawnPoint.BP_SpawnPoint_C|GetCharacter _array_element) "NewEnumerator1")
            (Variables|Setup|SetMageSpawnPoint _array_element)
            (Utilities|Array|RemoveItem (LocalVariables|GetSpawnPoints) _array_element)
            (goto _label Break)))))
    (:then_1
      ;[1 1 1] Get Scout SpawnPoint
      (bind _array_element_2 (Utilities|Array|ForEachLoopwithBreak (LocalVariables|GetSpawnPoints) :!label _label_2)
        (:LoopBody
          (if (Utilities|Enum|Equal(Enum) (Variables|/Game/Tech/Blueprints/Placeables/BP_SpawnPoint.BP_SpawnPoint_C|GetCharacter _array_element_2) "NewEnumerator0")
            (Variables|Setup|SetScoutSpawnPoint _array_element_2)
            (Utilities|Array|RemoveItem (LocalVariables|GetSpawnPoints) _array_element_2)
            (goto _label_2 Break)))))
    (:then_2
      ;[1 0 0] Debug Check
      (Utilities|IsValid (Variables|Setup|GetMageSpawnPoint)
        (:Is%20Valid
          _)
        (:Is%20Not%20Valid
          (Development|PrintString "No valid spawn point for mage" true true "(R=0.000000,G=0.026397,B=1.000000,A=1.000000)")))
      (Utilities|IsValid (Variables|Setup|GetScoutSpawnPoint)
        (:Is%20Not%20Valid
          (Development|PrintString "No valid spawn point for scout" true true "(R=1.000000,G=0.047707,B=0.000000,A=1.000000)"))))))

(fn GetGameInstance
  (bind _asbp_game_instance (Utilities|Casting|CastToBP_GameInstance (Game|GetGameInstance)))
  (bind _output_get (Variables|Default|SetGameInstanceRef _asbp_game_instance))
  (Variables|Default|SetPlayer1Character (Variables|/Game/Tech/Blueprints/BP_GameInstance.BP_GameInstance_C|GetPlayer1Character _output_get))
  (Variables|Default|SetPlayer2Character (Variables|/Game/Tech/Blueprints/BP_GameInstance.BP_GameInstance_C|GetPlayer2Character _output_get)))

(fn SetupControllers
  ;[1 1 1] Get initial auto spawned controller and remove it
  (Class|GameplayStatics|RemovePlayer (Game|GetPlayerController 0) false)
  ;[1 1 1] Spawn new controller based on the one in class defaults, -1 to find next free controller index
  (Class|GameplayStatics|CreatePlayer -1)
  (Class|GameplayStatics|CreatePlayer -1))

(fn SetupUI
  (Utilities|FlowControl|Sequence
    (:then_0
      (bind _returnvalue (UserInterface|CreateWidget "/Game/Tech/Blueprints/UI/WB_MainHud.WB_MainHud_C" (Variables|Default|GetPlayer1Controller)))
      (Variables|Default|SetPlayer1MainHudRef _returnvalue)
      (UserInterface|Viewport|AddtoPlayerScreen _returnvalue)
      (Class|BPIInit|Init(Message) _returnvalue))
    (:then_1
      (bind _returnvalue_2 (UserInterface|CreateWidget "/Game/Tech/Blueprints/UI/WB_MainHud.WB_MainHud_C" (Variables|Default|GetPlayer2Controller)))
      (Variables|Default|SetPlayer2MainHudRef _returnvalue_2)
      (UserInterface|Viewport|AddtoPlayerScreen _returnvalue_2)
      (Class|BPIInit|Init(Message) _returnvalue_2))))

(fn UpdateTimer
  (Variables|Timer|SetTimerTimespawn (Math|Timespan|MakeTimespan (.Days (Math|Timespan|BreakTimespan (Variables|Timer|GetTimerTimespawn))) (.Hours (Math|Timespan|BreakTimespan (Variables|Timer|GetTimerTimespawn))) (.Minutes (Math|Timespan|BreakTimespan (Variables|Timer|GetTimerTimespawn))) (+ (.Seconds (Math|Timespan|BreakTimespan (Variables|Timer|GetTimerTimespawn))) 1) (.Milliseconds (Math|Timespan|BreakTimespan (Variables|Timer|GetTimerTimespawn)))))
  (Default|CallTimerModified))

(fn SetupCharacters
  (Setup|SpawnCharacter (Variables|Default|GetPlayer1Controller) (Variables|Default|GetPlayer1Character))
  (Setup|SpawnCharacter (Variables|Default|GetPlayer2Controller) (Variables|Default|GetPlayer2Character)))

(fn SpawnCharacter
  (params (Controller :type Controller%20Object%20Reference) (Character :type E_Characters%20Enum :default "NewEnumerator1"))
  (switch Utilities|FlowControl|Switch|SwitchonE_Characters Character
    (:NewEnumerator1
      (bind _returnvalue (Game|SpawnActorfromClass "/Game/Tech/Blueprints/Characters/BP_Mage.BP_Mage_C" (Math|Transform|MakeTransform (Transformation|GetWorldLocation (Variables|/Game/Tech/Blueprints/Placeables/BP_SpawnPoint.BP_SpawnPoint_C|GetSpawnPoint (Variables|Setup|GetMageSpawnPoint))) "0, 0, 0" "1,1,1") "AdjustIfPossibleButAlwaysSpawn" 0 0))
      (Pawn|Possess Controller _returnvalue)
      (Class|BPIInit|Init(Message) _returnvalue))
    (:NewEnumerator0
      (bind _returnvalue_2 (Game|SpawnActorfromClass "/Game/Tech/Blueprints/Characters/BP_Scout.BP_Scout_C" (Math|Transform|MakeTransform (Transformation|GetWorldLocation (Variables|/Game/Tech/Blueprints/Placeables/BP_SpawnPoint.BP_SpawnPoint_C|GetSpawnPoint (Variables|Setup|GetScoutSpawnPoint))) "0, 0, 0" "1,1,1") "AdjustIfPossibleButAlwaysSpawn" 0 0))
      (Pawn|Possess Controller _returnvalue_2)
      (Class|BPIInit|Init(Message) _returnvalue_2))))

(fn RespawnCharacter
  (params (Controller :type Controller%20Object%20Reference) (Character :type E_Characters%20Enum :default "NewEnumerator1"))
  (switch Utilities|FlowControl|Switch|SwitchonE_Characters Character
    (:NewEnumerator1
      (bind _returnvalue (Game|SpawnActorfromClass "/Game/Tech/Blueprints/Characters/BP_Mage.BP_Mage_C" (Math|Transform|MakeTransform (Variables|Respawn|GetMageRespawnLocation) "0, 0, 0" "1,1,1") "AdjustIfPossibleButAlwaysSpawn" 0 0))
      (Pawn|Possess Controller _returnvalue)
      (Class|BPIInit|Init(Message) _returnvalue))
    (:NewEnumerator0
      (bind _returnvalue_2 (Game|SpawnActorfromClass "/Game/Tech/Blueprints/Characters/BP_Scout.BP_Scout_C" (Math|Transform|MakeTransform (Variables|Respawn|GetScoutRespawnLocation) "0, 0, 0" "1,1,1") "AdjustIfPossibleButAlwaysSpawn" 0 0))
      (Pawn|Possess Controller _returnvalue_2)
      (Class|BPIInit|Init(Message) _returnvalue_2))))

(fn CharacterSwitch
  (bind _player1controller (Variables|Default|GetPlayer1Controller))
  (LocalVariables|SetTempPawnRef (Pawn|GetControlledPawn _player1controller))
  (Pawn|Possess _player1controller (Pawn|GetControlledPawn (Variables|Default|GetPlayer2Controller)))
  (Pawn|Possess (Variables|Default|GetPlayer2Controller) (LocalVariables|GetTempPawnRef)))

(fn RespawnPlayers
  (bind _player2controller (Variables|Default|GetPlayer2Controller))
  (bind _player1controller (Variables|Default|GetPlayer1Controller))
  (Actor|DestroyActor (Pawn|GetControlledPawn _player1controller))
  (Setup|RespawnCharacter _player1controller (Variables|Default|GetPlayer1Character))
  (Actor|DestroyActor (Pawn|GetControlledPawn _player2controller))
  (Setup|RespawnCharacter _player2controller (Variables|Default|GetPlayer2Character))
  (return true))