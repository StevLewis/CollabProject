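; BP_BossDoor is an interactable sliding double door that, when used, opens and triggers the boss-area AI and camera change.
; Interact calls the parent logic, then OpenDoor, whose timeline lerps two pivots outward to left and right targets.
; It also calls GetAIPathFlags on every AI character.
; Every player controller's view target switches to the first spectate camera found in the level.
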(event Custom|OpenDoor
  ;[1 1 1] Moves the left and right door outwards away from each other
  (bind _movement (Timeline|DoorOpen PlayFromStart)
    (:Update
      (Transformation|SetRelativeLocation (Variables|Default|GetPivot1) (Math|Vector|Lerp(Vector) "0, 0, 0" (Math|Vector|MakeVector (Variables|Default|GetDoorTargetLeft) 0.0 0.0) _movement) false false)
      (Transformation|SetRelativeLocation (Variables|Default|GetPivot2) (Math|Vector|Lerp(Vector) "0, 0, 0" (Math|Vector|MakeVector (Variables|Default|GetDoorTargetRight) 0.0 0.0) _movement) false false))))

(event EventInteract
  (params (Interacting :type Actor%20Object%20Reference))
  (|CallParentFunction Interacting)
  (CallFunction|OpenDoor)
  (Development|PrintString "Boss door trgger ai")
  (bind _outactors (Actor|GetAllActorsOfClass "/Game/Tech/Blueprints/AI/BP_AICharacter.BP_AICharacter_C"))
  (for _array_element _outactors
    (Default|GetAIPathFlags _array_element))
  (bind _outactors_2 (Actor|GetAllActorsOfClass "/Game/Tech/Blueprints/BP_SpectateCamera.BP_SpectateCamera_C"))
  (bind _outactors_3 (Actor|GetAllActorsOfClass "/Game/Tech/Blueprints/Characters/BP_PlayerController.BP_PlayerController_C"))
  (for _array_element_2 _outactors_3
    (Game|Player|SetViewTargetwithBlend _array_element_2 (Utilities|Array|Get(acopy) _outactors_2) 0.0 "VTBlend_Linear" 0.0 false)))

(fn ConstructionScript
  (|CallParentFunction))