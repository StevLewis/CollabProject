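; BP_Checkpoint is a placeable trigger that updates respawn points when a player character enters it.
; Its construction script sizes the box from an editable Size variable.
; On overlap by a BP_BaseCharacter, it passes the world locations of its separate MageSpawn and ScoutSpawn components to the cached BP_GameplayGamemode through SetRespawnPointsMessage.
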(event OnComponentBeginOverlap(Box)
  (params (OverlappedComponent :type Primitive%20Component%20Object%20Reference) (OtherActor :type Actor%20Object%20Reference) (OtherComp :type Primitive%20Component%20Object%20Reference) (OtherBodyIndex :type Integer) (bFromSweep :type Boolean) (SweepResult :type Hit%20Result%20Structure%20%28by%20ref%29))
  (Utilities|Casting|CastToBP_BaseCharacter OtherActor)
  (Class|BPIRespawn|SetRespawnPoints(Message) (Variables|Default|GetGamemodeRef) (Transformation|GetWorldLocation (Variables|Default|GetMageSpawn)) (Transformation|GetWorldLocation (Variables|Default|GetScoutSpawn))))

(event EventBeginPlay
  (bind _asbp_gameplay_gamemode (Utilities|Casting|CastToBP_GameplayGamemode (Game|GetGameMode)))
  (Variables|Default|SetGamemodeRef _asbp_gameplay_gamemode))

(fn ConstructionScript
  (Components|Box|SetBoxExtent (Variables|Default|GetBox) (Variables|Default|GetSize) true))