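; BP_NextLevelStairs is a placeable stairs interactable that ends the current level and loads the next.
; On Interact, it calls GetAIPathFlags on every AI character, then switches each player controller's view to a randomly picked AI character.
; It also starts a 30-second delay, after which it opens the level named by LevelName.
; An unconnected branch that would view through a BP_SpectateCamera never runs.
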(event EventInteract
  (params (Interacting :type Actor%20Object%20Reference))
  (Utilities|FlowControl|Sequence
    (:then_0
      (bind _outactors (Actor|GetAllActorsOfClass "/Game/Tech/Blueprints/AI/BP_AICharacter.BP_AICharacter_C"))
      (for _array_element _outactors
        (Default|GetAIPathFlags _array_element))
      (bind _outactors_2 (Actor|GetAllActorsOfClass "/Game/Tech/Blueprints/Characters/BP_PlayerController.BP_PlayerController_C"))
      (for _array_element_2 _outactors_2
        (Game|Player|SetViewTargetwithBlend _array_element_2 (Utilities|Array|Get(acopy) _outactors (Math|Random|RandomIntegerinRange 0 (Utilities|Array|LastIndex _outactors))) 0.0 "VTBlend_Linear" 0.0 false)))
    (:then_1
      (Utilities|FlowControl|Delay 3e+01)
      (Game|OpenLevel(byName) (Variables|Default|GetLevelName)))))

(fn ConstructionScript
  (|CallParentFunction))