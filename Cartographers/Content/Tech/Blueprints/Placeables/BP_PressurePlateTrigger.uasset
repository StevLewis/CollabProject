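; A placeable pressure plate that triggers a referenced trap when an actor overlaps its box and untriggers it once the box is empty.
; Overlapping actors are tracked in an array, and an optional linked plate must also be empty before the trap untriggers.
; A timeline lowers and raises the plate mesh, switching it to green when down and blue when up.
; Debug strings print on overlap and untrigger.
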(event OnComponentBeginOverlap(Box)
  (params (OverlappedComponent :type Primitive%20Component%20Object%20Reference) (OtherActor :type Actor%20Object%20Reference) (OtherComp :type Primitive%20Component%20Object%20Reference) (OtherBodyIndex :type Integer) (bFromSweep :type Boolean) (SweepResult :type Hit%20Result%20Structure%20%28by%20ref%29))
  (bind _pressureplate (Variables|Default|GetPressurePlate))
  (if (not (Variables|Default|GetTriggered?))
    (Class|BPITrigger|Trigger(Message) (Variables|Default|GetTrapRef))
    (Variables|Default|SetTriggered? true))
  (Utilities|Array|Add (Variables|Default|GetOverlappedActors) OtherActor)
  (Development|PrintString "Hello")
  (Variables|Default|SetPlateDown? true)
  (bind _newtrack_0 (Timeline|PlateGoesUp Play)
    (:Update
      (Transformation|SetRelativeLocation (Variables|Default|GetPressurePlate) (Math|Vector|Lerp(Vector) "0, 0,10.000000" "0, 0,1.000000" _newtrack_0) false false))
    (:Finished
      (if (Variables|Default|GetPlateDown?)
        (Rendering|Material|SetMaterial _pressureplate 0 "/Game/Tech/BasicMaterials/M_Green.M_Green")
        (else
          (Rendering|Material|SetMaterial _pressureplate 0 "/Game/Tech/BasicMaterials/M_Blue.M_Blue"))))))

(event OnComponentEndOverlap(Box)
  (params (OverlappedComponent :type Primitive%20Component%20Object%20Reference) (OtherActor :type Actor%20Object%20Reference) (OtherComp :type Primitive%20Component%20Object%20Reference) (OtherBodyIndex :type Integer))
  (bind _othertriggerref (Variables|Default|GetOtherTriggerRef))
  (bind _pressureplate (Variables|Default|GetPressurePlate))
  (Utilities|Array|RemoveItem (Variables|Default|GetOverlappedActors) OtherActor)
  (Utilities|IsValid (Utilities|Array|Get(acopy) (Variables|Default|GetOverlappedActors))
    (:Is%20Not%20Valid
      (Utilities|FlowControl|Sequence
        (:then_0
          (Variables|Default|SetPlateDown? false)
          (bind _newtrack_0 (Timeline|PlateGoesUp Reverse)
            (:Update
              (Transformation|SetRelativeLocation (Variables|Default|GetPressurePlate) (Math|Vector|Lerp(Vector) "0, 0,10.000000" "0, 0,1.000000" _newtrack_0) false false))
            (:Finished
              (if (Variables|Default|GetPlateDown?)
                (Rendering|Material|SetMaterial _pressureplate 0 "/Game/Tech/BasicMaterials/M_Green.M_Green")
                (else
                  (Rendering|Material|SetMaterial _pressureplate 0 "/Game/Tech/BasicMaterials/M_Blue.M_Blue"))))))
        (:then_1
          (Utilities|IsValid _othertriggerref
            (:Is%20Valid
              (Utilities|IsValid (Utilities|Array|Get(acopy) (Variables|BP_PressurePlateTrigger_C|GetOverlappedActors _othertriggerref))
                (:Is%20Not%20Valid
                  _)))
            (:Is%20Not%20Valid
              _))
          (Class|BPITrigger|UnTrigger(Message) (Variables|Default|GetTrapRef))
          (Variables|Default|SetTriggered? false)
          (Development|PrintString "Goodbye")
          (Timeline|PlateGoesUp Reverse))))))

(fn ConstructionScript
  (|CallParentFunction))