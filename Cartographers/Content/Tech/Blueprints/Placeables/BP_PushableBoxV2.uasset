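; Placeable physics box, still work in progress, that the player can interact with to push along one axis.
; X and Y trigger volumes detect BP_BaseCharacter, show an info prompt and record the side overlapped.
; Interact alternates between enabling physics locked to that side's plane, then calling Hold, and disabling physics.
; Mass and drag are applied at BeginPlay; physics-constraint attachment to the character is left unwired.
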(event OnComponentBeginOverlap(YCollision)
  (params (OverlappedComponent :type Primitive%20Component%20Object%20Reference) (OtherActor :type Actor%20Object%20Reference) (OtherComp :type Primitive%20Component%20Object%20Reference) (OtherBodyIndex :type Integer) (bFromSweep :type Boolean) (SweepResult :type Hit%20Result%20Structure%20%28by%20ref%29))
  ;[1 1 1] Checks if player is overlapped in Y
  (Utilities|Casting|CastToBP_BaseCharacter OtherActor)
  (Rendering|SetVisibility (Variables|Default|GetInfo) true false)
  (bind _output_get (Variables|Default|SetOverlapped%20in%20Y? true))
  (Development|PrintString "Pushable on Y, Overlapped")
  (Development|PrintString (Utilities|String|ToString(Boolean) _output_get)))

(event OnComponentEndOverlap(YCollision)
  (params (OverlappedComponent :type Primitive%20Component%20Object%20Reference) (OtherActor :type Actor%20Object%20Reference) (OtherComp :type Primitive%20Component%20Object%20Reference) (OtherBodyIndex :type Integer))
  ;[1 1 1] Checks if player is overlapped in Y
  (Utilities|Casting|CastToBP_BaseCharacter OtherActor)
  (Rendering|SetVisibility (Variables|Default|GetInfo) false false)
  (bind _output_get (Variables|Default|SetOverlapped%20in%20Y? false))
  (Development|PrintString "No longer pushable on Y, no longer overlapped")
  (Development|PrintString (Utilities|String|ToString(Boolean) _output_get)))

(event OnComponentBeginOverlap(XCollision)
  (params (OverlappedComponent :type Primitive%20Component%20Object%20Reference) (OtherActor :type Actor%20Object%20Reference) (OtherComp :type Primitive%20Component%20Object%20Reference) (OtherBodyIndex :type Integer) (bFromSweep :type Boolean) (SweepResult :type Hit%20Result%20Structure%20%28by%20ref%29))
  ;[1 1 1] Checks if player is overlapped in X
  (Utilities|Casting|CastToBP_BaseCharacter OtherActor)
  (Rendering|SetVisibility (Variables|Default|GetInfo) true false)
  (bind _output_get (Variables|Default|SetOverlapped%20in%20X? true))
  (Development|PrintString "Pushable on X, Overlapped")
  (Development|PrintString (Utilities|String|ToString(Boolean) _output_get)))

(event OnComponentEndOverlap(XCollision)
  (params (OverlappedComponent :type Primitive%20Component%20Object%20Reference) (OtherActor :type Actor%20Object%20Reference) (OtherComp :type Primitive%20Component%20Object%20Reference) (OtherBodyIndex :type Integer))
  ;[1 1 1] Checks if player is overlapped in X
  (Utilities|Casting|CastToBP_BaseCharacter OtherActor)
  (Rendering|SetVisibility (Variables|Default|GetInfo) false false)
  (bind _output_get (Variables|Default|SetOverlapped%20in%20X? false))
  (Development|PrintString "No longer pushable on X, no longer overlapped")
  (Development|PrintString (Utilities|String|ToString(Boolean) _output_get)))

(event Custom|Init
  (bind _box (Variables|Default|GetBox))
  ;[1 1 1] Init sets the weight and drag of the pushable object
  (Class|PrimitiveComponent|SetMassOverrideinKg _box "None" (Variables|Default|GetMassKG) true)
  (Class|PrimitiveComponent|SetLinearDamping _box (Variables|Default|GetDrag)))

(event Custom|Holding
  (if (Variables|Default|GetInteracted?)
    (CallFunction|Hold)
    (Development|PrintString "Called")))

(event EventBeginPlay
  ;[1 1 1] EventBeginPlay call init
  (CallFunction|Init))

(event EventInteract
  (params (Interacting :type Actor%20Object%20Reference))
  ;[1 1 1] WIP
  (Utilities|FlowControl|FlipFlop
    (:A
      (if (Variables|Default|GetOverlapped%20in%20Y?)
        (Physics|SetSimulatePhysics (Variables|Default|GetBox) true)
        (Class|PrimitiveComponent|SetConstraintMode (Variables|Default|GetBox) "YZPlane")
        (Variables|Default|SetInteracted? true)
        (CallFunction|Holding)
        (elif (Variables|Default|GetOverlapped%20in%20X?)
          (Physics|SetSimulatePhysics (Variables|Default|GetBox) true)
          (Class|PrimitiveComponent|SetConstraintMode (Variables|Default|GetBox) "XZPlane")
          (Variables|Default|SetInteracted? true)
          (CallFunction|Holding))))
    (:B
      (if (Variables|Default|GetOverlapped%20in%20Y?)
        (Physics|SetSimulatePhysics (Variables|Default|GetBox) false)
        (Class|PrimitiveComponent|SetConstraintMode (Variables|Default|GetBox) "SixDOF")
        (Variables|Default|SetInteracted? false)
        (CallFunction|Holding)
        (elif (Variables|Default|GetOverlapped%20in%20X?)
          (Physics|SetSimulatePhysics (Variables|Default|GetBox) false)
          (Class|PrimitiveComponent|SetConstraintMode (Variables|Default|GetBox) "SixDOF")
          (Variables|Default|SetInteracted? false)
          (CallFunction|Holding))))))

(fn ConstructionScript)