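; BP_SpawnPoint is a placeable spawn point marker tagged with a character, either Mage or Scout.
; Its construction script switches on the Character value to set the TextRender label to that name, colored blue for Mage and red for Scout.
; The event graph holds only disabled stub events, so this Blueprint's graphs contain no spawning logic.
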(event EventBeginPlay)

(event Collision|EventActorBeginOverlap
  (params (OtherActor :type Actor%20Object%20Reference)))

(event EventTick
  (params (DeltaSeconds :type Float%20%28single-precision%29)))

(fn ConstructionScript
  (bind _textrender (Variables|Default|GetTextRender))
  (bind _textrender_2 (Variables|Default|GetTextRender))
  (switch Utilities|FlowControl|Switch|SwitchonE_Characters (Variables|Default|GetCharacter)
    (:NewEnumerator1
      (Rendering|Components|TextRender|SetText _textrender_2 (Utilities|Text|FormatText "Mage"))
      (Rendering|Components|TextRender|SetTextRenderColor _textrender_2 (Math|Color|MakeColor 255 0 0)))
    (:NewEnumerator0
      (Rendering|Components|TextRender|SetText _textrender (Utilities|Text|FormatText "Scout"))
      (Rendering|Components|TextRender|SetTextRenderColor _textrender (Math|Color|MakeColor 0 0 255)))))