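; Placeable torch that the Interact event switches between lit and unlit.
; A FlipFlop alternates between Trigger and UnTrigger, starting with Trigger on the first interaction.
; Trigger shows the Torchlight component and spawns a fire actor at FirePoint, keeping it in FireRef.
; UnTrigger hides the light and destroys that actor, so the fire is respawned on each ignition rather than toggled by visibility.
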(event EventTrigger
  ;[1 1 1] Sets visibility of light and particles
  (Rendering|SetVisibility (Variables|Default|GetTorchlight) true false)
  (bind _returnvalue (Game|SpawnActorfromClass "/Game/Art/EnvironmentArt/Particles/BP_PS_Fire.BP_PS_Fire_C" (Transformation|GetWorldTransform (Variables|Default|GetFirePoint)) "Undefined" 0 0))
  (Variables|Default|SetFireRef _returnvalue))

(event EventUnTrigger
  ;[1 1 1] Unsets visibility of light and particles
  (Rendering|SetVisibility (Variables|Default|GetTorchlight) false false)
  (Actor|DestroyActor (Variables|Default|GetFireRef)))

(event EventInteract
  (params (Interacting :type Actor%20Object%20Reference))
  ;[1 0 0] When interacted with, will switch between calling ignite or extinguish
  (Utilities|FlowControl|FlipFlop
    (:A
      (CallFunction|Trigger))
    (:B
      (CallFunction|UnTrigger))))

(fn ConstructionScript)