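; BP_BossDoor is an interactable double door, judging by its name for a boss encounter, that slides open when interacted with.
; BeginPlay records each panel's world position and adds a target offset to get its open position.
; Interact runs the parent logic, then OpenDoor plays a timeline that lerps both panels between those positions.
; CloseDoor reverses the same timeline at twice the opening rate, both scaled by a speed modifier.
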(event Custom|OpenDoor
  (Components|Timeline|SetPlayRate (Variables|Default|GetOpen) (* (Variables|Default|GetSpeedModifier) 1.0))
  (bind _newtrack_0 (Timeline|Open Play)
    (:Update
      (Transformation|SetWorldLocation (Variables|Default|GetLeftDoor) (Math|Vector|Lerp(Vector) (Variables|Default|GetLeftDoorStartLocation) (Variables|Default|GetLeftDoorEndLocation) _newtrack_0) false false)
      (Transformation|SetWorldLocation (Variables|Default|GetRightDoor) (Math|Vector|Lerp(Vector) (Variables|Default|GetRightDoorStartLocation) (Variables|Default|GetRightDoorEndLocation) _newtrack_0) false false))))

(event Custom|CloseDoor
  (Components|Timeline|SetPlayRate (Variables|Default|GetOpen) (* (Variables|Default|GetSpeedModifier) 2.0))
  (bind _newtrack_0 (Timeline|Open Reverse)
    (:Update
      (Transformation|SetWorldLocation (Variables|Default|GetLeftDoor) (Math|Vector|Lerp(Vector) (Variables|Default|GetLeftDoorStartLocation) (Variables|Default|GetLeftDoorEndLocation) _newtrack_0) false false)
      (Transformation|SetWorldLocation (Variables|Default|GetRightDoor) (Math|Vector|Lerp(Vector) (Variables|Default|GetRightDoorStartLocation) (Variables|Default|GetRightDoorEndLocation) _newtrack_0) false false))))

(event EventBeginPlay
  (bind _output_get (Variables|Default|SetLeftDoorStartLocation (Transformation|GetWorldLocation (Variables|Default|GetLeftDoor))))
  (Variables|Default|SetLeftDoorEndLocation (+ _output_get (Variables|Default|GetLeftDoorTargetLocation)))
  (bind _output_get_2 (Variables|Default|SetRightDoorStartLocation (Transformation|GetWorldLocation (Variables|Default|GetRightDoor))))
  (Variables|Default|SetRightDoorEndLocation (+ _output_get_2 (Variables|Default|GetRightDoorTargetLocation))))

(event EventInteract
  (params (Interacting :type Actor%20Object%20Reference))
  (|CallParentFunction Interacting)
  (CallFunction|OpenDoor))

(fn ConstructionScript
  (|CallParentFunction))