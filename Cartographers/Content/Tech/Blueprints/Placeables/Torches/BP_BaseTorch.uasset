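; Base torch placeable that can be lit or put out through Trigger and UnTrigger events.
; Trigger spawns a BP_PS_Fire actor at the FirePoint transform and stores it, and BeginPlay calls it when TurnedOn is set.
; UnTrigger destroys the stored fire actor if valid, so the flame is toggled by spawning and destroying rather than by visibility.
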(event EventTrigger
  ;[1 1 1] Sets visibility of light and particles
  (bind _returnvalue (Game|SpawnActorfromClass "/Game/Art/EnvironmentArt/Particles/BP_PS_Fire.BP_PS_Fire_C" (Transformation|GetWorldTransform (Variables|Default|GetFirePoint)) "Undefined" 0 0))
  (Variables|Default|SetFireRef _returnvalue))

(event EventUnTrigger
  (bind _fireref (Variables|Default|GetFireRef))
  ;[1 1 1] Unsets visibility of light and particles
  (Utilities|IsValid _fireref
    (:Is%20Valid
      (Actor|DestroyActor _fireref))))

(event EventBeginPlay
  (if (Variables|Default|GetTurnedOn?)
    (CallFunction|Trigger)))

(fn ConstructionScript)