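; BP_MovingWall is a placeable trap wall whose Cube slides between its start position and an offset TargetLocation.
; BeginPlay caches the start and end world positions.
; Trigger plays the Open timeline, lerping the Cube's world location between them without sweep.
; UnTrigger reverses the timeline at five times the speed, so the wall returns much faster than it moves out.
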(event EventBeginPlay
  (bind _output_get (Variables|Default|SetStartLocation (Transformation|GetWorldLocation (Variables|Default|GetCube))))
  (Variables|Default|SetEndLocation (+ _output_get (Variables|Default|GetTargetLocation))))

(event EventTrigger
  (Components|Timeline|SetPlayRate (Variables|Default|GetOpen) 1.0)
  (bind _newtrack_0 (Timeline|Open Play)
    (:Update
      (Transformation|SetWorldLocation (Variables|Default|GetCube) (Math|Vector|Lerp(Vector) (Variables|Default|GetStartLocation) (Variables|Default|GetEndLocation) _newtrack_0) false false))))

(event EventUnTrigger
  (Components|Timeline|SetPlayRate (Variables|Default|GetOpen) 5.0)
  (bind _newtrack_0 (Timeline|Open Reverse)
    (:Update
      (Transformation|SetWorldLocation (Variables|Default|GetCube) (Math|Vector|Lerp(Vector) (Variables|Default|GetStartLocation) (Variables|Default|GetEndLocation) _newtrack_0) false false))))

(fn ConstructionScript
  (|CallParentFunction))