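; BP_RisingBlock is a placeable trap block that moves its Cube vertically when triggered and returns it when untriggered.
; Trigger plays the RisingBlock timeline, lerping relative Z from BlockStartingLocation to BlockEndLocation.
; UnTrigger plays a separate ResetBlock timeline with the endpoints swapped, rather than reversing the first.
; Both use Play rather than PlayFromStart and set the location without sweeping.
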(event EventTrigger
  (bind _newtrack_0 (Timeline|RisingBlock Play)
    (:Update
      (Transformation|SetRelativeLocation (Variables|Default|GetCube) (Math|Vector|Lerp(Vector) (Math|Vector|MakeVector 0.0 0.0 (Variables|Default|GetBlockStartingLocation)) (Math|Vector|MakeVector 0.0 0.0 (Variables|Default|GetBlockEndLocation)) _newtrack_0) false false))))

(event EventUnTrigger
  (bind _newtrack_0 (Timeline|Reset%20Block Play)
    (:Update
      (Transformation|SetRelativeLocation (Variables|Default|GetCube) (Math|Vector|Lerp(Vector) (Math|Vector|MakeVector 0.0 0.0 (Variables|Default|GetBlockEndLocation)) (Math|Vector|MakeVector 0.0 0.0 (Variables|Default|GetBlockStartingLocation)) _newtrack_0) false false))))

(fn ConstructionScript
  (|CallParentFunction))