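; Placeable trap-category bridge of four blocks that rise one after another when triggered.
; Trigger starts a chain of per-cube timelines that lerp each block upward, each calling the next from its update through a short delay, running Cube4 to Cube1.
; UnTrigger drops the whole bridge at once by lowering the shared Scene component on a timeline at double play rate.
; No timeline is reversed or restarted from the beginning here.
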(event Custom|RiseCube3
  (bind _newtrack_0 (Timeline|RiseBlock3 Play)
    (:Update
      (Transformation|SetRelativeLocation (Variables|Default|GetCube3) (Math|Vector|Lerp(Vector) "50.000000,0.000000,-50.000000" "50.000000,0.000000,50.000000" _newtrack_0) false false)
      (Utilities|FlowControl|Delay 0.5)
      (CallFunction|RiseCube2))))

(event Custom|RiseCube2
  (bind _newtrack_0 (Timeline|RiseBlock2 Play)
    (:Update
      (Transformation|SetRelativeLocation (Variables|Default|GetCube2) (Math|Vector|Lerp(Vector) "-50.000000,0.000000,-50.000000" "-50.000000,0.000000,50.000000" _newtrack_0) false false)
      (Utilities|FlowControl|Delay 0.5)
      (CallFunction|RiseCube1))))

(event Custom|RiseCube1
  (bind _newtrack_0 (Timeline|RiseBlock1 Play)
    (:Update
      (Transformation|SetRelativeLocation (Variables|Default|GetCube1) (Math|Vector|Lerp(Vector) "-150.000000,0.000000,-50.000000" "-150.000000,0.000000,50.000000" _newtrack_0) false false))
    (:Finished
      (Utilities|FlowControl|Delay 2.0))))

(event EventTrigger
  (bind _newtrack_0 (Timeline|RiseBlocks Play)
    (:Update
      (Transformation|SetRelativeLocation (Variables|Default|GetCube4) (Math|Vector|Lerp(Vector) "150.000000,0.000000,-50.000000" "150.000000,0.000000,50.000000" _newtrack_0) false false)
      (Utilities|FlowControl|Delay 0.5)
      (CallFunction|RiseCube3))))

(event EventUnTrigger
  (Components|Timeline|SetPlayRate (Variables|Default|GetDropAllBridge) 2.0)
  (bind _newtrack_0 (Timeline|DropAllBridge Play)
    (:Update
      (Transformation|SetRelativeLocation (Variables|Default|GetScene) (Math|Vector|Lerp(Vector) "0, 0, 0" "0, 0,-100.000000" _newtrack_0) false false))))

(fn ConstructionScript
  (|CallParentFunction))