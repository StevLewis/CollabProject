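; Placeable spike trap that raises its spike when a character steps on it and damages actors that touch its hit box.
; SpikeTrigger overlaps by BP_BaseCharacter call Trigger if Triggerable, which waits a delay, then plays a timeline that lerps the spike upward.
; Any character leaving reverses the timeline immediately, even if others remain in OverlappedActors.
; A separate Box overlap applies damage to any actor, independent of trigger state.
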(event OnComponentBeginOverlap(SpikeTrigger)
  (params (OverlappedComponent :type Primitive%20Component%20Object%20Reference) (OtherActor :type Actor%20Object%20Reference) (OtherComp :type Primitive%20Component%20Object%20Reference) (OtherBodyIndex :type Integer) (bFromSweep :type Boolean) (SweepResult :type Hit%20Result%20Structure%20%28by%20ref%29))
  (if (Variables|Default|GetTriggerable?)
    (bind _asbp_base_character (Utilities|Casting|CastToBP_BaseCharacter OtherActor))
    (CallFunction|Trigger)
    (Utilities|Array|Add (Variables|Default|GetOverlappedActors) _asbp_base_character)))

(event OnComponentEndOverlap(SpikeTrigger)
  (params (OverlappedComponent :type Primitive%20Component%20Object%20Reference) (OtherActor :type Actor%20Object%20Reference) (OtherComp :type Primitive%20Component%20Object%20Reference) (OtherBodyIndex :type Integer))
  (bind _asbp_base_character (Utilities|Casting|CastToBP_BaseCharacter OtherActor))
  (CallFunction|UnTrigger)
  (Utilities|Array|RemoveItem (Variables|Default|GetOverlappedActors) _asbp_base_character))

(event OnComponentBeginOverlap(Box)
  (params (OverlappedComponent :type Primitive%20Component%20Object%20Reference) (OtherActor :type Actor%20Object%20Reference) (OtherComp :type Primitive%20Component%20Object%20Reference) (OtherBodyIndex :type Integer) (bFromSweep :type Boolean) (SweepResult :type Hit%20Result%20Structure%20%28by%20ref%29))
  (Game|Damage|ApplyDamage OtherActor 1.0 0 0))

(event EventTrigger
  (Utilities|FlowControl|Delay (Variables|Default|GetDelay))
  (bind _newtrack_0 (Timeline|SpikeGoUp PlayFromStart)
    (:Update
      (Transformation|SetRelativeLocation (Variables|Default|GetSpike) (Math|Vector|Lerp(Vector) "0, 0,-100.000000" "0.000000,0.000000,100.000000" _newtrack_0) false false))))

(event EventUnTrigger
  (bind _newtrack_0 (Timeline|SpikeGoUp Reverse)
    (:Update
      (Transformation|SetRelativeLocation (Variables|Default|GetSpike) (Math|Vector|Lerp(Vector) "0, 0,-100.000000" "0.000000,0.000000,100.000000" _newtrack_0) false false))))

(fn ConstructionScript
  (|CallParentFunction))