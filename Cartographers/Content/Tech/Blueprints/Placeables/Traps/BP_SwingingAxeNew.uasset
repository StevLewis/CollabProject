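; BP_SwingingAxeNew is a placeable trap: an axe that swings back and forth and damages actors that touch it.
; A timeline starts on BeginPlay, lerps the Pivot's relative rotation between two angles, and restarts itself whenever it finishes, printing a debug string.
; The Box component applies damage on overlap.
; Trigger sets a flag that stops the swing when the current cycle ends, while UnTrigger is empty.
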(event OnComponentBeginOverlap(Box)
  (params (OverlappedComponent :type Primitive%20Component%20Object%20Reference) (OtherActor :type Actor%20Object%20Reference) (OtherComp :type Primitive%20Component%20Object%20Reference) (OtherBodyIndex :type Integer) (bFromSweep :type Boolean) (SweepResult :type Hit%20Result%20Structure%20%28by%20ref%29))
  ;[1 1 1] Apply damage to character
  (Game|Damage|ApplyDamage OtherActor 1.0 0 0))

(event EventBeginPlay
  ;[1 1 1] Plays swinging animation for the axe
  (bind _newtrack_0 (Timeline|SwingingAction Play)
    (:Update
      (Transformation|SetRelativeRotation (Variables|Default|GetPivot) (Math|Rotator|Lerp(Rotator) "-50.000000, 0, 0" "50.000000,0.000000, 0" _newtrack_0) false false))
    (:Finished
      (Development|PrintString "Harry Sucks")
      (if (Variables|Default|GetRequestStop)
        (Audio|Components|Audio|Stop (Variables|Default|GetSwingingAction))
        (else
          (Timeline|SwingingAction PlayFromStart))))))

(event EventUnTrigger)

(event EventTrigger
  (Variables|Default|SetRequestStop true))

(fn ConstructionScript
  (|CallParentFunction))