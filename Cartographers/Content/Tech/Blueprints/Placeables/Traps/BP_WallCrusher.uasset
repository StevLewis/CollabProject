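; BP_WallCrusher is a placeable trap whose two walls slide toward each other to crush the space between them.
; Trigger waits briefly, then plays a timeline that lerps both walls' relative locations inward without sweep.
; After a pause in the closed position, the timeline reverses to reopen the walls.
; The construction script calls its parent and sets the timeline play rate from CrushSpeed.
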(event EventTrigger
  (Utilities|FlowControl|Delay 0.5)
  (bind _newtrack_0 (Timeline|Timeline_0 PlayFromStart)
    (:Update
      (Transformation|SetRelativeLocation (Variables|Default|GetWall1) (Math|Vector|Lerp(Vector) "-150.000000,0.000000,50.000000" "-50.000000,0.000000,50.000000" _newtrack_0) false false)
      (Transformation|SetRelativeLocation (Variables|Default|GetWall2) (Math|Vector|Lerp(Vector) "150.000000,0.000000,50.000000" "50.000000,0.000000,50.000000" _newtrack_0) false false))
    (:Finished
      (Utilities|FlowControl|Delay 5.0)
      (Timeline|Timeline_0 ReverseFromEnd))))

(fn ConstructionScript
  (|CallParentFunction)
  (Components|Timeline|SetPlayRate (Variables|Default|GetTimeline_0) (Variables|Default|GetCrushSpeed)))