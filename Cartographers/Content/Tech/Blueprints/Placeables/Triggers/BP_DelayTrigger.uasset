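; BP_DelayTrigger is a pressure plate that fires an array of linked traps in sequence, separated by a set delay.
; Overlap lowers the plate via a timeline, swaps its material and starts a looping timer to step through the traps with TriggerMessage.
; When the last actor leaves, the plate rises.
; Unless an optional partner trigger is still occupied, all traps receive UnTriggerMessage and the sequence resets.
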(event OnComponentBeginOverlap(Box)
  (params (OverlappedComponent :type Primitive%20Component%20Object%20Reference) (OtherActor :type Actor%20Object%20Reference) (OtherComp :type Primitive%20Component%20Object%20Reference) (OtherBodyIndex :type Integer) (bFromSweep :type Boolean) (SweepResult :type Hit%20Result%20Structure%20%28by%20ref%29))
  (bind _pressureplate (Variables|Default|GetPressurePlate))
  (if (not (Variables|Default|GetTriggered?))
    (bind _returnvalue (Utilities|Time|SetTimerbyEvent (EventDispatchers|CreateEvent :!event TriggerTrap) (Variables|Default|GetTrapDelay) true))
    (Variables|Default|SetTimerDelayTH _returnvalue))
  (Variables|Default|SetTriggered? true)
  (Utilities|Array|Add (Variables|Default|GetOverlappedActors) OtherActor)
  (Variables|Default|SetPlateDown? true)
  (bind _newtrack_0 (Timeline|Timeline_0 Play)
    (:Update
      (Transformation|SetRelativeLocation (Variables|Default|GetPressurePlate) (Math|Vector|Lerp(Vector) "0, 0,10.000000" "0, 0,1.000000" _newtrack_0) false false))
    (:Finished
      (if (Variables|Default|GetPlateDown?)
        (Rendering|Material|SetMaterial _pressureplate 0 "/Game/Tech/BasicMaterials/M_Brown.M_Brown")
        (else
          (Rendering|Material|SetMaterial _pressureplate 0 "/Game/Tech/BasicMaterials/M_Green.M_Green"))))))

(event OnComponentEndOverlap(Box)
  (params (OverlappedComponent :type Primitive%20Component%20Object%20Reference) (OtherActor :type Actor%20Object%20Reference) (OtherComp :type Primitive%20Component%20Object%20Reference) (OtherBodyIndex :type Integer))
  (bind _othertriggerref (Variables|Default|GetOtherTriggerRef))
  (bind _pressureplate (Variables|Default|GetPressurePlate))
  (Utilities|Array|RemoveItem (Variables|Default|GetOverlappedActors) OtherActor)
  (Utilities|IsValid (Utilities|Array|Get(acopy) (Variables|Default|GetOverlappedActors))
    (:Is%20Not%20Valid
      (Utilities|FlowControl|Sequence
        (:then_0
          (Variables|Default|SetPlateDown? false)
          (bind _newtrack_0 (Timeline|Timeline_0 Reverse)
            (:Update
              (Transformation|SetRelativeLocation (Variables|Default|GetPressurePlate) (Math|Vector|Lerp(Vector) "0, 0,10.000000" "0, 0,1.000000" _newtrack_0) false false))
            (:Finished
              (if (Variables|Default|GetPlateDown?)
                (Rendering|Material|SetMaterial _pressureplate 0 "/Game/Tech/BasicMaterials/M_Brown.M_Brown")
                (else
                  (Rendering|Material|SetMaterial _pressureplate 0 "/Game/Tech/BasicMaterials/M_Green.M_Green"))))))
        (:then_1
          (Utilities|IsValid _othertriggerref
            (:Is%20Valid
              (Utilities|IsValid (Utilities|Array|Get(acopy) (Variables|/Game/Tech/Blueprints/Placeables/Triggers/BP_PressurePlateTrigger.BP_PressurePlateTrigger_C|GetOverlappedActors _othertriggerref))
                (:Is%20Not%20Valid
                  _)))
            (:Is%20Not%20Valid
              _))
          (for _array_element (Variables|Default|GetTrapRef)
            (Class|BPITrigger|UnTrigger(Message) _array_element))
          (Variables|Default|SetTriggered? false)
          (Variables|Default|SetTrapIndex 0)
          (Utilities|Time|ClearandInvalidateTimerbyHandle (Variables|Default|GetTimerDelayTH)))))))

(fn ConstructionScript
  (|CallParentFunction))

(fn TriggerTrap
  (bind _trapref (Variables|Default|GetTrapRef))
  (bind _trapindex (Variables|Default|GetTrapIndex))
  (bind _output (Utilities|Array|Get(acopy) _trapref _trapindex))
  (Utilities|IsValid _output
    (:Is%20Valid
      (Class|BPITrigger|Trigger(Message) _output)
      (Math|Integer|IncrementInt (Variables|Default|GetTrapIndex)))
    (:Is%20Not%20Valid
      (Utilities|Time|ClearandInvalidateTimerbyHandle (Variables|Default|GetTimerDelayTH)))))