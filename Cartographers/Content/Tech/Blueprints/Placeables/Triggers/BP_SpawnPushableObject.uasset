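; Placeable interactable that resets a pushable box to its starting position.
; On BeginPlay it caches the location of the referenced pushable object.
; Interacting destroys that object and spawns a new BP_PushableBoxV2 at the cached location with a fixed enlarged scale.
; The reference then points to the new box, which receives a HoldMessage call.
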(event Custom|RespawnObject
  ;[1 1 1] Respawns the object to the original objects location
  (Actor|DestroyActor (Variables|Default|GetPushableObjectRef))
  (bind _returnvalue (Game|SpawnActorfromClass "/Game/Tech/Blueprints/Placeables/BP_PushableBoxV2.BP_PushableBoxV2_C" (Math|Transform|MakeTransform (Variables|Default|GetObjectLocation) "0, 0, 0" "2.000000,2.000000,2.000000") "Undefined" 0 0))
  (bind _output_get (Variables|Default|SetPushableObjectRef _returnvalue))
  (Class|BPIHold|Hold(Message) _output_get)
  (Development|PrintString "Respawned"))

(event Custom|Init
  ;[1 1 1] Set Object location to the referenced object
  (Variables|Default|SetObjectLocation (Transformation|GetActorLocation (Variables|Default|GetPushableObjectRef))))

(event EventInteract
  (params (Interacting :type Actor%20Object%20Reference))
  ;[1 1 1] On interact, call respawn object
  (|CallParentFunction Interacting)
  (CallFunction|RespawnObject)
  (Development|PrintString "Pushed"))

(event EventBeginPlay
  ;[1 1 1] Event BeginPlay, call init
  (CallFunction|Init))

(fn ConstructionScript
  (|CallParentFunction))