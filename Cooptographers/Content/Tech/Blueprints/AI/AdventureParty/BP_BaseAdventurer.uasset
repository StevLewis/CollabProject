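; Base AI character for adventuring party members that follow a spawn point's spline toward the boss room, notifying and despawning past the last point.
; Feeds leader and pause state to the Blackboard, serves spline waypoints at its current height, and turns its nameplate toward the camera.
; An idle counter asks GM_Gameplay to teleport to the next point when stuck.
; Death selects sound, effects, and montage or ragdoll by damage type.
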(event Custom|IdleUpdate
  ;[0.001723 0.1094 0] Idle
  (if (not (Variables|Default|GetDead?))
    (if (<= (Math|Vector|VectorLength (Transformation|GetVelocity)) 0.0)
      (bind _result (Math|Float|IncrementFloat (Variables|Default|GetIdleTime))
        (:%20%20
          (if (>= _result 15.0)
            (bind _asgm_gameplay (Utilities|Casting|CastToGM_Gameplay (Game|GetGameMode)))
            (Default|TeleporttoNextPoint _asgm_gameplay 0.0))))
      (else
        (Variables|Default|SetIdleTime 0.0)))))

(event Custom|Init
  (params (SpawnPoint :type BP%20Adventure%20Party%20Spawn%20Point%20Object%20Reference) (Name :type Text) (MovementSpeed :type Float%20%28single-precision%29))
  ;[0.001723 0.1094 0] Init
  (Variables|Default|SetSpawnPoint SpawnPoint)
  (Variables|Default|SetName Name)
  (Variables|/Script/Engine.CharacterMovementComponent|SetMaxWalkSpeed (Variables|Character|GetCharacterMovement) MovementSpeed)
  (Default|Init (.AsWB%20Nameplate (Utilities|Casting|CastToWB_Nameplate (UserInterface|GetWidget (Variables|Default|GetNameWidget)))) (Variables|Default|GetName))
  (Variables|Default|SetSplinePath (Variables|/Game/Tech/Blueprints/Placeables/Spawnpoints/BP_AdventurePartySpawnPoint.BP_AdventurePartySpawnPoint_C|GetSplinePath (Variables|Default|GetSpawnPoint)))
  (Variables|Default|SetSplinePoints (Spline|GetNumberOfSplinePoints (Variables|Default|GetSplinePath)))
  (Utilities|Time|SetTimerbyEvent (EventDispatchers|CreateEvent :!event Custom|IdleUpdate) 1.0 true))

(event Custom|PauseMovement
  (params (PauseTime :type Float%20%28single-precision%29))
  ;[0.001723 0.1094 0] Pausing / Resuming Movement
  (if (> PauseTime 0.0)
    (Utilities|Time|SetTimerbyEvent (delegate Custom|ResumeMovement) PauseTime))
  (bind _output_get (Variables|Default|SetShouldMove? false))
  (AI|Components|Blackboard|SetValueasBool (AI|GetBlackboard 0) (Utilities|Name|MakeLiteralName "ShouldMove?") _output_get))

(event Custom|ResumeMovement
  ;[0.001723 0.1094 0] Pausing / Resuming Movement
  (bind _output_get (Variables|Default|SetShouldMove? true))
  (AI|Components|Blackboard|SetValueasBool (AI|GetBlackboard 0) (Utilities|Name|MakeLiteralName "ShouldMove?") _output_get))

(event EventTick
  (params (DeltaSeconds :type Float%20%28single-precision%29))
  (bind _namewidget (Variables|Default|GetNameWidget))
  ;[0.001723 0.1094 0] Tick
  (Transformation|SetWorldRotation _namewidget (Math|Rotator|FindLookatRotation (Transformation|GetWorldLocation _namewidget) (Transformation|GetWorldLocation (Variables|/Script/Engine.PlayerCameraManager|GetTransformComponent (Game|GetPlayerCameraManager 0)))) false false))

(event EventApplyDamagebyType
  (params (Damage :type Float%20%28single-precision%29) (DamageCauser :type Actor%20Object%20Reference) (DamageType :type E_DamageTypes%20Enum :default "NewEnumerator0"))
  ;[0.001723 0.1094 0] Damage
  (CallFunction|Death DamageType))

(fn ConstructionScript)

(fn GetNextSplinePoint
  (if (<= (Variables|Default|GetCurrentSplinePoint) (Variables|Default|GetSplinePoints))
    (bind _targetlocation (CallFunction|FindNextPointAlongSpline (Variables|Default|GetCurrentSplinePoint)))
    (Variables|Default|SetTargetLocation _targetlocation)
    (Math|Integer|IncrementInt (Variables|Default|GetCurrentSplinePoint)
      (:%20%20
        (return _targetlocation)))
    (else
      (Variables|Default|SetBossRoomReached? true)
      (Default|CallBossRoomReached)
      (Actor|DestroyActor))))

(fn Death
  (params (DamageType :type E_DamageTypes%20Enum :default "NewEnumerator0"))
  (LocalVariables|SetDamageType%20%28local%29 DamageType)
  (if (not (Variables|Default|GetDead?))
    (Utilities|FlowControl|Sequence
      (:then_0
        (Variables|Default|SetDead? true)
        (Pawn|Components|CharacterMovement|DisableMovement (Variables|Character|GetCharacterMovement)))
      (:then_1
        (CallFunction|SpawnSoundAttached (Utilities|Select :Index (LocalVariables|GetDamageType%20%28local%29) :NewEnumerator0 "/Game/Tech/Sounds/Cues/SC_Death.SC_Death" :NewEnumerator1 "/Game/Design/SFX/Death-SpikeTrap.Death-SpikeTrap" :NewEnumerator2 "/Game/Design/SFX/Death-Burning.Death-Burning" :NewEnumerator3 "/Game/Design/SFX/Death-Electricity.Death-Electricity"))
        (Niagara|SpawnSystemAttached (Utilities|Select :Index (LocalVariables|GetDamageType%20%28local%29) :NewEnumerator0 "/Game/Tech/FX/NS_Death.NS_Death" :NewEnumerator1 0 :NewEnumerator2 "/Game/Tech/FX/PS_Fire.PS_Fire" :NewEnumerator3 0) (Variables|Character|GetMesh) "pelvis" "0, 0, 0" "0, 0, 0" "KeepRelativeOffset" false)
        (if (Utilities|Enum|Equal(Enum) (LocalVariables|GetDamageType%20%28local%29) "NewEnumerator0")
          (CallFunction|Ragdoll)
          (else
            (bind _returnvalue (Animation|PlayAnimMontage (Utilities|Select :Index (LocalVariables|GetDamageType%20%28local%29) :NewEnumerator0 0 :NewEnumerator1 "/Game/Tech/Blueprints/Animation/Death/AM_Death_Spikes.AM_Death_Spikes" :NewEnumerator2 "/Game/Tech/Blueprints/Animation/Death/AM_Death_Burn.AM_Death_Burn" :NewEnumerator3 "/Game/Tech/Blueprints/Animation/Death/AM_Death_Electric.AM_Death_Electric") 1.0 "None"))
            (Utilities|Time|SetTimerbyEvent (EventDispatchers|CreateEvent :!event Ragdoll) _returnvalue))))
      (:then_2
        (Default|CallOnDeath)))))

(fn Ragdoll
  (bind _mesh (Variables|Character|GetMesh))
  (Physics|SetSimulatePhysics _mesh true)
  (Collision|SetCollisionEnabled _mesh "QueryAndPhysics")
  (Utilities|Time|SetTimerbyEvent (EventDispatchers|CreateEvent :!event Destroy) 1.0))

(fn UpdatePathing
  (params (Leader :type BP%20Base%20Adventurer%20Object%20Reference) (Leader? :type Boolean) (CurrentSplinePoint :type Integer))
  (Variables|Default|SetLeader Leader)
  (Variables|Default|SetLeader? Leader?)
  (Variables|Default|SetCurrentSplinePoint CurrentSplinePoint)
  (AI|Components|Blackboard|SetValueasObject (AI|GetBlackboard 0) (Utilities|Name|MakeLiteralName "Leader") (Variables|Default|GetLeader))
  (AI|Components|Blackboard|SetValueasBool (AI|GetBlackboard 0) (Utilities|Name|MakeLiteralName "Leader?") (Variables|Default|GetLeader?)))

(fn FindNextPointAlongSpline
  (params (CurrentSplinePoint :type Integer))
  (bind _splinepath (Variables|Default|GetSplinePath))
  (bind _returnvalue (Spline|GetLocationatSplinePoint _splinepath CurrentSplinePoint "World"))
  (bind (_x _y) (Math|Vector|BreakVector _returnvalue))
  (return (Math|Vector|MakeVector _x _y (.Z (Math|Vector|BreakVector (Transformation|GetActorLocation))))))

(fn Destroy
  (Actor|DestroyActor))

(fn SpawnSoundAttached
  (params (Sound :type Sound%20Base%20Object%20Reference))
  (Audio|SpawnSoundAttached Sound (Variables|Collision|GetCapsuleComponent) "None" (Transformation|GetActorLocation) "0, 0, 0" "SnapToTarget" false 1.0 1.0 0.0 "/Game/Tech/Sounds/SA_DefaultAttentuation.SA_DefaultAttentuation" 0))