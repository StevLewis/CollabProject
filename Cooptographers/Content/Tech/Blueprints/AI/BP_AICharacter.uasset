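; AI character with a nameplate that walks a route of placed flags to a boss door.
; It gathers all BP_PlaceableFlag actors, visits them in array order via recursive AIMoveTo calls, skipping invalid ones, then heads to the door and calls BossRoomReached.
; A separate MoveTo event sends it to any destination.
; Any damage kills it, enabling mesh physics, disabling movement and calling OnDeath.
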(event Custom|MoveTo
  (params (Destination :type Vector))
  (AI|AIMoveTo self Destination 0 1e+01 false))

(event Custom|GetAIPathFlags
  (params (BossDoorRef :type BP%20Boss%20Door%20Object%20Reference))
  (Variables|Default|SetBossDoorRef BossDoorRef)
  (bind _outactors (Actor|GetAllActorsOfClass "/Game/Tech/Blueprints/Placeables/BP_PlaceableFlag.BP_PlaceableFlag_C"))
  (for _array_element _outactors
    (Utilities|Array|Add (Variables|Default|GetPathFlags) _array_element))
  (Variables|Default|SetMaxFlags (Utilities|Array|LastIndex (Variables|Default|GetPathFlags))))

(event Custom|Move
  (bind _pathflags (Variables|Default|GetPathFlags))
  (bind _currentpoint (Variables|Default|GetCurrentPoint))
  (bind _output (Utilities|Array|Get(acopy) _pathflags _currentpoint))
  (Utilities|IsValid _output
    (:Is%20Valid
      (AI|AIMoveTo self "0, 0, 0" _output 2e+01 false
        (:OnSuccess
          _)))
    (:Is%20Not%20Valid
      _))
  (bind _result (Math|Integer|IncrementInt (Variables|Default|GetCurrentPoint))
    (:%20%20
      (if (> _result (Variables|Default|GetMaxFlags))
        (AI|AIMoveTo self (Transformation|GetActorLocation (Variables|Default|GetBossDoorRef)) 0 2e+01 false
          (:OnSuccess
            (Default|CallBossRoomReached)))
        (else
          (CallFunction|Move))))))

(event Game|Damage|EventAnyDamage
  (params (Damage :type Float%20%28single-precision%29) (DamageType :type Damage%20Type%20Object%20Reference) (InstigatedBy :type Controller%20Object%20Reference) (DamageCauser :type Actor%20Object%20Reference))
  (CallFunction|Death)
  (Default|CallOnDeath self))

(event EventInit
  (Default|Init (.AsWB%20Nameplate (Utilities|Casting|CastToWB_Nameplate (UserInterface|GetWidget (Variables|Default|GetNameWidget)))) (Variables|Default|GetName)))

(fn ConstructionScript)

(fn Death
  (if (not (Variables|Default|GetDead?))
    (Variables|Default|SetDead? true)
    (Physics|SetSimulatePhysics (Variables|Character|GetMesh) true)
    (Pawn|Components|CharacterMovement|DisableMovement (Variables|Character|GetCharacterMovement))))