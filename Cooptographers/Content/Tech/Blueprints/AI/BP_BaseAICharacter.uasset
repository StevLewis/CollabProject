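; Base AI character that spawns with a name and walk speed, then follows its spawn point's spline toward a boss room.
; Init fills a camera-facing nameplate and sets the blackboard move flag; GetNextSplinePoint supplies successive targets at the actor's height.
; Any damage triggers death and its callback, while running out of points signals BossRoomReached and destroys the actor.
; StopMovementFor only clears the move flag, as its timed disable/resume logic is disconnected.
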(event Custom|MoveTo
  (params (Destination :type Vector))
  (AI|AIMoveTo self Destination 0 1e+01 false))

(event Custom|MoveAlongPath
  ;[1 1 1] Move Along Path
  (bind _output_get (Variables|Default|SetShouldMove? true))
  (AI|Components|Blackboard|SetValueasBool (AI|GetBlackboard 0) (Utilities|Name|MakeLiteralName "ShouldMove?") _output_get))

(event Custom|Init
  (params (SpawnPoint :type BP%20Adventure%20Party%20Spawn%20Point%20Object%20Reference) (Name :type Text) (MovementSpeed :type Float%20%28single-precision%29))
  ;[1 1 1] Init
  (Variables|Default|SetSpawnPoint SpawnPoint)
  (Variables|Default|SetName Name)
  (Variables|/Script/Engine.CharacterMovementComponent|SetMaxWalkSpeed (Variables|Character|GetCharacterMovement) MovementSpeed)
  (Default|Init (.AsWB%20Nameplate (Utilities|Casting|CastToWB_Nameplate (UserInterface|GetWidget (Variables|Default|GetNameWidget)))) (Variables|Default|GetName))
  (CallFunction|MoveAlongPath)
  (Variables|Default|SetSplinePath (Variables|/Game/Tech/Blueprints/Placeables/Spawnpoints/BP_AdventurePartySpawnPoint.BP_AdventurePartySpawnPoint_C|GetSplinePath (Variables|Default|GetSpawnPoint)))
  (Variables|Default|SetSplinePoints (Spline|GetNumberOfSplinePoints (Variables|Default|GetSplinePath)))
  (CallFunction|GetNextSplinePoint))

(event Custom|StopMovementFor
  (params (StopTime :type Float%20%28single-precision%29))
  (bind _output_get (Variables|Default|SetShouldMove? false))
  (AI|Components|Blackboard|SetValueasBool (AI|GetBlackboard 0) (Utilities|Name|MakeLiteralName "ShouldMove?") _output_get))

(event Custom|ResumeMovement
  (Pawn|Components|CharacterMovement|SetMovementMode (Variables|Character|GetCharacterMovement) "MOVE_Walking" 0))

(event Game|Damage|EventAnyDamage
  (params (Damage :type Float%20%28single-precision%29) (DamageType :type Damage%20Type%20Object%20Reference) (InstigatedBy :type Controller%20Object%20Reference) (DamageCauser :type Actor%20Object%20Reference))
  (CallFunction|Death)
  (Default|CallOnDeath))

(event EventTick
  (params (DeltaSeconds :type Float%20%28single-precision%29))
  (bind _namewidget (Variables|Default|GetNameWidget))
  ;[1 1 1] Tick
  (Transformation|SetWorldRotation _namewidget (Math|Rotator|FindLookatRotation (Transformation|GetWorldLocation _namewidget) (Transformation|GetWorldLocation (Variables|/Script/Engine.PlayerCameraManager|GetTransformComponent (Game|GetPlayerCameraManager 0)))) false false))

(fn ConstructionScript)

(fn Death
  (if (not (Variables|Default|GetDead?))
    (Variables|Default|SetDead? true)
    (Pawn|Components|CharacterMovement|DisableMovement (Variables|Character|GetCharacterMovement))))

(fn GetNextSplinePoint
  (bind _splinepath (Variables|Default|GetSplinePath))
  (bind _currentsplinepoint (Variables|Default|GetCurrentSplinePoint))
  (bind _returnvalue (Spline|GetLocationatSplinePoint _splinepath _currentsplinepoint "World"))
  (bind (_x _y) (Math|Vector|BreakVector _returnvalue))
  (if (<= (Variables|Default|GetCurrentSplinePoint) (Variables|Default|GetSplinePoints))
    (bind _output_get (Variables|Default|SetTargetLocation (Math|Vector|MakeVector _x _y (.Z (Math|Vector|BreakVector (Transformation|GetActorLocation))))))
    (Math|Integer|IncrementInt (Variables|Default|GetCurrentSplinePoint)
      (:%20%20
        (return _output_get)))
    (else
      (Default|CallBossRoomReached)
      (CallFunction|Death)
      (Actor|DestroyActor))))