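; AI controller for enemies that runs the BT_Enemy behavior tree and feeds it a target from perception.
; Sensed BP_BaseCharacter actors join a Targets list and are written to the Blackboard "Target" key.
; Lost ones are removed, and the key is cleared if no valid first entry remains.
; Otherwise the key is set to the character just lost, not the remaining entry.
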(event OnTargetPerceptionUpdated(AIPerception)
  (params (Actor :type Actor%20Object%20Reference) (Stimulus :type AI%20Stimulus%20Structure))
  (bind _targets (Variables|Default|GetTargets))
  (bind _asbp_base_character (Utilities|Casting|CastToBP_BaseCharacter Actor))
  (if (.bSuccessfullySensed (Utilities|Struct|BreakAIStimulus Stimulus))
    (Utilities|Array|Add _targets _asbp_base_character)
    (AI|Components|Blackboard|SetValueasObject (AI|GetBlackboard 0) (Utilities|Name|MakeLiteralName "Target") _asbp_base_character :!label _label)
    (else
      (Utilities|Array|RemoveItem _targets _asbp_base_character)
      (Utilities|IsValid (Utilities|Array|Get(acopy) (Variables|Default|GetTargets))
        (:Is%20Valid
          (goto _label))
        (:Is%20Not%20Valid
          (AI|Components|Blackboard|SetValueasObject (AI|GetBlackboard 0) (Utilities|Name|MakeLiteralName "Target") 0))))))

(event EventBeginPlay
  (AI|RunBehaviorTree "/Game/Tech/Blueprints/AI/Enemy/BT_Enemy.BT_Enemy"))

(fn ConstructionScript)