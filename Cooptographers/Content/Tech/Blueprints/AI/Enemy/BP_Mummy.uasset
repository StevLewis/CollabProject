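; BP_Mummy is a mummy enemy that growls periodically and shoves pawns to deal damage.
; On BeginPlay it starts a self-repeating Growl event that plays the mummy sound, then waits a random delay before growling again.
; Attack plays a shove montage and sound, box-traces a short way forward for a pawn and sends it a damage-by-type message.
; A DoOnce that resets after a short delay limits the attack rate.
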(event Custom|Growl
  (Audio|SpawnSoundAttached "/Game/Tech/Sounds/Cues/SC_Mummy.SC_Mummy" (Variables|Default|GetCapsuleComponent) "None" (Transformation|GetActorLocation) "0, 0, 0" "SnapToTarget" false 1.0 1.0 0.0 "/Game/Tech/Sounds/SA_DefaultAttentuation.SA_DefaultAttentuation" 0)
  (Utilities|FlowControl|Delay (Math|Random|RandomFloatinRange 0.0 1e+01))
  (CallFunction|Growl))

(event EventBeginPlay
  (CallFunction|Growl))

(event EventAttack
  (bind _returnvalue (Transformation|GetActorLocation))
  (Utilities|FlowControl|DoOnce false :!label _label
    (:Completed
      (Animation|PlayAnimMontage "/Game/Tech/Blueprints/Animation/Actions/AM_Shove.AM_Shove" 1.0 "None")
      (Audio|SpawnSoundAttached "/Game/Tech/Sounds/Cues/SC_Mummy.SC_Mummy" (Variables|Default|GetCapsuleComponent) "None" (Transformation|GetActorLocation) "0, 0, 0" "SnapToTarget" false 1.0 1.0 0.0 "/Game/Tech/Sounds/SA_DefaultAttentuation.SA_DefaultAttentuation" 0)
      (bind (_outhit _returnvalue_2) (Class|KismetSystemLibrary|BoxTraceSingleforObjects _returnvalue (+ _returnvalue (* (Transformation|GetActorForwardVector) 1e+02)) "20.000000,20.000000,20.000000" (Transformation|GetActorRotation) (Utilities|Array|MakeArray "ObjectTypeQuery3") false 0 "None" true))
      (if _returnvalue_2
        (Class|BPIDamage|ApplyDamagebyType(Message) (.HitActor (Collision|BreakHitResult _outhit)) 1.0 self "NewEnumerator0"))
      (Utilities|FlowControl|Delay 2.0)
      (goto _label Reset))))

(fn ConstructionScript
  (|CallParentFunction))