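; Slime enemy character that moves in a continuous bounce and sacrifices itself when its attack connects.
; BeginPlay launches it upward, and each landing plays the slime sound, then relaunches it after a short delay.
; Attack, which is not called within this graph, box-traces just ahead for a Pawn.
; On a hit it plays the sound, sends SlimeMessage to that actor and destroys itself.
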(event EventAttack
  (bind _returnvalue (Transformation|GetActorLocation))
  (bind (_outhit _returnvalue_2) (Class|KismetSystemLibrary|BoxTraceSingleforObjects _returnvalue (+ _returnvalue (* (Transformation|GetActorForwardVector) 1e+02)) "20.000000,20.000000,20.000000" (Transformation|GetActorRotation) (Utilities|Array|MakeArray "ObjectTypeQuery3") false 0 "None" true))
  (if _returnvalue_2
    (Audio|SpawnSoundAttached "/Game/Tech/Sounds/Cues/SC_Slime.SC_Slime" (Variables|Default|GetCapsuleComponent) "None" (Transformation|GetActorLocation) "0, 0, 0" "SnapToTarget" false 1.0 1.0 0.0 "/Game/Tech/Sounds/SA_DefaultAttentuation.SA_DefaultAttentuation" 0)
    (Class|BPIActions|Slime(Message) (.HitActor (Collision|BreakHitResult _outhit)))
    (Actor|DestroyActor)))

(event EventBeginPlay
  (Character|LaunchCharacter "0, 0,400.000000" false false))

(event EventOnLanded
  (params (Hit :type Hit%20Result%20Structure%20%28by%20ref%29))
  (Audio|SpawnSoundAttached "/Game/Tech/Sounds/Cues/SC_Slime.SC_Slime" (Variables|Default|GetCapsuleComponent) "None" (Transformation|GetActorLocation) "0, 0, 0" "SnapToTarget" false 1.0 1.0 0.0 "/Game/Tech/Sounds/SA_DefaultAttentuation.SA_DefaultAttentuation" 0)
  (Utilities|FlowControl|Delay 0.2)
  (Character|LaunchCharacter "0, 0,400.000000" false false))

(fn ConstructionScript
  (|CallParentFunction))