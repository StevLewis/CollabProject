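; Base player character for class-based (Mage, Scout) play, handling camera-relative movement, interaction, class equipment restored from the game instance, and death.
; Actions like interact, shove, whistle and help requests share a CanPerform gate, locking movement during montages or timers.
; Traces drive interaction, pushing, shoving and ledge pitfalls; slime inverts controls until removed, such as by a shove.
; Damage types and hard landings trigger death effects, montages or skeleton-spawning ragdoll, then timed respawn.
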(event Custom|MoveTo
  (params (Destination :type Vector) (ControllerOverwrite :type Controller%20Object%20Reference))
  ;[1 1 1] Move
  (AI|AIMoveTo self Destination 0 1e+01 false
    (:OnSuccess
      (Utilities|IsValid ControllerOverwrite
        (:Is%20Valid
          (Pawn|Possess ControllerOverwrite self))))))

(event Custom|Init
  (params (Player :type E_Player%20Enum :default "NewEnumerator1") (PlayerController :type BP%20Player%20Controller%20Object%20Reference))
  ;[1 1 1] Init
  (Variables|Player|SetPlayerIndex Player)
  (Variables|Default|SetPlayerController PlayerController)
  (Stats|SetupStats)
  (CallFunction|InitGameInstance)
  (Widgets|InitWidgets)
  (Variables|Default|SetGamemode (.AsGM%20Gameplay (Utilities|Casting|CastToGM_Gameplay (Game|GetGameMode))))
  (CallFunction|UpdateEquipment)
  (Utilities|Time|SetTimerbyEvent (EventDispatchers|CreateEvent :!event PushingCheck) 0.1 true))

(event Custom|RemoveSlime
  ;[1 1 1] Slime
  (Variables|Status|SetSlimeOnHead? false)
  (Rendering|SetVisibility (Variables|Default|GetSlimeMesh) false false)
  (Audio|Components|Audio|Stop (Variables|Default|GetSlimeOnHeadSFX)))

(event Custom|UpdateEquipment
  ;[1 1 1] Pickup / Equip class equipment
  (if (Variables|Equipment|GetHasClassEquipment?)
    (Variables|Default|SetPerformingAction? true)
    (bind _returnvalue (Animation|PlayAnimMontage "/Game/Tech/Blueprints/Animation/Actions/AM_Equip.AM_Equip" 2.0 "None"))
    (Rendering|SetVisibility (Variables|Default|GetEquipmentMesh) true true)
    (Utilities|FlowControl|Delay (/ _returnvalue 2.0))
    (Variables|Default|SetPerformingAction? false)))

(event Custom|PickupEquipment
  (bind _gameinstance (Variables|Components|GetGameInstance))
  ;[1 1 1] Pickup / Equip class equipment
  (Variables|Equipment|SetHasClassEquipment? true)
  (CallFunction|UpdateEquipment)
  (switch Utilities|FlowControl|Switch|SwitchonE_Class (Variables|Default|GetClass)
    (:NewEnumerator1
      (Default|SaveMageEquipment _gameinstance (Variables|Equipment|GetHasClassEquipment?)))
    (:NewEnumerator0
      (Default|SaveScoutEquipment _gameinstance (Variables|Equipment|GetHasClassEquipment?)))))

(event EventOnWalkingOffLedge
  (params (PreviousFloorImpactNormal :type Vector%20%28by%20ref%29 :default "0, 0, 0") (PreviousFloorContactNormal :type Vector%20%28by%20ref%29 :default "0, 0, 0") (PreviousLocation :type Vector%20%28by%20ref%29 :default "0, 0, 0") (TimeDelta :type Float%20%28single-precision%29))
  ;[1 1 1] Special Fall
  (bind _floorhit_ (CallFunction|FloorTrace))
  (if (not _floorhit_)
    (if (not (Variables|Status|GetSpecialFalling?))
      (Pawn|Components|CharacterMovement|SetMovementMode (Variables|Character|GetCharacterMovement) "MOVE_Flying" 0)
      (Variables|Status|SetSpecialFalling? true)
      (Variables|Default|SetPerformingAction? true)
      (bind _returnvalue (Animation|PlayAnimMontage "/Game/Tech/Blueprints/Animation/Actions/AM_Pitfall.AM_Pitfall" 1.0 "None"))
      (Utilities|FlowControl|Delay 0.2)
      (Pawn|Components|CharacterMovement|DisableMovement (Variables|Character|GetCharacterMovement))
      (Utilities|FlowControl|Delay (* _returnvalue 0.8))
      (Pawn|Components|CharacterMovement|SetMovementMode (Variables|Character|GetCharacterMovement) "MOVE_Walking" 0)
      (Variables|Default|SetPerformingAction? false))))

(event EventSlime
  ;[1 1 1] Slime
  (Variables|Status|SetSlimeOnHead? true)
  (Rendering|SetVisibility (Variables|Default|GetSlimeMesh) true false)
  (bind _spawnedsound (CallFunction|SpawnSoundAttached "/Game/Tech/Sounds/Cues/SC_SlimeOnHead.SC_SlimeOnHead"))
  (Variables|Default|SetSlimeOnHeadSFX _spawnedsound))

(event EventTick
  (params (DeltaSeconds :type Float%20%28single-precision%29))
  (bind _helpwidget (Variables|Default|GetHelpWidget))
  ;[1 1 1] Event Tick
  (Transformation|SetWorldRotation _helpwidget (Math|Rotator|FindLookatRotation (Transformation|GetWorldLocation _helpwidget) (Transformation|GetWorldLocation (Variables|/Script/Engine.PlayerCameraManager|GetTransformComponent (Game|GetPlayerCameraManager 0)))) false false)
  (if (Utilities|IsFalling?)
    (Variables|Default|SetFallSpeed (CallFunction|GetFallSpeed))))

(event EventOnLanded
  (params (Hit :type Hit%20Result%20Structure%20%28by%20ref%29))
  ;[1 1 1] Special Fall
  (if (> (Variables|Default|GetFallSpeed) 5e+02)
    (Damage|Death "NewEnumerator0")
    (if (Variables|Status|GetSpecialFalling?)
      (Variables|Status|SetSpecialFalling? false))
    (else
      (Variables|Default|SetFallSpeed 0.0))))

(event EventApplyDamagebyType
  (params (Damage :type Float%20%28single-precision%29) (DamageCauser :type Actor%20Object%20Reference) (DamageType :type E_DamageTypes%20Enum :default "NewEnumerator0"))
  ;[0.001723 0.1094 0] Damage
  (Damage|Death DamageType))

(event Input|KeyboardEvents|1
  (params (Key :type Key%20Structure))
  ;[1 0 0] Debug
  (:Pressed
    (Class|BPISwitch|SwitchCharacters(Message) (Game|GetGameMode))))

(event Input|AxisEvents|InputAxisMoveForwardBack
  (params (AxisValue :type Float%20%28single-precision%29))
  ;[1 1 1] Movement
  (bind _output_get (Variables|Control|SetForward/BackAxis AxisValue))
  (Pawn|Input|AddMovementInput (Math|Vector|GetForwardVector (Utilities|GetCameraRotation)) (select (Variables|Status|GetSlimeOnHead?) (* _output_get -1.0) _output_get) false))

(event Input|AxisEvents|InputAxisMoveRightLeft
  (params (AxisValue :type Float%20%28single-precision%29))
  ;[1 1 1] Movement
  (bind _output_get (Variables|Control|SetRight/LeftAxis AxisValue))
  (Pawn|Input|AddMovementInput (Math|Vector|GetRightVector (Utilities|GetCameraRotation)) (select (Variables|Status|GetSlimeOnHead?) (* _output_get -1.0) _output_get) false))

(event EventLevitatefor
  (params (LevitationTime :type Float%20%28single-precision%29))
  ;[1 1 1] Levitation
  (Variables|Default|SetLevitating? true)
  (Physics|AddForce (Variables|Character|GetCharacterMovement) "0, 0,100.000000")
  (Variables|/Script/Engine.CharacterMovementComponent|SetGravityScale (Variables|Character|GetCharacterMovement) 0.0)
  (Utilities|FlowControl|Delay LevitationTime)
  (Variables|Default|SetLevitating? false)
  (Variables|/Script/Engine.CharacterMovementComponent|SetGravityScale (Variables|Character|GetCharacterMovement) 1.0))

(event Input|ActionEvents|InputActionWhistle
  (params (Key :type Key%20Structure))
  ;[1 1 1] Whistle
  (:Pressed
    (Whistle|StartWhistling)))

(event Input|ActionEvents|InputActionInteract
  (params (Key :type Key%20Structure))
  ;[1 1 1] Interact
  (:Pressed
    (Interact|StartInteract)))

(event Input|ActionEvents|InputActionHelp
  (params (Key :type Key%20Structure))
  ;[1 1 1] Help
  (:Pressed
    (Variables|Help|SetHelpHeld? true)
    (Help|StartAskingforHelp))
  (:Released
    (Variables|Help|SetHelpHeld? false)
    (if (Class|KismetSystemLibrary|TimerExistsHandle (Variables|Help|GetHelpTH))
      (Utilities|Time|SetTimerbyEvent (EventDispatchers|CreateEvent :!event StopAskingforHelp) (Utilities|Time|GetTimerRemainingTimebyHandle (Variables|Help|GetHelpTH))))))

(event Input|ActionEvents|InputActionClue
  (params (Key :type Key%20Structure))
  ;[1 1 1] Clue
  (:Pressed
    (CallFunction|UpdateDialogueText (Variables|Clue|GetClueText) (Variables|Clue|GetClueTime))))

(event Input|ActionEvents|InputActionShove
  (params (Key :type Key%20Structure))
  ;[1 1 1] Shove
  (:Pressed
    (Shove|StartShove)))

(fn ConstructionScript)

(fn SetupStats
  (Variables|/Script/Engine.CharacterMovementComponent|SetMaxWalkSpeed (Variables|Character|GetCharacterMovement) (Variables|Stats|GetMoveSpeed))
  (Variables|Default|SetPlayerRotationRate (Variables|/Script/Engine.CharacterMovementComponent|GetRotationRate (Variables|Character|GetCharacterMovement))))

(fn Death
  (params (DamageType :type E_DamageTypes%20Enum :default "NewEnumerator0"))
  (bind _mesh (Variables|Character|GetMesh))
  (LocalVariables|SetDamageType%20%28local%29 DamageType)
  (if (not (Variables|Damage|GetDead?))
    (Utilities|FlowControl|Sequence
      (:then_0
        (Variables|Damage|SetDead? true)
        (Pawn|Components|CharacterMovement|DisableMovement (Variables|Character|GetCharacterMovement)))
      (:then_1
        (CallFunction|SpawnSoundAttached (Utilities|Select :Index (LocalVariables|GetDamageType%20%28local%29) :NewEnumerator0 "/Game/Tech/Sounds/Cues/SC_Death.SC_Death" :NewEnumerator1 "/Game/Design/SFX/Death-SpikeTrap.Death-SpikeTrap" :NewEnumerator2 "/Game/Design/SFX/Death-Burning.Death-Burning" :NewEnumerator3 "/Game/Design/SFX/Death-Electricity.Death-Electricity" :NewEnumerator5 "/Game/Tech/Sounds/Cues/SC_Death_Crushing.SC_Death_Crushing"))
        (switch Utilities|FlowControl|Switch|SwitchonE_DamageTypes (LocalVariables|GetDamageType%20%28local%29)
          (:NewEnumerator0
            (Effects|SpawnEmitterAttached "/Game/VFX-Merged/VFX_BloodSplat.VFX_BloodSplat" _mesh "pelvis" "0, 0, 0" "0, 0, 0" "1.000000,1.000000,1.000000" "SnapToTarget" :!label _label))
          (:NewEnumerator1
            (goto _label))
          (:NewEnumerator2
            (Niagara|SpawnSystemAttached "/Game/Tech/FX/PS_Fire.PS_Fire" _mesh "pelvis" "0, 0, 0" "0, 0, 0" "SnapToTarget" false))
          (:NewEnumerator3
            (goto _label))
          (:NewEnumerator5
            (goto _label)))
        (if (or (Utilities|Enum|Equal(Enum) (LocalVariables|GetDamageType%20%28local%29) "NewEnumerator0") (Utilities|Enum|Equal(Enum) (LocalVariables|GetDamageType%20%28local%29) "NewEnumerator5"))
          (CallFunction|Ragdoll)
          (else
            (bind _returnvalue (Animation|PlayAnimMontage (Utilities|Select :Index (LocalVariables|GetDamageType%20%28local%29) :NewEnumerator0 0 :NewEnumerator1 "/Game/Tech/Blueprints/Animation/Death/AM_Death_Spikes.AM_Death_Spikes" :NewEnumerator2 "/Game/Tech/Blueprints/Animation/Death/AM_Death_Burn.AM_Death_Burn" :NewEnumerator3 "/Game/Tech/Blueprints/Animation/Death/AM_Death_Electric.AM_Death_Electric" :NewEnumerator5 0) 1.0 "None"))
            (Variables|Stats|Spawn|SetRespawnTime (+ _returnvalue 1.0))
            (Utilities|Time|SetTimerbyEvent (EventDispatchers|CreateEvent :!event Ragdoll) _returnvalue))))
      (:then_2
        (Utilities|Time|SetTimerbyEvent (EventDispatchers|CreateEvent :!event Respawn) (Variables|Stats|Spawn|GetRespawnTime))))))

(fn SetWalking
  (Pawn|Components|CharacterMovement|SetMovementMode (Variables|Character|GetCharacterMovement) "MOVE_Walking" 0))

(fn InteractWidgetCheck
  (Utilities|IsValid (Interact|InteractTrace)
    (:Is%20Valid
      (if (not (Widget|IsVisible (Variables|Interact|GetInteractPopup)))
        (Default|ShowPopup (Variables|Interact|GetInteractPopup))))
    (:Is%20Not%20Valid
      (if (Widget|IsVisible (Variables|Interact|GetInteractPopup))
        (Default|HidePopup (Variables|Interact|GetInteractPopup))))))

(fn InteractTrace
  (bind _hits (CallFunction|ConeTrace 2e+01 2e+01 2e+01 2e+01))
  (for _array_element _hits
    (if (Utilities|DoesObjectImplementInterface (.HitActor (Collision|BreakHitResult _array_element)) "/Game/Tech/Blueprints/Characters/BPI_Interact.BPI_Interact_C")
      (bind _interactable_ (Class|BPIInteract|GetInteractable?(Message) (.HitActor (Collision|BreakHitResult _array_element))))
      (if _interactable_
        (return (.HitActor (Collision|BreakHitResult _array_element))))))
  (return 0))

(fn StartInteract
  (bind _interactable (Interact|InteractTrace))
  (if (Checks|CanPerform?)
    (Utilities|IsValid _interactable
      (:Is%20Valid
        (Class|BPIInteract|Interact(Message) _interactable self)
        (bind _returnvalue (Animation|PlayAnimMontage "/Game/Tech/Blueprints/Animation/Actions/AM_Interact.AM_Interact" 1.0 "None"))
        (Variables|Default|SetPerformingAction? true)
        (Pawn|Components|CharacterMovement|DisableMovement (Variables|Character|GetCharacterMovement))
        (Utilities|Time|SetTimerbyEvent (EventDispatchers|CreateEvent :!event StopPerformingAction) _returnvalue)))))

(fn InitHelpWidget
  (if (Variables|Help|GetHelpHeld?)
    (Class|BPIInit|Init(Message) (UserInterface|GetWidget (Variables|Default|GetHelpWidget)))))

(fn StartAskingforHelp
  (if (Checks|CanPerform?)
    (if (not (Class|KismetSystemLibrary|TimerExistsHandle (Variables|Help|GetHelpTH)))
      (Variables|Default|SetPerformingAction? true)
      (Variables|Help|SetRequestingHelp? true)
      (Pawn|Components|CharacterMovement|DisableMovement (Variables|Character|GetCharacterMovement))
      (Help|InitHelpWidget)
      (bind _returnvalue (Utilities|Time|SetTimerbyEvent (EventDispatchers|CreateEvent :!event InitHelpWidget) 1.0 true))
      (Variables|Help|SetHelpTH _returnvalue))))

(fn StopAskingforHelp
  (if (Variables|Help|GetRequestingHelp?)
    (Variables|Help|SetRequestingHelp? false)
    (Utilities|Time|ClearandInvalidateTimerbyHandle (Variables|Help|GetHelpTH))
    (CallFunction|StopPerformingAction)))

(fn FloorTrace
  (bind _returnvalue (Transformation|GetActorLocation))
  (bind _capsulecomponent (Variables|Collision|GetCapsuleComponent))
  (bind _returnvalue_2 (Components|Capsule|GetScaledCapsuleHalfHeight _capsulecomponent))
  (bind _returnvalue_3 (- _returnvalue (Math|Vector|MakeVector 0.0 0.0 _returnvalue_2)))
  (bind _returnvalue_4 (Class|KismetSystemLibrary|CapsuleTraceMultiforObjects _returnvalue_3 _returnvalue_3 75.0 1e+02 (Utilities|Array|MakeArray "ObjectTypeQuery1" "ObjectTypeQuery2") false (Utilities|Array|MakeArray self) "None" true))
  (return _returnvalue_4))

(fn Respawn
  (Default|CallHasDied))

(fn InitWidgets
  (bind _aswb_interact_popup (Utilities|Casting|CastToWB_InteractPopup (UserInterface|GetWidget (Variables|Default|GetInteractPopupWidget))))
  (bind _output_get (Variables|Interact|SetInteractPopup _aswb_interact_popup))
  (Default|Init _output_get self)
  (Utilities|Time|SetTimerbyEvent (EventDispatchers|CreateEvent :!event InteractWidgetCheck) 0.1 true))

(fn IsGrounded?
  (return (and (not (AI|Components|NavMovement|IsFalling (Variables|Character|GetCharacterMovement))) (not (Class|NavMovementComponent|IsFlying (Variables|Character|GetCharacterMovement))))))

(fn CanPerform?
  (return (Math|Boolean|ANDBoolean (Checks|IsGrounded?) (not (Variables|Default|GetPerformingAction?)) (not (Variables|Damage|GetDead?)))))

(fn InitGameInstance
  (bind _output_get (Variables|Components|SetGameInstance (.AsBP%20Game%20Instance (Utilities|Casting|CastToBP_GameInstance (Game|GetGameInstance)))))
  (bind (_magestaffenabled_ _scoutlassoenabled_) (Default|LoadEquipment _output_get))
  (switch Utilities|FlowControl|Switch|SwitchonE_Class (Variables|Default|GetClass)
    (:NewEnumerator1
      (Variables|Equipment|SetHasClassEquipment? _magestaffenabled_))
    (:NewEnumerator0
      (Variables|Equipment|SetHasClassEquipment? _scoutlassoenabled_))))

(fn UpdateDialogueText
  (params (DialogueText :type Text) (DialogueTime :type Float%20%28single-precision%29))
  (Variables|Dialogue|SetDialogueText DialogueText)
  (Variables|Dialogue|SetDialogueTime DialogueTime)
  (Default|CallDialogueTextModified))

(fn GetFallSpeed
  (bind _returnvalue (Transformation|GetVelocity))
  (return (Math|Float|Absolute(Float) (Math|Float|SelectFloat (.z _returnvalue) 0.0 (< (.z _returnvalue) 0.0)))))

(fn PushingCheck
  (Utilities|IsValid (Push|PushingTrace)
    (:Is%20Valid
      (Push|StartPushing))
    (:Is%20Not%20Valid
      (Push|StopPushing))))

(fn PushingTrace
  (bind _returnvalue (Transformation|GetActorLocation))
  (bind (_outhits _returnvalue_2) (Class|KismetSystemLibrary|BoxTraceMultiforObjects _returnvalue (+ _returnvalue (* (Transformation|GetActorForwardVector) (Variables|Interact|GetInteractRange))) "0.000000,20.000000,50.000000" (Transformation|GetActorRotation) (Utilities|Array|MakeArray "ObjectTypeQuery8") false 0 "None" true "(R=1.000000,G=0.000000,B=0.000000,A=1.000000)" "(R=0.000000,G=1.000000,B=0.000000,A=1.000000)" 0.1))
  (if _returnvalue_2
    (for _array_element _outhits
      (if (Utilities|DoesObjectImplementInterface (.HitActor (Collision|BreakHitResult _array_element)) "/Game/Tech/Blueprints/Placeables/PushableObjects/BPI_Pushable.BPI_Pushable_C")
        (return (.HitActor (Collision|BreakHitResult _array_element)))))
    (return 0)
    (else
      (return 0))))

(fn StartPushing
  (if (not (Variables|Push|GetPushing?))
    (Variables|Push|SetPushing? true)
    (bind _spawnedsound (CallFunction|SpawnSoundAttached "/Game/Tech/Sounds/Cues/SC_PushBlock.SC_PushBlock"))
    (Variables|Default|SetPushSFX _spawnedsound)
    (Variables|/Script/Engine.CharacterMovementComponent|SetMaxWalkSpeed (Variables|Character|GetCharacterMovement) (/ (Variables|Stats|GetMoveSpeed) 2.0))
    (Components|Capsule|SetCapsuleRadius (Variables|Collision|GetCapsuleComponent) 8e+01 true)
    (Pawn|Components|CharacterMovement|DisableMovement (Variables|Character|GetCharacterMovement))
    (Utilities|Time|SetTimerbyEvent (EventDispatchers|CreateEvent :!event SetWalking) 0.2)))

(fn StopPushing
  (if (Variables|Push|GetPushing?)
    (Variables|Push|SetPushing? false)
    (Audio|Components|Audio|Stop (Variables|Default|GetPushSFX))
    (Variables|/Script/Engine.CharacterMovementComponent|SetMaxWalkSpeed (Variables|Character|GetCharacterMovement) (Variables|Stats|GetMoveSpeed))
    (Components|Capsule|SetCapsuleRadius (Variables|Collision|GetCapsuleComponent) 4e+01 true)))

(fn StartWhistling
  (if (Checks|CanPerform?)
    (Variables|Default|SetPerformingAction? true)
    (bind _returnvalue (Animation|PlayAnimMontage "/Game/Tech/Blueprints/Animation/Actions/AM_Whistle.AM_Whistle" 2.0 "None"))
    (Utilities|Time|SetTimerbyEvent (EventDispatchers|CreateEvent :!event StopPerformingAction) (/ _returnvalue 2.0))
    (Audio|PlaySoundatLocation "/Game/Tech/Sounds/Cues/Whistle/TwoWhistle.TwoWhistle" (Transformation|GetActorLocation) "0, 0, 0" 1.0 1.0 0.0 0 0 0)
    (Default|WhistlePause (Variables|Default|GetGamemode) 2.0)
    (Pawn|Components|CharacterMovement|DisableMovement (Variables|Character|GetCharacterMovement))))

(fn StopPerformingAction
  (Variables|Default|SetPerformingAction? false)
  (MovementMode|SetWalking))

(fn CooldownShove
  (Variables|Shove|SetShoveOnCooldown? false))

(fn StartShove
  (bind _returnvalue (Transformation|GetActorLocation))
  (bind _returnvalue_2 (Transformation|GetActorForwardVector))
  (bind _shoveforce (Variables|Shove|GetShoveForce))
  (if (Checks|CanPerform?)
    (if (not (Variables|Shove|GetShoveOnCooldown?))
      (Variables|Shove|SetShoveOnCooldown? true)
      (Utilities|Time|SetTimerbyEvent (EventDispatchers|CreateEvent :!event CooldownShove) (Variables|Shove|GetShoveCooldownTime))
      (Variables|Default|SetPerformingAction? true)
      (CallFunction|SpawnSoundAttached "/Game/Tech/Sounds/Cues/SC_Shove.SC_Shove")
      (bind _returnvalue_3 (Animation|PlayAnimMontage "/Game/Tech/Blueprints/Animation/Actions/AM_Shove.AM_Shove" 1.0 "None"))
      (Utilities|Time|SetTimerbyEvent (EventDispatchers|CreateEvent :!event StopPerformingAction) _returnvalue_3)
      (Pawn|Components|CharacterMovement|DisableMovement (Variables|Character|GetCharacterMovement))
      (bind _outhit (Collision|LineTraceForObjects _returnvalue (+ _returnvalue (* (Transformation|GetActorForwardVector) 1e+02)) (Utilities|Array|MakeArray "ObjectTypeQuery3") false 0 "None"))
      (bind _asbp_base_character (Utilities|Casting|CastToBP_BaseCharacter (.HitActor (Collision|BreakHitResult _outhit))))
      (Character|LaunchCharacter _asbp_base_character (Math|Vector|MakeVector (* (.x _returnvalue_2) _shoveforce) (* (.y _returnvalue_2) _shoveforce) 3e+02) false false)
      (CallFunction|RemoveSlime _asbp_base_character))))

(fn Ragdoll
  (bind _mesh (Variables|Character|GetMesh))
  (bind _mesh_2 (Variables|Character|GetMesh))
  (bind _returnvalue (Transformation|GetWorldTransform _mesh))
  (Physics|SetSimulatePhysics _mesh_2 true)
  (Collision|SetCollisionEnabled _mesh_2 "QueryAndPhysics")
  (Rendering|SetVisibility _mesh false false)
  (bind _returnvalue_2 (Game|SpawnActorfromClass "/Game/Art/CharacterArt/Skeleton/BP_Skeleton.BP_Skeleton_C" (Math|Transform|MakeTransform (.location _returnvalue) (.rotation _returnvalue) "1,1,1") "AdjustIfPossibleButAlwaysSpawn" 0 0))
  (Default|OnSpawned _returnvalue_2))

(fn ConeTrace
  (params (ConeLength :type Float%20%28single-precision%29) (ConeRadius :type Float%20%28single-precision%29) (LengthIncrease :type Float%20%28single-precision%29) (RadiusIncrease :type Float%20%28single-precision%29))
  (LocalVariables|SetLength%20%28local%29 ConeLength)
  (LocalVariables|SetRadius%20%28local%29 ConeRadius)
  (LocalVariables|SetLengthIncrease%20%28local%29 LengthIncrease)
  (LocalVariables|SetRadiusIncrease%20%28local%29 RadiusIncrease)
  (for _index (range 0 2)
    (bind _outhits (Collision|MultiSphereTraceForObjects (+ (Transformation|GetActorLocation) (* (Transformation|GetActorForwardVector) (LocalVariables|GetLength%20%28local%29))) (+ (Transformation|GetActorLocation) (* (Transformation|GetActorForwardVector) (LocalVariables|GetLength%20%28local%29))) (LocalVariables|GetRadius%20%28local%29) (Utilities|Array|MakeArray "ObjectTypeQuery2" "ObjectTypeQuery3" "ObjectTypeQuery4" "ObjectTypeQuery5" "ObjectTypeQuery6") false 0 "None"))
    (for _array_element _outhits
      (Utilities|Array|Add (LocalVariables|GetHits%20%28local%29) _array_element))
    (LocalVariables|SetLength%20%28local%29 (+ (LocalVariables|GetLength%20%28local%29) (LocalVariables|GetLengthIncrease%20%28local%29)))
    (LocalVariables|SetRadius%20%28local%29 (+ (LocalVariables|GetRadius%20%28local%29) (LocalVariables|GetRadiusIncrease%20%28local%29))))
  (return (LocalVariables|GetHits%20%28local%29)))

(fn SpawnSoundAttached
  (params (Sound :type Sound%20Base%20Object%20Reference))
  (bind _returnvalue (Audio|SpawnSoundAttached Sound (Variables|Collision|GetCapsuleComponent) "None" (Transformation|GetActorLocation) "0, 0, 0" "SnapToTarget" false 1.0 1.0 0.0 "/Game/Tech/Sounds/SA_DefaultAttentuation.SA_DefaultAttentuation" 0))
  (return _returnvalue))