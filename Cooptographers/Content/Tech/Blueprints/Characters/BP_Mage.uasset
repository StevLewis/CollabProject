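; BP_Mage is the mage character, whose equipment input casts a staff spell that levitates a target.
; Casting plays a sped-up montage with sound and locks movement, with timers at its midpoint and end, apparently for triggering levitation and restoring walking.
; Levitation runs a cone trace and messages the first hit actor implementing BPI_Actions to levitate briefly.
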(event Input|ActionEvents|InputActionEquipment
  (params (Key :type Key%20Structure :default "None"))
  ;[1 1 1] Mage Equipment
  (:Pressed
    (if (Variables|Default|GetHasClassEquipment?)
      (Staff|StartUsingStaff))))

(fn ConstructionScript
  (|CallParentFunction))

(fn StartUsingStaff
  (if (CallFunction|CanPerform?)
    (Audio|SpawnSoundAttached "/Game/Tech/Sounds/Cast1.Cast1" (Variables|Default|GetCapsuleComponent) "None" "0, 0, 0" "0, 0, 0" "SnapToTarget" false 1.0 1.0 0.0 "/Game/Tech/Sounds/SA_DefaultAttentuation.SA_DefaultAttentuation" 0)
    (bind _returnvalue (Animation|PlayAnimMontage "/Game/Tech/Blueprints/Animation/Actions/AM_StaffCast.AM_StaffCast" 2.0 "None"))
    (Utilities|FlowControl|Sequence
      (:then_0
        (Variables|Default|SetPerformingAction? true)
        (Pawn|Components|CharacterMovement|DisableMovement (Variables|Character|GetCharacterMovement))
        (Utilities|Time|SetTimerbyEvent (EventDispatchers|CreateEvent :!event StopUsingStaff) (/ _returnvalue 2.0)))
      (:then_1
        (Utilities|Time|SetTimerbyEvent (EventDispatchers|CreateEvent :!event TriggerLevitation) (* (/ _returnvalue 2.0) 0.5))))))

(fn StopUsingStaff
  (Variables|Default|SetPerformingAction? false)
  (CallFunction|SetWalking))

(fn TriggerLevitation
  (bind _hits (CallFunction|ConeTrace 5e+01 3e+01 5e+01 3e+01))
  (bind _array_element (Utilities|Array|ForEachLoopwithBreak _hits)
    (:LoopBody
      (if (Utilities|DoesObjectImplementInterface (.HitActor (Collision|BreakHitResult _array_element)) "/Game/Tech/Blueprints/Characters/BPI_Actions.BPI_Actions_C")
        (Class|BPIActions|Levitatefor(Message) (.HitActor (Collision|BreakHitResult _array_element)) 5.0)
        (return)))))