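; BP_Scout is the Scout character Blueprint, whose equipment input throws a lasso when the class equipment is held.
; The throw plays a montage, locks movement and uses timers, apparently to launch BP_LassoProj mid-animation and later restore walking.
; The projectile's destruction is bound to an event, likely spawning a reversed return projectile.
; A stick poke, not called here, box-traces ahead and messages BPI_Trigger actors.
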(event Input|ActionEvents|InputActionEquipment
  (params (Key :type Key%20Structure))
  ;[1 1 1] Scout Equipment
  (:Pressed
    (if (Variables|Default|GetHasClassEquipment?)
      (Lasso|StartUsingLasso))))

(fn ConstructionScript
  (|CallParentFunction))

(fn StartUsingStick
  (bind _returnvalue (Transformation|GetActorLocation))
  (Audio|PlaySound2D "/Game/Tech/Sounds/Poke1.Poke1" 1.0 1.0 0.0 0 0)
  (bind _returnvalue_2 (Animation|PlayAnimMontage "/Game/Tech/Blueprints/Animation/Actions/AM_Lasso.AM_Lasso" 2.0 "None"))
  (Utilities|FlowControl|Sequence
    (:then_0
      (Variables|Default|SetPerformingAction? true)
      (Pawn|Components|CharacterMovement|DisableMovement (Variables|Character|GetCharacterMovement))
      (Utilities|Time|SetTimerbyEvent (EventDispatchers|CreateEvent :!event FinishUsingStick) (/ _returnvalue_2 2.0)))
    (:then_1
      (bind (_outhits _returnvalue_3) (Class|KismetSystemLibrary|BoxTraceMultiforObjects _returnvalue (+ _returnvalue (* (Transformation|GetActorForwardVector) 2e+02)) "0.000000,50.000000,100.000000" "0, 0, 0" (Utilities|Array|MakeArray "ObjectTypeQuery1" "ObjectTypeQuery2" "ObjectTypeQuery3" "ObjectTypeQuery4" "ObjectTypeQuery5" "ObjectTypeQuery6") false (Utilities|Array|MakeArray self) "None" true))
      (if _returnvalue_3
        (bind _array_element (Utilities|Array|ForEachLoopwithBreak _outhits)
          (:LoopBody
            (if (Utilities|DoesObjectImplementInterface (.HitActor (Collision|BreakHitResult _array_element)) "/Game/Tech/Blueprints/Placeables/Triggers/BPI_Trigger.BPI_Trigger_C")
              (Class|BPITrigger|Trigger(Message) (.HitActor (Collision|BreakHitResult _array_element))))))))))

(fn FinishUsingStick
  (Variables|Default|SetPerformingAction? false)
  (CallFunction|SetWalking))

(fn Respawn
  (|CallParentFunction))

(fn StartUsingLasso
  (if (CallFunction|CanPerform?)
    (Audio|SpawnSoundAttached "/Game/Tech/Sounds/Cast1.Cast1" (Variables|Default|GetCapsuleComponent) "None" "0, 0, 0" "0, 0, 0" "SnapToTarget" false 1.0 1.0 0.0 "/Game/Tech/Sounds/SA_DefaultAttentuation.SA_DefaultAttentuation" 0)
    (bind _returnvalue (Animation|PlayAnimMontage "/Game/Tech/Blueprints/Animation/Actions/AM_Lasso.AM_Lasso" 2.0 "None"))
    (Utilities|FlowControl|Sequence
      (:then_0
        (Variables|Default|SetPerformingAction? true)
        (Pawn|Components|CharacterMovement|DisableMovement (Variables|Character|GetCharacterMovement))
        (Utilities|Time|SetTimerbyEvent (EventDispatchers|CreateEvent :!event StopUsingLasso) (/ _returnvalue 2.0)))
      (:then_1
        (Utilities|Time|SetTimerbyEvent (EventDispatchers|CreateEvent :!event TriggerLasso) (* (/ _returnvalue 2.0) 0.5))))))

(fn StopUsingLasso
  (Variables|Default|SetPerformingAction? false)
  (CallFunction|SetWalking))

(fn TriggerLasso
  (bind _returnvalue (Game|SpawnActorfromClass "/Game/Tech/Blueprints/Placeables/LassoableObjects/BP_LassoProj.BP_LassoProj_C" (Math|Transform|MakeTransform (+ (Transformation|GetActorLocation) (* (Transformation|GetActorForwardVector) 1e+02)) (Transformation|GetActorRotation) "2.000000,2.000000,2.000000") "AlwaysSpawn" 0 false 1.2e+03 0))
  (bind _output_get (Variables|Default|SetSpawnProj _returnvalue))
  (Game|BindEventtoOnDestroyed _output_get (EventDispatchers|CreateEvent :!event SpawnReturnProjectile)))

(fn SpawnReturnProjectile
  (params (DestroyedActor :type Actor%20Object%20Reference))
  (Game|SpawnActorfromClass "/Game/Tech/Blueprints/Placeables/LassoableObjects/BP_LassoProj.BP_LassoProj_C" (Math|Transform|MakeTransform (Transformation|GetActorLocation DestroyedActor) (Math|Conversions|RotationFromXVector (Math|Vector|NegateVector (Math|Rotator|GetRotationXVector (Transformation|GetActorRotation DestroyedActor)))) "2.000000,2.000000,2.000000") "AlwaysSpawn" 0 true 2.4e+03 0))