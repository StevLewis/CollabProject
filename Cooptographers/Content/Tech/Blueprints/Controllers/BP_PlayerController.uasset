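; Player controller that handles per-player setup, pausing and respawn signalling.
; Init stores the player index, game mode and character, and binds to the character's death event; RespawnCharacter fires the Respawn dispatcher.
; Pause toggles a lazily created WB_PauseMenu, game pause and input mode, changing cursor visibility only for Player 1.
; Holding Left Shift speeds up global time through a hard-wired key event.
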(event Custom|Init
  (params (Player :type E_Player%20Enum :default "NewEnumerator1") (Gamemode :type GM%20Gameplay%20Object%20Reference) (PlayerCharacter :type BP%20Base%20Character%20Object%20Reference))
  ;[1 1 1] Init
  (Variables|Default|SetPlayerIndex Player)
  (Variables|Default|SetGamemode Gamemode)
  (bind _output_get (Variables|Default|SetPlayerCharacter PlayerCharacter))
  (bind _playercharacter (Variables|Default|GetPlayerCharacter)
    (:then
      (EventDispatchers|BindEventtoHasDied _output_get (EventDispatchers|CreateEvent :!event RespawnCharacter)))
    (:else)))

(event Input|ActionEvents|InputActionPause
  (params (Key :type Key%20Structure :default "None"))
  ;[1 1 1] Pause
  (:Pressed
    (Variables|Default|GetPauseMenuRef
      (:then
        _)
      (:else
        (bind _returnvalue (UserInterface|CreateWidget "/Game/Tech/Blueprints/Widgets/Menus/WB_PauseMenu.WB_PauseMenu_C"))
        (Variables|Default|SetPauseMenuRef _returnvalue)))
    (if (Game|IsGamePaused)
      (Widget|RemovefromParent (Variables|Default|GetPauseMenuRef))
      (Game|SetGamePaused false)
      (Input|SetInputModeGameOnly self)
      (switch Utilities|FlowControl|Switch|SwitchonE_Player (Variables|Default|GetPlayerIndex)
        (:NewEnumerator1
          (Variables|/Script/Engine.PlayerController|SetbShowMouseCursor self false)))
      (else
        (UserInterface|Viewport|AddtoViewport (Variables|Default|GetPauseMenuRef) 0)
        (Game|SetGamePaused true)
        (Input|SetInputModeGameandUI self (Variables|Default|GetPauseMenuRef) "LockInFullscreen" false)
        (switch Utilities|FlowControl|Switch|SwitchonE_Player (Variables|Default|GetPlayerIndex)
          (:NewEnumerator1
            (Variables|/Script/Engine.PlayerController|SetbShowMouseCursor self true)))))))

(event Input|KeyboardEvents|LeftShift
  (params (Key :type Key%20Structure :default "None"))
  (:Pressed
    (Utilities|Time|SetGlobalTimeDilation 5.0))
  (:Released
    (Utilities|Time|SetGlobalTimeDilation 1.0)))

(fn ConstructionScript)

(fn RespawnCharacter
  (Default|CallRespawn))