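; Gameplay game mode for two local players as Mage or Scout, followed by an AI adventurer party's run toward the boss door.
; Init reads game-instance classes and level details, then creates controllers, HUDs, a round timer and characters at level markers.
; Players can swap characters or respawn.
; The end scene walks both to the stairs, drops player two and spawns randomly typed adventurers, whose surviving count and flag usage feed the score menu.
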(event Custom|Init
  ;[1 1 1] Setup
  (GameInstance|InitGameInstance) ; Check if any save data
  (Classes|InitDefaultClasses) ; If no valid class then set default
  (Controllers|InitControllers) ; Setup players
  (Widgets|InitWidgets)
  (Timer|InitRoundTimer)
  (StartPoints|InitStartPoints)
  (Characters|InitCharacters)
  (Goals|InitGoals)
  (AI|InitAISpawnPoint))

(event Custom|SpawnAIParty
  ;[1 1 1] AI
  (Variables|AI|SetTempAdventurerNames (Variables|AI|GetAdventurerNames))
  (for _index (range 0 (- (Variables|AI|GetAdventurePartyNumber) 1))
    (CallFunction|SpawnAICharacter _index))
  (for _array_element (Variables|AI|GetAICharacters)
    (EventDispatchers|BindEventtoOnDeath _array_element (EventDispatchers|CreateEvent :!event RemoveDeadAdventurer)))
  (Game|Player|SetViewTargetwithBlend (Variables|PlayerControllers|GetPlayer1Controller) (Utilities|Array|Get(acopy) (Variables|AI|GetAICharacters)) 5.0 "VTBlend_Linear" 0.0 false)
  (EventDispatchers|BindEventtoBossRoomReached (Utilities|Array|Get(acopy) (Variables|AI|GetAICharacters)) (EventDispatchers|CreateEvent :!event ShowScore))
  (Utilities|FlowControl|Delay 5.0)
  (for _array_element_2 (Variables|AI|GetAICharacters)
    (Default|Move _array_element_2)))

(event EventBeginPlay
  ;[0.001723 0.1094 0] Event Begin Play
  (CallFunction|Init))

(event EventSwitchCharacters
  ;[1 1 1] Switch Characters
  (CallFunction|CharacterSwitch))

(event EventActivateEndStairs
  ;[1 1 1] Goal
  (Default|ActivateTrigger (Variables|Goal|GetEndStairs)))

(event EventSetupEndScene
  ;[1 1 1] AI
  (Default|AnimationFadeOutin (Variables|Widgets|GetMainHud))
  (Utilities|FlowControl|Delay 0.2)
  (Pawn|Possess (Variables|PlayerAIControllers|GetPlayer1AIController) (Variables|Characters|GetPlayer1Character))
  (Pawn|Possess (Variables|PlayerAIControllers|GetPlayer2AIController) (Variables|Characters|GetPlayer2Character))
  (Utilities|FlowControl|Delay 0.1)
  (Game|Player|SetViewTargetwithBlend (Variables|PlayerControllers|GetPlayer1Controller) (Variables|Characters|GetPlayer1Character) 0.0 "VTBlend_Linear" 0.0 false)
  (Game|Player|SetViewTargetwithBlend (Variables|PlayerControllers|GetPlayer2Controller) (Variables|Characters|GetPlayer2Character) 0.0 "VTBlend_Linear" 0.0 false)
  (Default|Moveto (Variables|Characters|GetPlayer1Character) (Transformation|GetWorldLocation (Variables|/Game/Tech/Blueprints/Placeables/Goal/BP_EndStairs.BP_EndStairs_C|GetEndPoint (Variables|Goal|GetEndStairs))))
  (Default|Moveto (Variables|Characters|GetPlayer2Character) (Transformation|GetWorldLocation (Variables|/Game/Tech/Blueprints/Placeables/Goal/BP_EndStairs.BP_EndStairs_C|GetEndPoint (Variables|Goal|GetEndStairs))))
  (Utilities|FlowControl|Delay 1.0)
  (Default|AnimationFadeOutin (Variables|Widgets|GetMainHud))
  (Utilities|FlowControl|Delay 0.2)
  (Class|GameplayStatics|RemovePlayer (Variables|PlayerControllers|GetPlayer2Controller) false)
  (Input|SetInputModeUIOnly (Variables|PlayerControllers|GetPlayer1Controller) 0 "DoNotLock")
  (CallFunction|SpawnAIParty))

(event EventSetSpawnPoints
  (params (MageSpawnPoint :type Transform) (ScoutSpawnPoint :type Transform))
  ;[1 1 1] Set Spawn Points
  (Variables|SpawnPoints|SetMageSpawnTransform MageSpawnPoint)
  (Variables|SpawnPoints|SetScoutSpawnTransform ScoutSpawnPoint))

(fn ConstructionScript)

(fn InitStartPoints
  (bind _outactors (Actor|GetAllActorsOfClass "/Game/Tech/Blueprints/Placeables/Spawnpoints/BP_PlayerStart.BP_PlayerStart_C"))
  (LocalVariables|SetSpawnPoints%20%28local%29 _outactors)
  (bind _array_element (Utilities|Array|ForEachLoopwithBreak (LocalVariables|GetSpawnPoints%20%28local%29))
    (:LoopBody
      (switch Utilities|FlowControl|Switch|SwitchonE_Player (Variables|/Game/Tech/Blueprints/Placeables/Spawnpoints/BP_PlayerStart.BP_PlayerStart_C|GetPlayer _array_element)
        (:NewEnumerator1
          (Variables|SpawnPoints|SetPlayer1SpawnPoint (Transformation|GetWorldTransform (Variables|/Game/Tech/Blueprints/Placeables/Spawnpoints/BP_PlayerStart.BP_PlayerStart_C|GetSpawnPoint _array_element)))
          (Variables|SpawnPoints|SetPlayer1MoveToPoint (Variables|/Game/Tech/Blueprints/Placeables/Spawnpoints/BP_PlayerStart.BP_PlayerStart_C|GetMovePoint _array_element)))
        (:NewEnumerator0
          (Variables|SpawnPoints|SetPlayer2SpawnPoint (Transformation|GetWorldTransform (Variables|/Game/Tech/Blueprints/Placeables/Spawnpoints/BP_PlayerStart.BP_PlayerStart_C|GetSpawnPoint _array_element)))
          (Variables|SpawnPoints|SetPlayer2MoveToPoint (Variables|/Game/Tech/Blueprints/Placeables/Spawnpoints/BP_PlayerStart.BP_PlayerStart_C|GetMovePoint _array_element)))))))

(fn InitGameInstance
  (bind _output_get (Variables|Default|SetGameInstanceRef (.AsBP%20Game%20Instance (Utilities|Casting|CastToBP_GameInstance (Game|GetGameInstance)))))
  (bind (_player1class _player2class) (Default|GetClasses _output_get))
  (Variables|Classes|SetPlayer1Class _player1class)
  (Variables|Classes|SetPlayer2Class _player2class)
  (bind (_adventurepartynumber _leveldifficulty _levelflagpar) (Default|GetLevelDetails (Variables|Default|GetGameInstanceRef)))
  (Variables|AI|SetAdventurePartyNumber _adventurepartynumber)
  (Variables|Default|SetLevelDifficulty _leveldifficulty)
  (Variables|Default|SetLevelFlagPar _levelflagpar))

(fn InitControllers
  (bind _outactors (Actor|GetAllActorsOfClass "/Game/Tech/Blueprints/Controllers/BP_PlayerController.BP_PlayerController_C"))
  (for _array_element _outactors
    (Class|GameplayStatics|RemovePlayer _array_element false))
  (Utilities|FlowControl|Sequence
    (:then_0
      (bind _returnvalue (Class|GameplayStatics|CreatePlayer -1))
      (bind _output_get (Variables|PlayerControllers|SetPlayer1Controller (.AsBP%20Player%20Controller (Utilities|Casting|CastToBP_PlayerController _returnvalue))))
      (EventDispatchers|BindEventtoRespawn _output_get (EventDispatchers|CreateEvent :!event RespawnCharacters))
      (Input|SetInputModeGameOnly _output_get)
      (Default|Init _output_get "NewEnumerator1" self))
    (:then_1
      (bind _returnvalue_2 (Class|GameplayStatics|CreatePlayer -1))
      (bind _output_get_2 (Variables|PlayerControllers|SetPlayer2Controller (.AsBP%20Player%20Controller (Utilities|Casting|CastToBP_PlayerController _returnvalue_2))))
      (EventDispatchers|BindEventtoRespawn _output_get_2 (EventDispatchers|CreateEvent :!event RespawnCharacters))
      (Input|SetInputModeGameOnly _output_get_2)
      (Default|Init _output_get_2 "NewEnumerator0" self))))

(fn InitWidgets
  (Utilities|FlowControl|Sequence
    (:then_0
      (bind _returnvalue (UserInterface|CreateWidget "/Game/Tech/Blueprints/Widgets/WB_MainHud.WB_MainHud_C"))
      (bind _output_get (Variables|Widgets|SetMainHud _returnvalue))
      (UserInterface|Viewport|AddtoViewport _output_get 0)
      (Default|Init _output_get))
    (:then_1
      (bind _returnvalue_2 (UserInterface|CreateWidget "/Game/Tech/Blueprints/Widgets/WB_Player1Hud.WB_Player1Hud_C" (Variables|PlayerControllers|GetPlayer1Controller)))
      (bind _output_get_2 (Variables|Widgets|SetPlayer1MainHud _returnvalue_2))
      (UserInterface|Viewport|AddtoPlayerScreen _output_get_2))
    (:then_2
      (bind _returnvalue_3 (UserInterface|CreateWidget "/Game/Tech/Blueprints/Widgets/WB_Player2Hud.WB_Player2Hud_C" (Variables|PlayerControllers|GetPlayer2Controller)))
      (bind _output_get_3 (Variables|Widgets|SetPlayer2MainHud _returnvalue_3))
      (UserInterface|Viewport|AddtoPlayerScreen _output_get_3))))

(fn InitCharacters
  (Characters|SpawnandMoveCharacter (Variables|PlayerControllers|GetPlayer1Controller) "NewEnumerator1" true)
  (Characters|SpawnandMoveCharacter (Variables|PlayerControllers|GetPlayer2Controller) "NewEnumerator0" true))

(fn SpawnandMoveCharacter
  (params (PlayerController :type BP%20Player%20Controller%20Object%20Reference) (Player :type E_Player%20Enum :default "NewEnumerator1") (Move? :type Boolean))
  (LocalVariables|SetPlayerController%20%28local%29 PlayerController)
  (LocalVariables|SetPlayer%20%28local%29 Player)
  (LocalVariables|SetMove?%20%28local%29 Move?)
  (LocalVariables|SetSpawnPoint%20%28local%29 (Utilities|Select :Index (LocalVariables|GetPlayer%20%28local%29) :NewEnumerator1 (Variables|SpawnPoints|GetPlayer1SpawnPoint) :NewEnumerator0 (Variables|SpawnPoints|GetPlayer2SpawnPoint)))
  (switch Utilities|FlowControl|Switch|SwitchonE_Class (Utilities|Select :Index (LocalVariables|GetPlayer%20%28local%29) :NewEnumerator1 (Variables|Classes|GetPlayer1Class) :NewEnumerator0 (Variables|Classes|GetPlayer2Class))
    (:NewEnumerator1
      (bind _returnvalue (Game|SpawnActorfromClass "/Game/Tech/Blueprints/Characters/BP_Mage.BP_Mage_C" (LocalVariables|GetSpawnPoint%20%28local%29) "AdjustIfPossibleButAlwaysSpawn" 0 0))
      (LocalVariables|SetSpawnedCharacter%20%28local%29 _returnvalue))
    (:NewEnumerator0
      (bind _returnvalue_2 (Game|SpawnActorfromClass "/Game/Tech/Blueprints/Characters/BP_Scout.BP_Scout_C" (LocalVariables|GetSpawnPoint%20%28local%29) "AdjustIfPossibleButAlwaysSpawn" 0 0))
      (LocalVariables|SetSpawnedCharacter%20%28local%29 _returnvalue_2)))
  (switch Utilities|FlowControl|Switch|SwitchonE_Player (LocalVariables|GetPlayer%20%28local%29)
    (:NewEnumerator1
      (bind _output_get (Variables|Characters|SetPlayer1Character (LocalVariables|GetSpawnedCharacter%20%28local%29)))
      (Variables|PlayerAIControllers|SetPlayer1AIController (Pawn|GetController _output_get)))
    (:NewEnumerator0
      (bind _output_get_2 (Variables|Characters|SetPlayer2Character (LocalVariables|GetSpawnedCharacter%20%28local%29)))
      (Variables|PlayerAIControllers|SetPlayer1AIController (Pawn|GetController _output_get_2))))
  (Default|Init (LocalVariables|GetSpawnedCharacter%20%28local%29) (LocalVariables|GetPlayer%20%28local%29))
  (Default|Init (LocalVariables|GetPlayerController%20%28local%29) (LocalVariables|GetPlayer%20%28local%29) self (LocalVariables|GetSpawnedCharacter%20%28local%29))
  (Game|Player|SetViewTargetwithBlend (LocalVariables|GetPlayerController%20%28local%29) (LocalVariables|GetSpawnedCharacter%20%28local%29) 0.0 "VTBlend_Linear" 0.0 false)
  (if (LocalVariables|GetMove?%20%28local%29)
    (Default|Moveto (LocalVariables|GetSpawnedCharacter%20%28local%29) (+ (.Location (Math|Transform|BreakTransform (LocalVariables|GetSpawnPoint%20%28local%29))) (Utilities|Select :Index (LocalVariables|GetPlayer%20%28local%29) :NewEnumerator1 (Variables|SpawnPoints|GetPlayer1MoveToPoint) :NewEnumerator0 (Variables|SpawnPoints|GetPlayer2MoveToPoint))) (LocalVariables|GetPlayerController%20%28local%29))
    (else
      (Pawn|Possess (LocalVariables|GetPlayerController%20%28local%29) (LocalVariables|GetSpawnedCharacter%20%28local%29)))))

(fn CharacterSwitch
  (LocalVariables|SetTempCharacterRef (Variables|Characters|GetPlayer1Character))
  (LocalVariables|SetTempCharacter (Variables|Classes|GetPlayer1Class))
  (Utilities|FlowControl|Sequence
    (:then_0
      (Pawn|Possess (Variables|PlayerControllers|GetPlayer1Controller) (Variables|Characters|GetPlayer2Character))
      (Variables|Classes|SetPlayer1Class (Variables|Classes|GetPlayer2Class))
      (Variables|Characters|SetPlayer1Character (Variables|Characters|GetPlayer2Character)))
    (:then_1
      (Pawn|Possess (Variables|PlayerControllers|GetPlayer2Controller) (LocalVariables|GetTempCharacterRef))
      (Variables|Classes|SetPlayer2Class (LocalVariables|GetTempCharacter))
      (Variables|Characters|SetPlayer2Character (LocalVariables|GetTempCharacterRef)))))

(fn InitGoals
  (bind _outactors (Actor|GetAllActorsOfClass "/Game/Tech/Blueprints/Placeables/Goal/BP_BossDoor.BP_BossDoor_C"))
  (Utilities|IsValid (Utilities|Array|Get(acopy) _outactors)
    (:Is%20Valid
      (Variables|Goal|SetBossDoor (Utilities|Array|Get(acopy) _outactors)))
    (:Is%20Not%20Valid
      _))
  (bind _outactors_2 (Actor|GetAllActorsOfClass "/Game/Tech/Blueprints/Placeables/Goal/BP_EndStairs.BP_EndStairs_C"))
  (Utilities|IsValid (Utilities|Array|Get(acopy) _outactors_2)
    (:Is%20Valid
      (bind _output_get (Variables|Goal|SetEndStairs (Utilities|Array|Get(acopy) _outactors_2)))
      (Variables|Goal|SetNextLevelName (Variables|/Game/Tech/Blueprints/Placeables/Goal/BP_EndStairs.BP_EndStairs_C|GetNextLevelName _output_get)))))

(fn InitAISpawnPoint
  (bind _outactors (Actor|GetAllActorsOfClass "/Game/Tech/Blueprints/AI/BP_AISpawnPoint.BP_AISpawnPoint_C"))
  (Utilities|IsValid (Utilities|Array|Get(acopy) _outactors)
    (:Is%20Valid
      (Variables|Default|SetAISpawnPoin (Utilities|Array|Get(acopy) _outactors)))))

(fn SpawnAICharacter
  (params (CurrentAdventurer :type Integer))
  (bind _aispawnpoint (Variables|AI|GetAISpawnPoint))
  (bind _location (Math|Transform|BreakTransform _aispawnpoint))
  (bind (_x _y _z) (Math|Vector|BreakVector _location))
  (bind _returnvalue (Game|SpawnActorfromClass (Utilities|Select :Index (Math|Random|RandomIntegerinRange 0 2) :Option%200 "/Game/Tech/Blueprints/AI/BP_AIKnight.BP_AIKnight_C" :Option%201 "/Game/Tech/Blueprints/AI/BP_AICleric.BP_AICleric_C" :Option%202 "/Game/Tech/Blueprints/AI/BP_AIArcher.BP_AIArcher_C") (Variables|AI|GetAISpawnPoint) "Undefined" 0 0))
  (Utilities|Array|Add (Variables|AI|GetAICharacters) (.AsBP%20AICharacter (Utilities|Casting|CastToBP_AICharacter _returnvalue)))
  (bind _output_get (Variables|/Game/Tech/Blueprints/AI/BP_AICharacter.BP_AICharacter_C|SetName (.AsBP%20AICharacter (Utilities|Casting|CastToBP_AICharacter _returnvalue)) (.OutItem (Utilities|Array|Random (Variables|AI|GetTempAdventurerNames)))))
  (Utilities|Array|RemoveItem (Variables|AI|GetTempAdventurerNames) _output_get)
  (Class|BPIInit|Init(Message) _returnvalue)
  (Default|Moveto (.AsBP%20AICharacter (Utilities|Casting|CastToBP_AICharacter _returnvalue)) (Math|Vector|MakeVector (+ _x (* CurrentAdventurer 1e+02)) _y _z))
  (Default|GetAIPathFlags (.AsBP%20AICharacter (Utilities|Casting|CastToBP_AICharacter _returnvalue)) (Variables|Goal|GetBossDoor)))

(fn ShowScore
  (bind _returnvalue (UserInterface|CreateWidget "/Game/Tech/Blueprints/Widgets/Menus/WB_ScoreMenu.WB_ScoreMenu_C" (Variables|PlayerControllers|GetPlayer1Controller)))
  (Default|Init _returnvalue (Variables|AI|GetAdventurePartyNumber) (Utilities|Array|Length (Variables|AI|GetAICharacters)) (Variables|Default|GetLevelDifficulty) (Variables|Default|GetLevelFlagPar) (+ (Variables|/Game/Tech/Blueprints/Characters/BP_BaseCharacter.BP_BaseCharacter_C|GetFlagCount (Variables|Characters|GetPlayer1Character)) (Variables|/Game/Tech/Blueprints/Characters/BP_BaseCharacter.BP_BaseCharacter_C|GetFlagCount (Variables|Characters|GetPlayer2Character))) "None")
  (UserInterface|Viewport|AddtoViewport _returnvalue 0)
  (Variables|/Script/Engine.PlayerController|SetbShowMouseCursor (Variables|PlayerControllers|GetPlayer1Controller) true))

(fn RemoveDeadAdventurer
  (params (SelfRef :type BP%20AI%20Character%20Object%20Reference))
  (Utilities|Array|RemoveItem (Variables|AI|GetAICharacters) SelfRef))

(fn InitRoundTimer
  (bind _returnvalue (Utilities|Time|SetTimerbyEvent (EventDispatchers|CreateEvent :!event UpdateRoundTimer) 1.0 true))
  (Variables|Timer|SetTimerTH _returnvalue))

(fn UpdateRoundTimer
  (Variables|Timer|SetTimerTimespan (Math|Timespan|MakeTimespan (.Days (Math|Timespan|BreakTimespan (Variables|Timer|GetTimerTimespan))) (.Hours (Math|Timespan|BreakTimespan (Variables|Timer|GetTimerTimespan))) (.Minutes (Math|Timespan|BreakTimespan (Variables|Timer|GetTimerTimespan))) (+ (.Seconds (Math|Timespan|BreakTimespan (Variables|Timer|GetTimerTimespan))) 1) (.Milliseconds (Math|Timespan|BreakTimespan (Variables|Timer|GetTimerTimespan)))))
  (Default|CallTimerModified))

(fn InitDefaultClasses
  (if (or (Utilities|Enum|Equal(Enum) (Variables|Classes|GetPlayer1Class) "NewEnumerator2") (Utilities|Enum|Equal(Enum) (Variables|Classes|GetPlayer2Class) "NewEnumerator2"))
    (Variables|Classes|SetPlayer1Class "NewEnumerator1")
    (Variables|Classes|SetPlayer2Class "NewEnumerator0")))

(fn RespawnCharacters
  (Actor|DestroyActor (Variables|Characters|GetPlayer1Character))
  (Characters|SpawnandMoveCharacter (Variables|PlayerControllers|GetPlayer1Controller) "NewEnumerator1" false)
  (Characters|SpawnandMoveCharacter (Variables|PlayerControllers|GetPlayer2Controller) "NewEnumerator0" false))