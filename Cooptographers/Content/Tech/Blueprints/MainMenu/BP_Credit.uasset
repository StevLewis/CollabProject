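; BP_Credit is a main menu Blueprint that presents a Credits button through a widget component.
; It casts the component's widget to WB_MainMenuButton and initializes it with Credits.
; The same Init runs in both the Construction Script and BeginPlay, so the button is set up at construction and again at play start.
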(event EventBeginPlay
  (Default|Init (.AsWB%20Main%20Menu%20Button (Utilities|Casting|CastToWB_MainMenuButton (UserInterface|GetWidget (Variables|Default|GetWidget)))) (Variables|Default|GetCredits)))

(fn ConstructionScript
  (bind _aswb_main_menu_button (Utilities|Casting|CastToWB_MainMenuButton (UserInterface|GetWidget (Variables|Default|GetWidget))))
  (Default|Init _aswb_main_menu_button (Variables|Default|GetCredits)))