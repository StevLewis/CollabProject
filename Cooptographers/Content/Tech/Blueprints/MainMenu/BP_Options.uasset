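; BP_Options is a main menu actor whose widget component shows a button labeled "Options", initialized both in construction and on BeginPlay.
; Overlapping its Box starts a two-second timer, which is cleared if the overlap ends first, so activation works by dwelling rather than clicking.
; When the timer fires, it plays a sound, adds WB_Options to the viewport and switches to UI-only input with the mouse cursor shown.
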(event OnComponentBeginOverlap(Box)
  (params (OverlappedComponent :type Primitive%20Component%20Object%20Reference) (OtherActor :type Actor%20Object%20Reference) (OtherComp :type Primitive%20Component%20Object%20Reference) (OtherBodyIndex :type Integer) (bFromSweep :type Boolean) (SweepResult :type Hit%20Result%20Structure%20%28by%20ref%29))
  (bind _returnvalue (Utilities|Time|SetTimerbyEvent (delegate Custom|Options) 2.0))
  (Variables|Default|SetButtonTH _returnvalue))

(event OnComponentEndOverlap(Box)
  (params (OverlappedComponent :type Primitive%20Component%20Object%20Reference) (OtherActor :type Actor%20Object%20Reference) (OtherComp :type Primitive%20Component%20Object%20Reference) (OtherBodyIndex :type Integer))
  (Utilities|Time|ClearandInvalidateTimerbyHandle (Variables|Default|GetButtonTH)))

(event Custom|Options
  (bind _returnvalue (Game|GetPlayerController 0))
  (Audio|PlaySound2D "/Game/Design/SFX/UI/HoverButton.HoverButton" 1.0 1.0 0.0 0 0)
  (bind _returnvalue_2 (UserInterface|CreateWidget "/Game/Tech/Blueprints/Widgets/Menus/WB_Options.WB_Options_C"))
  (UserInterface|Viewport|AddtoViewport _returnvalue_2 0)
  (Input|SetInputModeUIOnly _returnvalue 0 "DoNotLock")
  (Variables|/Script/Engine.PlayerController|SetbShowMouseCursor _returnvalue true))

(event EventBeginPlay
  (Default|Init (.AsWB%20Main%20Menu%20Button (Utilities|Casting|CastToWB_MainMenuButton (UserInterface|GetWidget (Variables|Default|GetWidget)))) "Options"))

(fn ConstructionScript
  (bind _aswb_main_menu_button (Utilities|Casting|CastToWB_MainMenuButton (UserInterface|GetWidget (Variables|Default|GetWidget))))
  (Default|Init _aswb_main_menu_button "Options"))