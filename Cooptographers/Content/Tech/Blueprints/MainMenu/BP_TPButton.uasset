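; BP_TPButton is a main menu button actor that teleports whatever actor dwells inside its trigger box.
; Its widget component shows a WB_MainMenuButton, initialized with Text in both the construction script and BeginPlay.
; Box overlap starts a short timer that plays a sound and moves the overlapping actor to the Capsule's location.
; Any end overlap clears the timer, cancelling a pending teleport.
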(event OnComponentBeginOverlap(Box)
  (params (OverlappedComponent :type Primitive%20Component%20Object%20Reference) (OtherActor :type Actor%20Object%20Reference) (OtherComp :type Primitive%20Component%20Object%20Reference) (OtherBodyIndex :type Integer) (bFromSweep :type Boolean) (SweepResult :type Hit%20Result%20Structure%20%28by%20ref%29))
  (bind _returnvalue (Utilities|Time|SetTimerbyEvent (delegate Custom|LevelSelect) 2.0))
  (Variables|Default|SetButtonTH _returnvalue))

(event OnComponentEndOverlap(Box)
  (params (OverlappedComponent :type Primitive%20Component%20Object%20Reference) (OtherActor :type Actor%20Object%20Reference) (OtherComp :type Primitive%20Component%20Object%20Reference) (OtherBodyIndex :type Integer))
  (Utilities|Time|ClearandInvalidateTimerbyHandle (Variables|Default|GetButtonTH)))

(event Custom|LevelSelect
  (Audio|PlaySound2D "/Game/Design/SFX/UI/HoverButton.HoverButton" 1.0 1.0 0.0 0 0)
  (Transformation|SetActorLocation (stale OnComponentBeginOverlap(Box) OtherActor) (Transformation|GetWorldLocation (Variables|Default|GetCapsule)) false false))

(event EventBeginPlay
  (Default|Init (.AsWB%20Main%20Menu%20Button (Utilities|Casting|CastToWB_MainMenuButton (UserInterface|GetWidget (Variables|Default|GetWidget)))) (Variables|Default|GetText)))

(fn ConstructionScript
  (bind _aswb_main_menu_button (Utilities|Casting|CastToWB_MainMenuButton (UserInterface|GetWidget (Variables|Default|GetWidget))))
  (Default|Init _aswb_main_menu_button (Variables|Default|GetText)))