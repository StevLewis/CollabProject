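; Placeable moving platform that travels between its starting location and a configurable offset when its trigger box is overlapped.
; Successive overlaps alternate sending it out and back, and an optional GoBack flag also returns it when the overlap ends.
; Delayed timers play or reverse a timeline that lerps the actor location.
; Overlaps only check that the cached player character is valid, not which actor entered.
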(event OnComponentBeginOverlap(Box)
  (params (OverlappedComponent :type Primitive%20Component%20Object%20Reference) (OtherActor :type Actor%20Object%20Reference) (OtherComp :type Primitive%20Component%20Object%20Reference) (OtherBodyIndex :type Integer) (bFromSweep :type Boolean) (SweepResult :type Hit%20Result%20Structure%20%28by%20ref%29))
  (Utilities|IsValid (Variables|Default|GetCharacterRef)
    (:Is%20Valid
      (if (Variables|Default|GetTriggredOnce)
        (CallFunction|SendPlatformBack)
        (Variables|Default|SetTriggredOnce false)
        (else
          (CallFunction|MovePlatform)
          (Variables|Default|SetTriggredOnce true))))))

(event OnComponentEndOverlap(Box)
  (params (OverlappedComponent :type Primitive%20Component%20Object%20Reference) (OtherActor :type Actor%20Object%20Reference) (OtherComp :type Primitive%20Component%20Object%20Reference) (OtherBodyIndex :type Integer))
  (Utilities|IsValid (Variables|Default|GetCharacterRef)
    (:Is%20Valid
      (if (Variables|Default|GetGoBack?)
        (CallFunction|SendPlatformBack)))))

(event Custom|MovePlatform
  (Utilities|Time|SetTimerbyEvent (delegate Custom|PlatformGo) 2.0))

(event Custom|SendPlatformBack
  (Utilities|Time|SetTimerbyEvent (delegate Custom|PlatformGoBack) 2.0))

(event Custom|PlatformGo
  (bind _newtrack_0 (Timeline|PlatformMove Play)
    (:Update
      (Transformation|SetActorLocation (Math|Vector|Lerp(Vector) (Variables|Default|GetPlatformStartingLocation) (+ (Variables|Default|GetPlatformStartingLocation) (Variables|Default|GetPlatformEndLocation)) _newtrack_0) false false))))

(event Custom|PlatformGoBack
  (bind _newtrack_0 (Timeline|PlatformMove Reverse)
    (:Update
      (Transformation|SetActorLocation (Math|Vector|Lerp(Vector) (Variables|Default|GetPlatformStartingLocation) (+ (Variables|Default|GetPlatformStartingLocation) (Variables|Default|GetPlatformEndLocation)) _newtrack_0) false false))))

(event EventBeginPlay
  (Variables|Default|SetPlatformStartingLocation (Transformation|GetActorLocation))
  (bind _asbp_base_character (Utilities|Casting|CastToBP_BaseCharacter (Game|GetPlayerCharacter 0)))
  (Variables|Default|SetCharacterRef _asbp_base_character))

(fn ConstructionScript)