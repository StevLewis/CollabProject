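; BP_ClassSwitcher is a placeable two-chamber station that triggers a class switch between characters.
; Box overlaps track which BP_BaseCharacters stand in each capsule, and each entry checks whether both hold exactly one.
; If so, a timeline slides both doors closed, then after a short delay calls SwitchClassesMessage on the GameMode and reopens them.
; An entry that breaks that condition while the chambers are closed reverses the doors.
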(event OnComponentBeginOverlap(Box)
  (params (OverlappedComponent :type Primitive%20Component%20Object%20Reference) (OtherActor :type Actor%20Object%20Reference) (OtherComp :type Primitive%20Component%20Object%20Reference) (OtherBodyIndex :type Integer) (bFromSweep :type Boolean) (SweepResult :type Hit%20Result%20Structure%20%28by%20ref%29))
  (bind _asbp_base_character (Utilities|Casting|CastToBP_BaseCharacter OtherActor))
  (Utilities|Array|Add (Variables|Default|GetCapsule1Characters) _asbp_base_character)
  (CallFunction|ChamberStateCheck))

(event OnComponentBeginOverlap(Box1)
  (params (OverlappedComponent :type Primitive%20Component%20Object%20Reference) (OtherActor :type Actor%20Object%20Reference) (OtherComp :type Primitive%20Component%20Object%20Reference) (OtherBodyIndex :type Integer) (bFromSweep :type Boolean) (SweepResult :type Hit%20Result%20Structure%20%28by%20ref%29))
  (bind _asbp_base_character (Utilities|Casting|CastToBP_BaseCharacter OtherActor))
  (Utilities|Array|Add (Variables|Default|GetCapsule2Characters) _asbp_base_character)
  (CallFunction|ChamberStateCheck))

(event OnComponentEndOverlap(Box)
  (params (OverlappedComponent :type Primitive%20Component%20Object%20Reference) (OtherActor :type Actor%20Object%20Reference) (OtherComp :type Primitive%20Component%20Object%20Reference) (OtherBodyIndex :type Integer))
  (bind _asbp_base_character (Utilities|Casting|CastToBP_BaseCharacter OtherActor))
  (Utilities|Array|RemoveItem (Variables|Default|GetCapsule1Characters) _asbp_base_character))

(event OnComponentEndOverlap(Box1)
  (params (OverlappedComponent :type Primitive%20Component%20Object%20Reference) (OtherActor :type Actor%20Object%20Reference) (OtherComp :type Primitive%20Component%20Object%20Reference) (OtherBodyIndex :type Integer))
  (bind _asbp_base_character (Utilities|Casting|CastToBP_BaseCharacter OtherActor))
  (Utilities|Array|RemoveItem (Variables|Default|GetCapsule2Characters) _asbp_base_character))

(event Custom|OpenChambers
  (Variables|Default|SetChambersClosed? false)
  (bind _float (Timeline|Move Reverse)
    (:Update
      (Transformation|SetRelativeLocation (Variables|Default|GetDoor1) (Math|Vector|Lerp(Vector) (Variables|Default|GetChamber1StartingLocation) "80.000000, 0,0.000000" _float) false false)
      (Transformation|SetRelativeLocation (Variables|Default|GetDoor2) (Math|Vector|Lerp(Vector) (Variables|Default|GetChamber2StartingLocation) "80.000000,0.000000,0.000000" _float) false false))
    (:Finished
      (if (Variables|Default|GetChambersClosed?)
        (Utilities|FlowControl|Delay 1.0)
        (Class|BPISwitch|SwitchClasses(Message) (Game|GetGameMode))
        (Utilities|FlowControl|Delay 1.0)
        (CallFunction|OpenChambers)))))

(event Custom|CloseChambers
  (Variables|Default|SetChambersClosed? true)
  (bind _float (Timeline|Move Play)
    (:Update
      (Transformation|SetRelativeLocation (Variables|Default|GetDoor1) (Math|Vector|Lerp(Vector) (Variables|Default|GetChamber1StartingLocation) "80.000000, 0,0.000000" _float) false false)
      (Transformation|SetRelativeLocation (Variables|Default|GetDoor2) (Math|Vector|Lerp(Vector) (Variables|Default|GetChamber2StartingLocation) "80.000000,0.000000,0.000000" _float) false false))
    (:Finished
      (if (Variables|Default|GetChambersClosed?)
        (Utilities|FlowControl|Delay 1.0)
        (Class|BPISwitch|SwitchClasses(Message) (Game|GetGameMode))
        (Utilities|FlowControl|Delay 1.0)
        (CallFunction|OpenChambers)))))

(fn ConstructionScript
  (Variables|Default|SetChamber1StartingLocation (Variables|/Script/Engine.SceneComponent|GetRelativeLocation (Variables|Default|GetDoor1)))
  (Variables|Default|SetChamber2StartingLocation (Variables|/Script/Engine.SceneComponent|GetRelativeLocation (Variables|Default|GetDoor2))))

(fn ChamberStateCheck
  (if (and (== (Utilities|Array|Length (Variables|Default|GetCapsule1Characters)) 1) (== (Utilities|Array|Length (Variables|Default|GetCapsule2Characters)) 1))
    (CallFunction|CloseChambers)
    (elif (Variables|Default|GetChambersClosed?)
      (CallFunction|OpenChambers))))