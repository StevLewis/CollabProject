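; Placeable trigger that resets the current level with new party settings (wait time and party size).
; On box overlap it saves both values through BP_GameInstance, then reopens the current level by name.
; The construction script writes the configured values into a text label on the actor.
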(event OnComponentBeginOverlap(Box)
  (params (OverlappedComponent :type Primitive%20Component%20Object%20Reference) (OtherActor :type Actor%20Object%20Reference) (OtherComp :type Primitive%20Component%20Object%20Reference) (OtherBodyIndex :type Integer) (bFromSweep :type Boolean) (SweepResult :type Hit%20Result%20Structure%20%28by%20ref%29))
  (bind _asbp_game_instance (Utilities|Casting|CastToBP_GameInstance (Game|GetGameInstance)))
  (Default|SaveLevelDetails _asbp_game_instance (Variables|Default|GetPartyWaitTime) (Variables|Default|GetPartySize))
  (bind _returnvalue (Game|GetCurrentLevelName true))
  (Game|OpenLevel(byName) (Utilities|String|StringToName _returnvalue)))

(fn ConstructionScript
  (Rendering|Components|TextRender|SetText (Variables|Default|GetTextRender) (Utilities|Text|FormatText "Reset to {wait time} seconds, size {party size}" (Variables|Default|GetPartyWaitTime) (Variables|Default|GetPartySize))))