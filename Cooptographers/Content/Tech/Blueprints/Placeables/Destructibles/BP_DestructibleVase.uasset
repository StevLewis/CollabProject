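; BP_DestructibleVase is a placeable breakable prop that can hide a dialogue clue.
; Its construction script applies the configured destructible mesh to the Destructible component.
; On fracture it plays a break sound and, if flagged as containing a clue, spawns a BP_Clue at its location.
; The clue is initialized with the vase's dialogue settings, including optional Mage and Scout variants and popup time.
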(event OnComponentFracture(Destructible)
  (params (HitPoint :type Vector%20%28by%20ref%29 :default "0, 0, 0") (HitDirection :type Vector%20%28by%20ref%29 :default "0, 0, 0"))
  (Audio|PlaySoundatLocation "/Game/Tech/Sounds/Cues/SC_ChestBreak.SC_ChestBreak" (Transformation|GetActorLocation) "0, 0, 0" 1.0 1.0 0.0 "/Game/Tech/Sounds/SA_DefaultAttentuation.SA_DefaultAttentuation" 0 0)
  (if (Variables|Default|GetContainsClue?)
    (bind _returnvalue (Game|SpawnActorfromClass "/Game/Tech/Blueprints/Placeables/Pickups/BP_Clue.BP_Clue_C" (Math|Transform|MakeTransform (Transformation|GetActorLocation) "0, 0, 0" "1,1,1") "AlwaysSpawn" 0 0))
    (Default|Init _returnvalue (Variables|Default|GetClue%20Dialogue) (Variables|Default|GetDifferent%20Per%20Class?) (Variables|Default|GetMage%20Clue%20Dialogue) (Variables|Default|GetScout%20Clue%20Dialogue) (Variables|Default|GetPopup%20Time))))

(fn ConstructionScript
  (Class|DestructibleComponent|SetDestructibleMesh (Variables|Default|GetDestructible) (Variables|Default|GetMesh)))