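; BP_BossDoor is a placeable boss door that counts adventurers passing through it toward a needed number.
; A proximity trigger opens the door when an adventurer approaches, and the Trigger event also opens it.
; An enter collision increments the finished count, refreshes the WB_BossDoor widget, broadcasts AdventurerEntered and tells the adventurer to enter the boss door.
; BeginPlay initializes the widget and broadcasts the starting count.
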(event OnComponentBeginOverlap(EnterCollision)
  (params (OverlappedComponent :type Primitive%20Component%20Object%20Reference) (OtherActor :type Actor%20Object%20Reference) (OtherComp :type Primitive%20Component%20Object%20Reference) (OtherBodyIndex :type Integer) (bFromSweep :type Boolean) (SweepResult :type Hit%20Result%20Structure%20%28by%20ref%29))
  (bind _asbp_base_adventurer (Utilities|Casting|CastToBP_BaseAdventurer OtherActor))
  (Math|Integer|IncrementInt (Variables|Default|GetAdventurersFinished)
    (:%20%20
      (Default|Init (Variables|Default|GetAdventurerNumberWidget) (Variables|Default|GetAdventurersFinished) (Variables|Default|GetNeededAdventurers))
      (Default|CallAdventurerEntered (Variables|Default|GetAdventurersFinished) (Variables|Default|GetNeededAdventurers))
      (Default|EnterBossDoor _asbp_base_adventurer))))

(event OnComponentBeginOverlap(ProximityCollision)
  (params (OverlappedComponent :type Primitive%20Component%20Object%20Reference) (OtherActor :type Actor%20Object%20Reference) (OtherComp :type Primitive%20Component%20Object%20Reference) (OtherBodyIndex :type Integer) (bFromSweep :type Boolean) (SweepResult :type Hit%20Result%20Structure%20%28by%20ref%29))
  (Utilities|Casting|CastToBP_BaseAdventurer OtherActor)
  (CallFunction|Trigger))

(event EventTrigger
  (CallFunction|OpenDoor))

(event EventBeginPlay
  (bind _aswb_boss_door (Utilities|Casting|CastToWB_BossDoor (UserInterface|GetWidget (Variables|Default|GetWidget))))
  (Variables|Default|SetAdventurerNumberWidget _aswb_boss_door)
  (Default|Init (Variables|Default|GetAdventurerNumberWidget) (Variables|Default|GetAdventurersFinished) (Variables|Default|GetNeededAdventurers))
  (Default|CallAdventurerEntered (Variables|Default|GetAdventurersFinished) (Variables|Default|GetNeededAdventurers)))

(fn ConstructionScript
  (|CallParentFunction))