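; Placeable sliding double door that moves left and right meshes between start and target relative locations.
; OpenDoor and CloseDoor play or reverse a shared Move timeline, each with its own speed multiplier, and its update lerps both panels.
; The construction script records each mesh's placed relative location as its closed start position.
; Interact and Trigger are empty here, so opening and closing rely on calls to those door events.
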(event Custom|OpenDoor
  (Components|Timeline|SetPlayRate (Variables|Default|GetMove) (* 1.0 (Variables|Default|GetOpenMultiplier)))
  (bind _newtrack_0 (Timeline|Move Play)
    (:Update
      (CallFunction|MoveTimelineUpdate _newtrack_0))))

(event Custom|CloseDoor
  (Components|Timeline|SetPlayRate (Variables|Default|GetMove) (* 1.0 (Variables|Default|GetCloseMultiplier)))
  (bind _newtrack_0 (Timeline|Move Reverse)
    (:Update
      (CallFunction|MoveTimelineUpdate _newtrack_0))))

(event Custom|MoveTimelineUpdate
  (params (Alpha :type Float%20%28single-precision%29))
  (Transformation|SetRelativeLocation (Variables|Default|GetLeftDoorMesh) (Math|Vector|Lerp(Vector) (Variables|Default|GetLeftDoorStartLocation) (Variables|Default|GetLeftDoorTargetLocation) Alpha) false false)
  (Transformation|SetRelativeLocation (Variables|Default|GetRightDoorMesh) (Math|Vector|Lerp(Vector) (Variables|Default|GetRightDoorStartLocation) (Variables|Default|GetRightDoorTargetLocation) Alpha) false false))

(event EventInteract
  (params (Interactor :type Actor%20Object%20Reference)))

(event EventTrigger)

(fn ConstructionScript
  (Variables|Default|SetLeftDoorStartLocation (Variables|/Script/Engine.SceneComponent|GetRelativeLocation (Variables|Default|GetLeftDoorMesh)))
  (Variables|Default|SetRightDoorStartLocation (Variables|/Script/Engine.SceneComponent|GetRelativeLocation (Variables|Default|GetRightDoorMesh))))