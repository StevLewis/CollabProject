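; BP_EndStairs is a placeable goal that requires both BP_Mage and BP_Scout to stand on its stair plate.
; ActivateTrigger shows the plate and enables query collision on its trigger.
; Begin and end overlaps update an actor list, then CharactersCheck counts at most one of each character class.
; The count colors the plate red, orange or green, and two calls SetupEndSceneMessage on the game mode.
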(event OnComponentBeginOverlap(TriggerCollision)
  (params (OverlappedComponent :type Primitive%20Component%20Object%20Reference) (OtherActor :type Actor%20Object%20Reference) (OtherComp :type Primitive%20Component%20Object%20Reference) (OtherBodyIndex :type Integer) (bFromSweep :type Boolean) (SweepResult :type Hit%20Result%20Structure%20%28by%20ref%29))
  (bind _stairplate (Variables|Default|GetStairPlate))
  (Utilities|Array|Add (Variables|Default|GetOverlappedActors) OtherActor)
  (CallFunction|CharactersCheck)
  (switch int (Variables|Default|GetCharactersOn?)
    (:0
      (Rendering|Material|SetMaterial _stairplate 0 "/Game/Tech/Materials/MI_Red.MI_Red"))
    (:1
      (Rendering|Material|SetMaterial _stairplate 0 "/Game/Tech/Materials/MI_Orange.MI_Orange"))
    (:2
      (Rendering|Material|SetMaterial _stairplate 0 "/Game/Tech/Materials/MI_Green.MI_Green")
      (Class|BPIEnd|SetupEndScene(Message) (Game|GetGameMode)))))

(event OnComponentEndOverlap(TriggerCollision)
  (params (OverlappedComponent :type Primitive%20Component%20Object%20Reference) (OtherActor :type Actor%20Object%20Reference) (OtherComp :type Primitive%20Component%20Object%20Reference) (OtherBodyIndex :type Integer))
  (bind _stairplate (Variables|Default|GetStairPlate))
  (Utilities|Array|RemoveItem (Variables|Default|GetOverlappedActors) OtherActor)
  (CallFunction|CharactersCheck)
  (switch int (Variables|Default|GetCharactersOn?)
    (:0
      (Rendering|Material|SetMaterial _stairplate 0 "/Game/Tech/Materials/MI_Red.MI_Red"))
    (:1
      (Rendering|Material|SetMaterial _stairplate 0 "/Game/Tech/Materials/MI_Orange.MI_Orange"))
    (:2
      (Rendering|Material|SetMaterial _stairplate 0 "/Game/Tech/Materials/MI_Green.MI_Green")
      (Class|BPIEnd|SetupEndScene(Message) (Game|GetGameMode)))))

(event Custom|ActivateTrigger
  (Rendering|SetVisibility (Variables|Default|GetStairPlate) true false)
  (Collision|SetCollisionEnabled (Variables|Default|GetTriggerCollision) "QueryOnly"))

(fn ConstructionScript
  (|CallParentFunction))

(fn CharactersCheck
  (Variables|Default|SetCharactersOn? 0)
  (bind _array_element (Utilities|Array|ForEachLoopwithBreak (Variables|Default|GetOverlappedActors) :!label _label)
    (:LoopBody
      (if (== (Utilities|GetClass _array_element) "/Game/Tech/Blueprints/Characters/BP_Mage.BP_Mage_C")
        (Math|Integer|IncrementInt (Variables|Default|GetCharactersOn?)
          (:%20%20
            (goto _label Break)))))
    (:Completed
      (bind _array_element_2 (Utilities|Array|ForEachLoopwithBreak (Variables|Default|GetOverlappedActors) :!label _label_2)
        (:LoopBody
          (if (== (Utilities|GetClass _array_element_2) "/Game/Tech/Blueprints/Characters/BP_Scout.BP_Scout_C")
            (Math|Integer|IncrementInt (Variables|Default|GetCharactersOn?)
              (:%20%20
                (goto _label_2 Break)))))))))