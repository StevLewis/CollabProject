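; A lassoable pushable block that gets yanked along the trace when pulled.
; PullTowards prints the pull direction, then applies a velocity-change impulse to the physics mesh, pointing from the trace end back to its start.
; If the impact point is far enough from the trace start, it waits briefly, then toggles physics simulation off and on, which appears intended to halt the block's momentum.
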(event EventPullTowards
  (params (ActorHit :type Hit%20Result%20Structure))
  (bind (_bblockinghit _binitialoverlap _time _distance _location _impactpoint _normal _impactnormal _physmat _hitactor _hitcomponent _hitbonename _hititem _faceindex _tracestart _traceend) (Collision|BreakHitResult ActorHit))
  (bind _pushablemesh (Variables|Default|GetPushableMesh))
  (bind _returnvalue (Math|Vector|GetUnitDirection(Vector) _traceend _tracestart))
  (Development|PrintString (Utilities|String|ToString(Vector) _returnvalue))
  (Physics|AddImpulse (Variables|Default|GetPushableMesh) (* _returnvalue 1.2e+03) "None" true)
  (if (>= (Math|Vector|VectorLength (- _impactpoint _tracestart)) 5e+01)
    (Utilities|FlowControl|Delay 0.4)
    (Physics|SetSimulatePhysics _pushablemesh false)
    (Physics|SetSimulatePhysics _pushablemesh true)))

(fn ConstructionScript
  (|CallParentFunction))