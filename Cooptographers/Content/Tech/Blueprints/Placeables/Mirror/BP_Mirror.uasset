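; Placeable mirror that reflects incoming light beams, damaging what the reflected beam hits and chaining through other reflective actors.
; Reflect mirrors the incoming trace about the hit normal, then starts a short one-shot timer unless one is already running.
; SpawnLine positions the beam VFX, line traces, applies damage and forwards hits via BPI_Reflect.
; Only the Mirror component counts as reflectable; SpawnLineReverse is an unused stub.
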(event EventReflect
  (params (ActorHit :type Hit%20Result%20Structure))
  (bind (_bblockinghit _binitialoverlap _time _distance _location _impactpoint _normal _impactnormal _physmat _hitactor _hitcomponent _hitbonename _hititem _faceindex _tracestart _traceend) (Collision|BreakHitResult ActorHit))
  ;[1 1 1] Checks which collision is hit and spawns a line at the right angle based on that
  (Variables|Default|SetLine%20Start _location)
  (Variables|Default|SetLine%20End (+ _location (* (Math|Vector|GetReflectionVector (Math|Vector|GetUnitDirection(Vector) _tracestart _traceend) _normal) (Variables|Default|GetLine%20Trace%20Length))))
  (if (not (Utilities|Time|IsTimerActivebyHandle (Variables|Default|GetBeamTH)))
    (bind _returnvalue (Utilities|Time|SetTimerbyEvent (EventDispatchers|CreateEvent :!event SpawnLine) 0.1))
    (Variables|Default|SetBeamTH _returnvalue)))

(fn ConstructionScript
  (|CallParentFunction))

(fn SpawnLine
  (bind _vfx_lightbeam (Variables|Default|GetVFX_LightBeam))
  (bind _line_start (Variables|Default|GetLine%20Start))
  (Transformation|SetWorldLocation _vfx_lightbeam _line_start false false)
  (Components|Activation|Activate _vfx_lightbeam false)
  (bind (_outhit _returnvalue) (Collision|LineTraceForObjects _line_start (Variables|Default|GetLine%20End) (Utilities|Array|MakeArray "ObjectTypeQuery1" "ObjectTypeQuery2" "ObjectTypeQuery3" "ObjectTypeQuery4" "ObjectTypeQuery6" "ObjectTypeQuery10") false 0 "ForDuration" true "(R=1.000000,G=0.000000,B=0.000000,A=1.000000)" "(R=0.000000,G=1.000000,B=0.000000,A=1.000000)" 0.2))
  (if _returnvalue
    (Class|PrimitiveComponent|SetCullDistance (Variables|Default|GetVFX_LightBeam) (.Distance (Collision|BreakHitResult _outhit)))
    (Class|BPIDamage|ApplyDamagebyType(Message) (.HitActor (Collision|BreakHitResult _outhit)) 1.0 0 "NewEnumerator3")
    (if (Utilities|DoesObjectImplementInterface (.HitActor (Collision|BreakHitResult _outhit)) "/Game/Tech/Blueprints/Placeables/Mirror/BPI_Reflect.BPI_Reflect_C")
      (bind _isreflectablecomponent_ (Class|BPIReflect|IsReflectable?(Message) (.HitActor (Collision|BreakHitResult _outhit)) (.HitComponent (Collision|BreakHitResult _outhit))))
      (if _isreflectablecomponent_
        (Class|BPIReflect|Reflect(Message) (.HitActor (Collision|BreakHitResult _outhit)) _outhit)))))

(fn SpawnLineReverse)

(fn IsReflectable?
  (params (HitComponent :type Actor%20Component%20Object%20Reference))
  (return (== HitComponent (Variables|Default|GetMirror))))