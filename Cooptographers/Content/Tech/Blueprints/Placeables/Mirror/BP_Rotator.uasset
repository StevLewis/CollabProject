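; Placeable rotator in the Mirror folder that turns its root by a set yaw amount each time its Trigger event fires.
; A timeline (Play, not Play from Start) lerps relative rotation from the stored start to a target with zero pitch and roll.
; The start rotation is captured at construction and updated when the timeline finishes.
; An AttachTo snap-attach node in the construction script is disconnected.
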(event EventTrigger
  (Variables|Default|SetTarget%20Rotation (Math|Rotator|MakeRotator 0.0 0.0 (+ (.yaw (Variables|Default|GetStart%20Rotation)) (Variables|Default|GetRotation%20Amount))))
  (bind _newtrack_0 (Timeline|Timeline_0 Play)
    (:Update
      (Transformation|SetRelativeRotation (Variables|Default|GetDefaultSceneRoot) (Math|Rotator|Lerp(Rotator) (Variables|Default|GetStart%20Rotation) (Variables|Default|GetTarget%20Rotation) _newtrack_0) false false))
    (:Finished
      (Variables|Default|SetStart%20Rotation (Variables|/Script/Engine.SceneComponent|GetRelativeRotation (Variables|Default|GetDefaultSceneRoot))))))

(fn ConstructionScript
  (|CallParentFunction)
  (Variables|Default|SetStart%20Rotation (Variables|/Script/Engine.SceneComponent|GetRelativeRotation (Variables|Default|GetDefaultSceneRoot))))