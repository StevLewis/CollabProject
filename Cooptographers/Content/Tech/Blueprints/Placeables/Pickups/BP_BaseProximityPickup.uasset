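; BP_BaseProximityPickup is a base pickup Blueprint with a rotating movement component and a capsule collision volume.
; Its construction script applies the configurable rotation rate and sizes the capsule from the pickup height and radius variables.
; The height sets the capsule half-height, and the radius is capped at that value.
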(fn ConstructionScript
  (bind _collision (Variables|Default|GetCollision))
  (Variables|/Script/Engine.RotatingMovementComponent|SetRotationRate (Variables|Default|GetRotatingMovement) (Variables|Default|GetRotationRate))
  (Components|Capsule|SetCapsuleHalfHeight (Variables|Default|GetCollision) (Variables|Default|GetPickupHeight) true)
  (if (<= (Variables|Default|GetPickupRadius) (Variables|Default|GetPickupHeight))
    (Components|Capsule|SetCapsuleRadius _collision (Variables|Default|GetPickupRadius) true)
    (else
      (Components|Capsule|SetCapsuleRadius _collision (Variables|Default|GetPickupHeight) true))))