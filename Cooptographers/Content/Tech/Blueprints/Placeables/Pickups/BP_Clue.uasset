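; BP_Clue is a pickup that passes a timed clue message to the character who touches it.
; An Init event stores the dialogue options and popup time, then enables query-only collision after a short delay.
; On overlap with a BP_BaseCharacter, it writes either shared or class-specific (Mage or Scout) text and the display time onto that character, then destroys itself.
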(event OnComponentBeginOverlap(Collision)
  (params (OverlappedComponent :type Primitive%20Component%20Object%20Reference) (OtherActor :type Actor%20Object%20Reference) (OtherComp :type Primitive%20Component%20Object%20Reference) (OtherBodyIndex :type Integer) (bFromSweep :type Boolean) (SweepResult :type Hit%20Result%20Structure%20%28by%20ref%29))
  (bind _asbp_base_character (Utilities|Casting|CastToBP_BaseCharacter OtherActor))
  (if (Variables|Default|GetDifferentPerClass?)
    (Variables|/Game/Tech/Blueprints/Characters/BP_BaseCharacter.BP_BaseCharacter_C|SetClueText _asbp_base_character (Utilities|Select :Index (Variables|/Game/Tech/Blueprints/Characters/BP_BaseCharacter.BP_BaseCharacter_C|GetClass _asbp_base_character) :NewEnumerator2 "" :NewEnumerator1 (Variables|Default|GetMageClueDialogue) :NewEnumerator0 (Variables|Default|GetScoutClueDialogue)))
    (Variables|/Game/Tech/Blueprints/Characters/BP_BaseCharacter.BP_BaseCharacter_C|SetClueTime _asbp_base_character (Variables|Default|GetPopupTime))
    (Actor|DestroyActor)
    (else
      (Variables|/Game/Tech/Blueprints/Characters/BP_BaseCharacter.BP_BaseCharacter_C|SetClueText _asbp_base_character (Variables|Default|GetClueDialogue))
      (Variables|/Game/Tech/Blueprints/Characters/BP_BaseCharacter.BP_BaseCharacter_C|SetClueTime _asbp_base_character (Variables|Default|GetPopupTime))
      (Actor|DestroyActor))))

(event Custom|Init
  (params (ClueDialogue :type Text) (DifferentPerClass? :type Boolean) (MageClueDialogue :type Text) (ScoutClueDialogue :type Text) (PopupTime :type Float%20%28single-precision%29))
  (Variables|Default|SetClueDialogue ClueDialogue)
  (Variables|Default|SetDifferentPerClass? DifferentPerClass?)
  (Variables|Default|SetMageClueDialogue MageClueDialogue)
  (Variables|Default|SetScoutClueDialogue ScoutClueDialogue)
  (Variables|Default|SetPopupTime PopupTime)
  (Utilities|FlowControl|Delay 1.0)
  (Collision|SetCollisionEnabled (Variables|Default|GetCollision) "QueryOnly"))

(fn ConstructionScript
  (|CallParentFunction))