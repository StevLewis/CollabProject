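; BP_LassoProjectile is a lasso projectile that triggers a pull on actors it hits.
; On a collision hit with an actor implementing BPI_Actions, it destroys itself and sends that actor a PullTowards message with the hit result.
; When ReturnProj is set, overlapping a BP_Scout also destroys it.
; The construction script applies ProjSpeed as both initial and max projectile movement speed.
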(event OnComponentBeginOverlap(Collision)
  (params (OverlappedComponent :type Primitive%20Component%20Object%20Reference) (OtherActor :type Actor%20Object%20Reference) (OtherComp :type Primitive%20Component%20Object%20Reference) (OtherBodyIndex :type Integer) (bFromSweep :type Boolean) (SweepResult :type Hit%20Result%20Structure%20%28by%20ref%29))
  (if (Variables|Default|GetReturnProj?)
    (if (== (Utilities|GetClass OtherActor) "/Game/Tech/Blueprints/Characters/BP_Scout.BP_Scout_C")
      (Actor|DestroyActor))))

(event OnComponentHit(Collision)
  (params (HitComponent :type Primitive%20Component%20Object%20Reference) (OtherActor :type Actor%20Object%20Reference) (OtherComp :type Primitive%20Component%20Object%20Reference) (NormalImpulse :type Vector :default "0, 0, 0") (Hit :type Hit%20Result%20Structure%20%28by%20ref%29))
  (if (Utilities|DoesObjectImplementInterface OtherActor "/Game/Tech/Blueprints/Characters/BPI_Actions.BPI_Actions_C")
    (Actor|DestroyActor)
    (Class|BPIActions|PullTowards(Message) OtherActor Hit)))

(fn ConstructionScript
  (bind _projspeed (Variables|Default|GetProjSpeed))
  (bind _projectilemovement (Variables|Default|GetProjectileMovement))
  (Variables|/Script/Engine.ProjectileMovementComponent|SetInitialSpeed _projectilemovement _projspeed)
  (Variables|/Script/Engine.ProjectileMovementComponent|SetMaxSpeed _projectilemovement _projspeed))