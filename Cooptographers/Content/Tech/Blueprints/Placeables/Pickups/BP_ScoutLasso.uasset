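; BP_ScoutLasso is a placeable pickup that grants Scout the lasso equipment.
; When Scout overlaps its collision, a timeline lerps the actor toward Scout's current location.
; Once within range or when the timeline finishes, it calls Scout's PickupEquipment, shows a dialogue line pointing to the Equipment Menu, and destroys itself.
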(event OnComponentBeginOverlap(Collision)
  (params (OverlappedComponent :type Primitive%20Component%20Object%20Reference) (OtherActor :type Actor%20Object%20Reference) (OtherComp :type Primitive%20Component%20Object%20Reference) (OtherBodyIndex :type Integer) (bFromSweep :type Boolean) (SweepResult :type Hit%20Result%20Structure%20%28by%20ref%29))
  (bind _asbp_scout (Utilities|Casting|CastToBP_Scout OtherActor))
  (Variables|Default|SetScout _asbp_scout)
  (bind _newtrack_0 (Timeline|Move Play)
    (:Update
      (if (Math|Vector|Equal(Vector) (Transformation|GetActorLocation) (Transformation|GetActorLocation (Variables|Default|GetScout)) 1e+01)
        (Default|PickupEquipment (Variables|Default|GetScout) :!label _label)
        (Default|UpdateDialogueText (Variables|Default|GetScout) "I found Uncle Jones' lasso!  
I can check what it does in the Equipment Menu!" 4.0)
        (Actor|DestroyActor)
        (else
          (Transformation|SetActorLocation (Math|Vector|Lerp(Vector) (Transformation|GetActorLocation) (Transformation|GetActorLocation (Variables|Default|GetScout)) _newtrack_0) false false))))
    (:Finished
      (goto _label))))

(fn ConstructionScript
  (|CallParentFunction))