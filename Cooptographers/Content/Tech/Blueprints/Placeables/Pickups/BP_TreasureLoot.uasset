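; BP_TreasureLoot is a placeable treasure pickup that adventurers collect by walking into it.
; On overlap with a BP_BaseAdventurer, a Move timeline lerps the loot toward that adventurer's location, giving a magnet-like pull.
; When it gets within range or the timeline finishes, Pickup notifies the adventurer via LootPickedUp, plays a gold pickup sound and destroys the actor.
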(event OnComponentBeginOverlap(Collision)
  (params (OverlappedComponent :type Primitive%20Component%20Object%20Reference) (OtherActor :type Actor%20Object%20Reference) (OtherComp :type Primitive%20Component%20Object%20Reference) (OtherBodyIndex :type Integer) (bFromSweep :type Boolean) (SweepResult :type Hit%20Result%20Structure%20%28by%20ref%29))
  (bind _asbp_base_adventurer (Utilities|Casting|CastToBP_BaseAdventurer OtherActor))
  (Variables|Default|SetAICharacter _asbp_base_adventurer)
  (bind _newtrack_0 (Timeline|Move Play)
    (:Update
      (if (Math|Vector|Equal(Vector) (Transformation|GetActorLocation) (Transformation|GetActorLocation (Variables|Default|GetAICharacter)) 1e+01)
        (CallFunction|Pickup)
        (else
          (Transformation|SetActorLocation (Math|Vector|Lerp(Vector) (Transformation|GetActorLocation) (Transformation|GetActorLocation (Variables|Default|GetAICharacter)) _newtrack_0) false false))))
    (:Finished
      (CallFunction|Pickup))))

(event Custom|Pickup
  (Default|LootPickedUp (Variables|Default|GetAICharacter))
  (Audio|PlaySoundatLocation "/Game/Tech/Sounds/Cues/SC_GoldPickup.SC_GoldPickup" (Transformation|GetActorLocation) "0, 0, 0" 1.0 1.0 0.0 "/Game/Tech/Sounds/SA_DefaultAttentuation.SA_DefaultAttentuation" 0 0)
  (Actor|DestroyActor))

(fn ConstructionScript
  (|CallParentFunction))