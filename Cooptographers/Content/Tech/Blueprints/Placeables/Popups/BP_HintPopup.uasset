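; BP_HintPopup is a placeable trigger that shows hint dialogue to a player character entering its collision.
; On overlap it casts to BP_BaseCharacter and calls UpdateDialogueText on that character with the configured popup time.
; A DifferentPerPlayer flag chooses between one shared text and separate Player 1 and Player 2 texts, selected by the character's PlayerIndex.
; It has no one-shot guard, so every new overlap sends the hint again.
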(event OnComponentBeginOverlap(Collision)
  (params (OverlappedComponent :type Primitive%20Component%20Object%20Reference) (OtherActor :type Actor%20Object%20Reference) (OtherComp :type Primitive%20Component%20Object%20Reference) (OtherBodyIndex :type Integer) (bFromSweep :type Boolean) (SweepResult :type Hit%20Result%20Structure%20%28by%20ref%29))
  (bind _asbp_base_character (Utilities|Casting|CastToBP_BaseCharacter OtherActor))
  (if (Variables|Default|GetDifferentPerPlayer?)
    (Default|UpdateDialogueText _asbp_base_character (Utilities|Select :Index (Variables|/Game/Tech/Blueprints/Characters/BP_BaseCharacter.BP_BaseCharacter_C|GetPlayerIndex _asbp_base_character) :NewEnumerator1 (Variables|Default|GetPlayer1Dialogue) :NewEnumerator0 (Variables|Default|GetPlayer2Dialogue)) (Variables|Default|GetPopupTime))
    (else
      (Default|UpdateDialogueText _asbp_base_character (Variables|Default|GetDialogue) (Variables|Default|GetPopupTime)))))

(fn ConstructionScript)