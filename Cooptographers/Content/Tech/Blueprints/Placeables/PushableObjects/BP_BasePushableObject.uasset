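; Base pushable physics block that can be pulled, levitated, or broken into a destructible actor.
; Pulls cancel levitation and apply a velocity impulse toward the trace start.
; Levitation uses timelines to raise the block, lock it to the XY plane, then readjust rotation and release it.
; Breaking spawns DestructibleClass, then either respawns a copy at the construction-time transform or destroys itself; hits briefly toggle physics after a delay.
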(event OnComponentHit(Mesh)
  (params (HitComponent :type Primitive%20Component%20Object%20Reference) (OtherActor :type Actor%20Object%20Reference) (OtherComp :type Primitive%20Component%20Object%20Reference) (NormalImpulse :type Vector :default "0, 0, 0") (Hit :type Hit%20Result%20Structure%20%28by%20ref%29))
  (if (> (Transformation|GetDistanceTo (Game|GetPlayerCharacter 0) self) 1.3e+02)
    _
    (else
      _))
  (Utilities|FlowControl|Delay 0.2)
  (Physics|SetSimulatePhysics (Variables|Default|GetMesh) false)
  (Physics|SetSimulatePhysics (Variables|Default|GetMesh) true))

(event Custom|StopLevitating
  ;[1 1 1] Levitation
  (bind _rotate (Timeline|ReadjustRotation PlayFromStart)
    (:Update
      (Transformation|SetActorRotation (Math|Rotator|Lerp(Rotator) (Variables|/Script/Engine.SceneComponent|GetRelativeRotation (Variables|Default|GetMesh)) "0,90.000000, 0" _rotate))
      (Class|PrimitiveComponent|SetConstraintMode (Variables|Default|GetMesh) "Default")
      (Variables|Default|SetLevitating? false))))

(event Custom|Respawn
  (Game|SpawnActorfromClass (Utilities|GetClass self) (Variables|Default|GetSpawnTransform) "Undefined" 0 0)
  (Actor|DestroyActor))

(event EventBreak
  (Utilities|FlowControl|DoOnce false
    (:Completed
      (Components|StaticMesh|SetStaticMesh (Variables|Default|GetMesh) 0)
      (Game|SpawnActorfromClass (Variables|Default|GetDestructibleClass) (Transformation|GetActorTransform) "AlwaysSpawn" 0 0)
      (Utilities|FlowControl|Delay 2.0)
      (if (Variables|Default|GetShouldRespawn?)
        (CallFunction|Respawn)
        (else
          (Actor|DestroyActor))))))

(event EventPullTowards
  (params (ActorHit :type Hit%20Result%20Structure))
  (bind (_bblockinghit _binitialoverlap _time _distance _location _impactpoint _normal _impactnormal _physmat _hitactor _hitcomponent _hitbonename _hititem _faceindex _tracestart _traceend) (Collision|BreakHitResult ActorHit))
  ;[1 1 1] Pulls the block towards the trace that hit it
  (if (Variables|Default|GetLevitating?)
    (CallFunction|StopLevitating))
  (Physics|AddImpulse (Variables|Default|GetMesh) (* (Math|Vector|GetUnitDirection(Vector) _traceend _tracestart) 1.2e+03) "None" true))

(event EventLevitatefor
  (params (LevitationTime :type Float%20%28single-precision%29))
  ;[1 1 1] Levitation
  (if (not (Variables|Default|GetLevitating?))
    (Variables|Default|SetCurrentLocation (Transformation|GetActorLocation))
    (Variables|Default|SetLevitating? true)
    (bind _newtrack_0 (Timeline|Float PlayFromStart)
      (:Update
        (Transformation|SetActorRelativeLocation (Math|Vector|Lerp(Vector) (Variables|Default|GetCurrentLocation) (Math|Vector|MakeVector (.X (Math|Vector|BreakVector (Variables|Default|GetCurrentLocation))) (.Y (Math|Vector|BreakVector (Variables|Default|GetCurrentLocation))) (+ (.Z (Math|Vector|BreakVector (Variables|Default|GetCurrentLocation))) 1e+02)) _newtrack_0))
        (Utilities|FlowControl|Delay 0.5)
        (Class|PrimitiveComponent|SetConstraintMode (Variables|Default|GetMesh) "XYPlane")
        (Utilities|FlowControl|Delay LevitationTime)
        (CallFunction|StopLevitating)))))

(fn ConstructionScript
  (Variables|Default|SetSpawnTransform (Transformation|GetActorTransform)))