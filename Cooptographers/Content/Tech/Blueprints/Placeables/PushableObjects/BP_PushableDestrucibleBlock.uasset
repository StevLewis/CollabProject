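; A destructible pushable block that is replaced at its original placement when destroyed.
; The construction script caches the actor transform, and TriggerDestruction spawns a BP_BasePushableObject there before destroying itself.
; The replacement uses the base pushable class rather than this block's own class.
; Timed destruction, character push start/stop, and visibility, collision and physics toggles remain as unconnected nodes that never run.
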(event Custom|TriggerDestruction
  (Game|SpawnActorfromClass "/Game/Tech/Blueprints/Placeables/PushableObjects/BP_BasePushableObject.BP_BasePushableObject_C" (Variables|Default|GetSpawnTransform) "Undefined" 0 0)
  (Actor|DestroyActor))

(event EventBeginPlay)

(fn ConstructionScript
  (Variables|Default|SetSpawnTransform (Transformation|GetActorTransform)))