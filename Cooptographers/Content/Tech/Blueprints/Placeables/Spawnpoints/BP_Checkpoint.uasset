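; BP_Checkpoint is a placeable checkpoint that updates where the Mage and Scout players respawn.
; On BeginPlay it caches GM_Gameplay; when a BP_BaseCharacter overlaps its box, it sends the world transforms of Player1Spawn and Player2Spawn to that game mode as the new spawn points.
; The construction script sizes the trigger box from the Size variable.
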(event OnComponentBeginOverlap(Box)
  (params (OverlappedComponent :type Primitive%20Component%20Object%20Reference) (OtherActor :type Actor%20Object%20Reference) (OtherComp :type Primitive%20Component%20Object%20Reference) (OtherBodyIndex :type Integer) (bFromSweep :type Boolean) (SweepResult :type Hit%20Result%20Structure%20%28by%20ref%29))
  (Utilities|Casting|CastToBP_BaseCharacter OtherActor)
  (Class|BPIRespawn|SetSpawnPoints(Message) (Variables|Default|GetGamemode) (Transformation|GetWorldTransform (Variables|Default|GetPlayer1Spawn)) (Transformation|GetWorldTransform (Variables|Default|GetPlayer2Spawn))))

(event EventBeginPlay
  (bind _asgm_gameplay (Utilities|Casting|CastToGM_Gameplay (Game|GetGameMode)))
  (Variables|Default|SetGamemode _asgm_gameplay))

(fn ConstructionScript
  (Components|Box|SetBoxExtent (Variables|Default|GetBox) (Variables|Default|GetSize) true))