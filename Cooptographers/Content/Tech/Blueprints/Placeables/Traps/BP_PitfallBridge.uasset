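; BP_PitfallBridge is a placeable trap bridge that swings about a pivot when triggered and back when untriggered.
; Trigger enables bridge collision and plays the Lift timeline, which lerps TurnPoint from its BeginPlay world rotation toward the unset, default zero rotation.
; UnTrigger disables collision immediately and reverses the timeline at double speed, so the bridge stops being solid before it finishes swinging back.
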(event EventBeginPlay
  (Variables|Default|SetStartingRotation (Transformation|GetWorldRotation (Variables|Default|GetTurnPoint))))

(event EventTrigger
  (Collision|SetCollisionEnabled (Variables|Default|GetBridge) "QueryAndPhysics")
  (Components|Timeline|SetPlayRate (Variables|Default|GetLift) 1.0)
  (bind _newtrack_0 (Timeline|Lift Play)
    (:Update
      (Transformation|SetWorldRotation (Variables|Default|GetTurnPoint) (Math|Rotator|Lerp(Rotator) (Variables|Default|GetStartingRotation) "0, 0, 0" _newtrack_0) false false))))

(event EventUnTrigger
  (Collision|SetCollisionEnabled (Variables|Default|GetBridge) "NoCollision")
  (Components|Timeline|SetPlayRate (Variables|Default|GetLift) 2.0)
  (bind _newtrack_0 (Timeline|Lift Reverse)
    (:Update
      (Transformation|SetWorldRotation (Variables|Default|GetTurnPoint) (Math|Rotator|Lerp(Rotator) (Variables|Default|GetStartingRotation) "0, 0, 0" _newtrack_0) false false))))

(fn ConstructionScript
  (|CallParentFunction))