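; BP_RisingBlock is a placeable trap block that moves between its start position and an offset target when triggered and untriggered.
; BeginPlay caches the cube's world location and adds TargetLocation to it as a relative offset for the end point.
; Trigger enables collision and plays the Rise timeline to lerp the cube outward without sweep.
; UnTrigger disables collision and reverses the timeline at a much faster rate.
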(event EventBeginPlay
  (bind _output_get (Variables|Default|SetStartLocation (Transformation|GetWorldLocation (Variables|Default|GetCube))))
  (Variables|Default|SetEndLocation (+ _output_get (Variables|Default|GetTargetLocation))))

(event EventTrigger
  (Collision|SetCollisionEnabled (Variables|Default|GetCube) "QueryAndPhysics")
  (Components|Timeline|SetPlayRate (Variables|Default|GetRise) 1.0)
  (bind _newtrack_0 (Timeline|Rise Play)
    (:Update
      (Transformation|SetWorldLocation (Variables|Default|GetCube) (Math|Vector|Lerp(Vector) (Variables|Default|GetStartLocation) (Variables|Default|GetEndLocation) _newtrack_0) false false))))

(event EventUnTrigger
  (Collision|SetCollisionEnabled (Variables|Default|GetCube) "NoCollision")
  (Components|Timeline|SetPlayRate (Variables|Default|GetRise) 5.0)
  (bind _newtrack_0 (Timeline|Rise Reverse)
    (:Update
      (Transformation|SetWorldLocation (Variables|Default|GetCube) (Math|Vector|Lerp(Vector) (Variables|Default|GetStartLocation) (Variables|Default|GetEndLocation) _newtrack_0) false false))))

(fn ConstructionScript
  (|CallParentFunction))