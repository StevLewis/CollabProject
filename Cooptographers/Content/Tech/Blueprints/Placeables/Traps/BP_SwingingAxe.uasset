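; Swinging axe trap that starts swinging on BeginPlay and damages actors that touch it.
; A timeline lerps the pivot's pitch between configurable start and end points at a set speed, alternating direction after a delay between swings.
; Trigger sets a flag that halts the timeline when a swing next finishes, while UnTrigger does nothing.
; Four boxes apply fixed damage on begin overlap, except Box, which applies it on end overlap.
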(event OnComponentBeginOverlap(Box2)
  (params (OverlappedComponent :type Primitive%20Component%20Object%20Reference) (OtherActor :type Actor%20Object%20Reference) (OtherComp :type Primitive%20Component%20Object%20Reference) (OtherBodyIndex :type Integer) (bFromSweep :type Boolean) (SweepResult :type Hit%20Result%20Structure%20%28by%20ref%29))
  (Game|Damage|ApplyDamage OtherActor 1.0 0 0))

(event OnComponentBeginOverlap(Box3)
  (params (OverlappedComponent :type Primitive%20Component%20Object%20Reference) (OtherActor :type Actor%20Object%20Reference) (OtherComp :type Primitive%20Component%20Object%20Reference) (OtherBodyIndex :type Integer) (bFromSweep :type Boolean) (SweepResult :type Hit%20Result%20Structure%20%28by%20ref%29))
  (Game|Damage|ApplyDamage OtherActor 1.0 0 0))

(event OnComponentEndOverlap(Box)
  (params (OverlappedComponent :type Primitive%20Component%20Object%20Reference) (OtherActor :type Actor%20Object%20Reference) (OtherComp :type Primitive%20Component%20Object%20Reference) (OtherBodyIndex :type Integer))
  (Game|Damage|ApplyDamage OtherActor 1.0 0 0))

(event OnComponentBeginOverlap(Box1)
  (params (OverlappedComponent :type Primitive%20Component%20Object%20Reference) (OtherActor :type Actor%20Object%20Reference) (OtherComp :type Primitive%20Component%20Object%20Reference) (OtherBodyIndex :type Integer) (bFromSweep :type Boolean) (SweepResult :type Hit%20Result%20Structure%20%28by%20ref%29))
  (Game|Damage|ApplyDamage OtherActor 1.0 0 0))

(event EventBeginPlay
  ;[1 1 1] Plays swinging animation for the axe
  (Components|Timeline|SetPlayRate (Variables|Default|GetSwingingAction) (Variables|Default|GetAxeSpeed))
  (bind (_direction _newtrack_0) (Timeline|SwingingAction Play)
    (:Update
      (Transformation|SetRelativeRotation (Variables|Default|GetPivot) (Math|Rotator|Lerp(Rotator) (Math|Rotator|MakeRotator 0.0 (Variables|Default|GetAxeStartingPoint) 0.0) (Math|Rotator|MakeRotator 0.0 (Variables|Default|GetAxeEndPoint) 0.0) _newtrack_0) false false))
    (:Finished
      (if (Variables|Default|GetShouldStop?)
        (Audio|Components|Audio|Stop (Variables|Default|GetSwingingAction))
        (else
          (Utilities|FlowControl|Delay (Variables|Default|GetDelayBetweenSwings))
          (switch Utilities|FlowControl|Switch|SwitchonETimelineDirection _direction
            (:Forward
              (Timeline|SwingingAction Reverse))
            (:Backward
              (Timeline|SwingingAction Play))))))))

(event EventUnTrigger)

(event EventTrigger
  (Variables|Default|SetShouldStop? true))

(fn ConstructionScript
  (|CallParentFunction))