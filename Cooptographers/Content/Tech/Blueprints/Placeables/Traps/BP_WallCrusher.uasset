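; BP_WallCrusher is a placeable trap that slides two walls toward each other and damages actors caught between them.
; Trigger plays a timeline at CrushSpeed to lerp both walls inward, while UnTrigger reverses it at RetractSpeed.
; DeathTrigger starts without collision, is enabled on timeline updates in either direction and applies damage on overlap.
; Nothing switches its collision off again after BeginPlay.
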(event OnComponentBeginOverlap(DeathTrigger)
  (params (OverlappedComponent :type Primitive%20Component%20Object%20Reference) (OtherActor :type Actor%20Object%20Reference) (OtherComp :type Primitive%20Component%20Object%20Reference) (OtherBodyIndex :type Integer) (bFromSweep :type Boolean) (SweepResult :type Hit%20Result%20Structure%20%28by%20ref%29))
  (Game|Damage|ApplyDamage OtherActor 1.0 0 0))

(event EventBeginPlay
  (Collision|SetCollisionEnabled (Variables|Default|GetDeathTrigger) "NoCollision"))

(event EventUnTrigger
  (Components|Timeline|SetPlayRate (Variables|Default|GetTimeline_0) (Variables|Default|GetRetractSpeed))
  (bind (_direction _newtrack_0) (Timeline|Timeline_0 Reverse)
    (:Update
      (Transformation|SetRelativeLocation (Variables|Default|GetWall1) (Math|Vector|Lerp(Vector) "-150.000000,0.000000,50.000000" "-50.000000,0.000000,50.000000" _newtrack_0) false false)
      (Collision|SetCollisionEnabled (Variables|Default|GetDeathTrigger) "QueryAndPhysics")
      (Transformation|SetRelativeLocation (Variables|Default|GetWall2) (Math|Vector|Lerp(Vector) "150.000000,0.000000,50.000000" "50.000000,0.000000,50.000000" _newtrack_0) false false))
    (:Finished
      (switch Utilities|FlowControl|Switch|SwitchonETimelineDirection _direction
        (:Forward
          (Utilities|Time|SetTimerbyEvent (EventDispatchers|CreateEvent :!event UnTrigger) 0.0))))))

(event EventTrigger
  (Components|Timeline|SetPlayRate (Variables|Default|GetTimeline_0) (Variables|Default|GetCrushSpeed))
  (bind (_direction _newtrack_0) (Timeline|Timeline_0 Play)
    (:Update
      (Transformation|SetRelativeLocation (Variables|Default|GetWall1) (Math|Vector|Lerp(Vector) "-150.000000,0.000000,50.000000" "-50.000000,0.000000,50.000000" _newtrack_0) false false)
      (Collision|SetCollisionEnabled (Variables|Default|GetDeathTrigger) "QueryAndPhysics")
      (Transformation|SetRelativeLocation (Variables|Default|GetWall2) (Math|Vector|Lerp(Vector) "150.000000,0.000000,50.000000" "50.000000,0.000000,50.000000" _newtrack_0) false false))
    (:Finished
      (switch Utilities|FlowControl|Switch|SwitchonETimelineDirection _direction
        (:Forward
          (Utilities|Time|SetTimerbyEvent (EventDispatchers|CreateEvent :!event UnTrigger) 0.0))))))

(fn ConstructionScript
  (|CallParentFunction)
  (Components|Timeline|SetPlayRate (Variables|Default|GetTimeline_0) (Variables|Default|GetCrushSpeed)))