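; BP_CrushBlock is a triggerable placeable block that slides between two positions and damages actors that overlap its damage volume.
; Trigger enables mesh collision and plays the Move timeline, lerping BlockMesh without sweep from its construction-time location to TargetLocation.
; Untrigger disables mesh collision and reverses the timeline at five times the speed.
; DamageCollision applies damage on any begin overlap, independent of trigger state.
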(event OnComponentBeginOverlap(DamageCollision)
  (params (OverlappedComponent :type Primitive%20Component%20Object%20Reference) (OtherActor :type Actor%20Object%20Reference) (OtherComp :type Primitive%20Component%20Object%20Reference) (OtherBodyIndex :type Integer) (bFromSweep :type Boolean) (SweepResult :type Hit%20Result%20Structure%20%28by%20ref%29))
  (Game|Damage|ApplyDamage OtherActor 1.0 0 0))

(event EventTrigger
  (Collision|SetCollisionEnabled (Variables|Default|GetBlockMesh) "QueryAndPhysics")
  (Components|Timeline|SetPlayRate (Variables|Default|GetMove) 1.0)
  (bind _newtrack_0 (Timeline|Move Play)
    (:Update
      (Transformation|SetRelativeLocation (Variables|Default|GetBlockMesh) (Math|Vector|Lerp(Vector) (Variables|Default|GetStartLocation) (Variables|Default|GetTargetLocation) _newtrack_0) false false))))

(event EventUntrigger
  (Collision|SetCollisionEnabled (Variables|Default|GetBlockMesh) "NoCollision")
  (Components|Timeline|SetPlayRate (Variables|Default|GetMove) 5.0)
  (bind _newtrack_0 (Timeline|Move Reverse)
    (:Update
      (Transformation|SetRelativeLocation (Variables|Default|GetBlockMesh) (Math|Vector|Lerp(Vector) (Variables|Default|GetStartLocation) (Variables|Default|GetTargetLocation) _newtrack_0) false false))))

(fn ConstructionScript
  (|CallParentFunction)
  (Variables|Default|SetStartLocation (Variables|/Script/Engine.SceneComponent|GetRelativeLocation (Variables|Default|GetBlockMesh))))