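; BP_ExtendableSpike is a triggerable placeable spike that extends and retracts when triggered.
; On trigger, a Move timeline running at SpikeMoveSpeed lerps the spike between the start location captured in the construction script and TargetLocation.
; The timeline reverses after extending and replays after retracting while Loop is set.
; Untrigger clears Loop, letting the current cycle finish before stopping.
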(event EventTrigger
  (Components|Timeline|SetPlayRate (Variables|Default|GetMove) (Variables|Default|GetSpikeMoveSpeed))
  (bind (_direction _newtrack_0) (Timeline|Move Play)
    (:Update
      (Transformation|SetRelativeLocation (Variables|Default|GetSpike) (Math|Vector|Lerp(Vector) (Variables|Default|GetStartLocation) (Variables|Default|GetTargetLocation) _newtrack_0) false false))
    (:Finished
      (switch Utilities|FlowControl|Switch|SwitchonETimelineDirection _direction
        (:Forward
          (Timeline|Move Reverse))
        (:Backward
          (if (Variables|Default|GetLoop?)
            (Timeline|Move Play)))))))

(event EventUntrigger
  (Variables|Default|SetLoop? false))

(fn ConstructionScript
  (|CallParentFunction)
  (Variables|Default|SetStartLocation (Variables|/Script/Engine.SceneComponent|GetRelativeLocation (Variables|Default|GetSpike))))