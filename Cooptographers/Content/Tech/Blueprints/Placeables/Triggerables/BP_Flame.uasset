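; BP_Flame is a placeable triggerable flame hazard that damages actors overlapping its collision.
; Trigger lights the flame after a configurable delay, then a self-repeating timed cycle switches it off and, while Triggered holds, back on.
; Collision is disabled with the flame and re-enabled shortly after each relight within the cycle.
; Overlaps send a typed damage message to the actor, and Untrigger shuts off both flame and collision.
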(event OnComponentBeginOverlap(Collision)
  (params (OverlappedComponent :type Primitive%20Component%20Object%20Reference) (OtherActor :type Actor%20Object%20Reference) (OtherComp :type Primitive%20Component%20Object%20Reference) (OtherBodyIndex :type Integer) (bFromSweep :type Boolean) (SweepResult :type Hit%20Result%20Structure%20%28by%20ref%29))
  (Class|BPIDamage|ApplyDamagebyType(Message) OtherActor (Variables|Default|GetDamage) self "NewEnumerator2"))

(event Custom|Turn%20on/off
  ;[1 1 1] Will cycle between turning the flame on and off
  (Utilities|FlowControl|Delay 2.0)
  (Components|Activation|Deactivate (Variables|Default|GetFlame))
  (Collision|SetCollisionEnabled (Variables|Default|GetCollision) "NoCollision")
  (if (Variables|Default|GetTriggered?)
    (Utilities|FlowControl|Delay 2.0)
    (Components|Activation|Activate (Variables|Default|GetFlame) false)
    (Utilities|FlowControl|Delay 0.2)
    (Collision|SetCollisionEnabled (Variables|Default|GetCollision) "QueryAndPhysics")
    (CallFunction|TurnOn/off)))

(event EventTrigger
  ;[1 1 1] Activates the flame
  (Utilities|FlowControl|Delay (Variables|Default|GetDelay))
  (Components|Activation|Activate (Variables|Default|GetFlame) false)
  (CallFunction|TurnOn/off))

(event EventUntrigger
  ;[1 1 1] Deactivates the flame
  (Components|Activation|Deactivate (Variables|Default|GetFlame))
  (Collision|SetCollisionEnabled (Variables|Default|GetCollision) "NoCollision"))

(fn ConstructionScript
  (|CallParentFunction))