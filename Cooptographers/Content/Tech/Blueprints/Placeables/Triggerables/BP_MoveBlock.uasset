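; BP_MoveBlock is a triggerable placeable that slides a block mesh between its construction-time position and a target location.
; Trigger enables full collision and plays the Move timeline forward, lerping the mesh's relative location from StartLocation to TargetLocation.
; Untrigger disables collision and reverses the timeline at five times the speed, so the block snaps back quickly without blocking anything.
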(event EventTrigger
  (Collision|SetCollisionEnabled (Variables|Default|GetBlockMesh) "QueryAndPhysics")
  (Components|Timeline|SetPlayRate (Variables|Default|GetMove) 1.0)
  (bind _newtrack_0 (Timeline|Move Play)
    (:Update
      (Transformation|SetRelativeLocation (Variables|Default|GetBlockMesh) (Math|Vector|Lerp(Vector) (Variables|Default|GetStartLocation) (Variables|Default|GetTargetLocation) _newtrack_0) false false))))

(event EventUntrigger
  (Collision|SetCollisionEnabled (Variables|Default|GetBlockMesh) "NoCollision")
  (Components|Timeline|SetPlayRate (Variables|Default|GetMove) 5.0)
  (bind _newtrack_0 (Timeline|Move Reverse)
    (:Update
      (Transformation|SetRelativeLocation (Variables|Default|GetBlockMesh) (Math|Vector|Lerp(Vector) (Variables|Default|GetStartLocation) (Variables|Default|GetTargetLocation) _newtrack_0) false false))))

(fn ConstructionScript
  (|CallParentFunction)
  (Variables|Default|SetStartLocation (Variables|/Script/Engine.SceneComponent|GetRelativeLocation (Variables|Default|GetBlockMesh))))