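; BP_SwingingAxe is a triggerable swinging axe trap that damages actors overlapping its damage collision.
; Trigger plays the Swing timeline, which lerps the Pivot's pitch between start and end angles at a play rate set from AxeSpeed at construction.
; Each finished swing waits a delay, then runs in the opposite direction.
; Untrigger sets a stop flag checked when a swing finishes, and Trigger never clears it.
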(event OnComponentBeginOverlap(DamageCollision)
  (params (OverlappedComponent :type Primitive%20Component%20Object%20Reference) (OtherActor :type Actor%20Object%20Reference) (OtherComp :type Primitive%20Component%20Object%20Reference) (OtherBodyIndex :type Integer) (bFromSweep :type Boolean) (SweepResult :type Hit%20Result%20Structure%20%28by%20ref%29))
  (Game|Damage|ApplyDamage OtherActor (Variables|Default|GetDamage) 0 0))

(event EventTrigger
  (bind (_direction _newtrack_0) (Timeline|Swing Play)
    (:Update
      (Transformation|SetRelativeRotation (Variables|Default|GetPivot) (Math|Rotator|Lerp(Rotator) (Math|Rotator|MakeRotator 0.0 (Variables|Default|GetAxeStartingPoint) 0.0) (Math|Rotator|MakeRotator 0.0 (Variables|Default|GetAxeEndPoint) 0.0) _newtrack_0) false false))
    (:Finished
      (if (Variables|Default|GetShouldStop?)
        (Audio|Components|Audio|Stop (Variables|Default|GetSwing))
        (else
          (Utilities|FlowControl|Delay (Variables|Default|GetDelayBetweenSwings))
          (switch Utilities|FlowControl|Switch|SwitchonETimelineDirection _direction
            (:Forward
              (Timeline|Swing Reverse))
            (:Backward
              (Timeline|Swing Play))))))))

(event EventUntrigger
  (Variables|Default|SetShouldStop? true))

(fn ConstructionScript
  (|CallParentFunction)
  (Components|Timeline|SetPlayRate (Variables|Default|GetSwing) (Variables|Default|GetAxeSpeed)))