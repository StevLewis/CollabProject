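; Triggerable placeable that launches boulders, one after another, for as long as it stays triggered.
; Each cycle spawns a BP_Boulder at the Arrow's location and applies a velocity-change impulse to its mesh.
; After a configurable delay it destroys that boulder and recursively spawns the next if still triggered.
; Untrigger only clears the flag, so the current boulder lives out its delay.
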(event Custom|SpawnBoulder
  (Variables|Default|SetTriggered? true)
  (bind _returnvalue (Game|SpawnActorfromClass "/Game/Tech/Blueprints/Placeables/Hazards/BP_Boulder.BP_Boulder_C" (Math|Transform|MakeTransform (Transformation|GetWorldLocation (Variables|Default|GetArrow)) "0, 0, 0" "1,1,1") "AlwaysSpawn" 0 0))
  (Physics|AddImpulse (Variables|/Game/Tech/Blueprints/Placeables/Hazards/BP_Boulder.BP_Boulder_C|GetBoulderMesh _returnvalue) (Variables|Default|GetImpulse) "None" true)
  (Utilities|FlowControl|Delay (Variables|Default|GetDestroyBoulderdelay))
  (Actor|DestroyActor _returnvalue)
  (if (Variables|Default|GetTriggered?)
    (CallFunction|SpawnBoulder)))

(event EventUntrigger
  (Variables|Default|SetTriggered? false))

(event EventTrigger
  (CallFunction|SpawnBoulder))

(fn ConstructionScript
  (|CallParentFunction))