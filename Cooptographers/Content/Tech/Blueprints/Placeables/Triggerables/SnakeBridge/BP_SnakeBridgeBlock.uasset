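; A snake bridge block, a triggerable placeable that travels along the spline of a BP_SnakeBridgePath actor and destroys itself at the end.
; The construction script finds the path, randomises the material colour and calls MoveObject, whose timeline drives position by spline distance with rotation sampled at the start.
; Trigger separately lerps the mesh to a target location before destroying the actor, while Untrigger stops only the spline movement.
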(event Custom|Move%20Object
  (bind _path_ref (Variables|Default|GetPath%20ref))
  (bind _spline (Variables|/Game/Tech/Blueprints/Placeables/Triggerables/SnakeBridge/BP_SnakeBridgePath.BP_SnakeBridgePath_C|GetSpline _path_ref))
  (Components|Timeline|SetPlayRate (Variables|Default|GetMove%20Along) (/ 1.0 (Variables|Default|GetTime%20To%20Complete%20%28In%20Seconds%29))) ; Playrate (disabled for now for testing)
  (bind _newtrack_0 (Timeline|Move%20Along Play)
    (:Update
      (Variables|Default|SetDistance (Math|Float|Lerp 0.0 (Spline|GetSplineLength (Variables|/Game/Tech/Blueprints/Placeables/Triggerables/SnakeBridge/BP_SnakeBridgePath.BP_SnakeBridgePath_C|GetSpline (Variables|Default|GetPath%20ref))) _newtrack_0))
      (Transformation|SetActorTransform (Math|Transform|MakeTransform (Spline|GetLocationatDistanceAlongSpline _spline (Math|Float|Lerp 0.0 (Spline|GetSplineLength (Variables|/Game/Tech/Blueprints/Placeables/Triggerables/SnakeBridge/BP_SnakeBridgePath.BP_SnakeBridgePath_C|GetSpline (Variables|Default|GetPath%20ref))) _newtrack_0) "World") (Spline|GetRotationatDistanceAlongSpline _spline 0.0 "Local") "1,1,1")))
    (:Finished
      (Actor|DestroyActor))))

(event EventTrigger
  ;[1 1 1] When triggered will move to target location and then destroy itself
  (Components|Timeline|SetPlayRate (Variables|Default|GetMove) 1.0)
  (bind _newtrack_0 (Timeline|Move Play)
    (:Update
      (Transformation|SetRelativeLocation (Variables|Default|GetBlockMesh) (Math|Vector|Lerp(Vector) (Variables|Default|GetStartLocation) (Variables|Default|GetTargetLocation) _newtrack_0) false false))
    (:Finished
      (Actor|DestroyActor))))

(event EventUntrigger
  (bind _path_ref (Variables|Default|GetPath%20ref))
  (bind _spline (Variables|/Game/Tech/Blueprints/Placeables/Triggerables/SnakeBridge/BP_SnakeBridgePath.BP_SnakeBridgePath_C|GetSpline _path_ref))
  (bind _newtrack_0 (Timeline|Move%20Along Stop)
    (:Update
      (Variables|Default|SetDistance (Math|Float|Lerp 0.0 (Spline|GetSplineLength (Variables|/Game/Tech/Blueprints/Placeables/Triggerables/SnakeBridge/BP_SnakeBridgePath.BP_SnakeBridgePath_C|GetSpline (Variables|Default|GetPath%20ref))) _newtrack_0))
      (Transformation|SetActorTransform (Math|Transform|MakeTransform (Spline|GetLocationatDistanceAlongSpline _spline (Math|Float|Lerp 0.0 (Spline|GetSplineLength (Variables|/Game/Tech/Blueprints/Placeables/Triggerables/SnakeBridge/BP_SnakeBridgePath.BP_SnakeBridgePath_C|GetSpline (Variables|Default|GetPath%20ref))) _newtrack_0) "World") (Spline|GetRotationatDistanceAlongSpline _spline 0.0 "Local") "1,1,1")))
    (:Finished
      (Actor|DestroyActor))))

(fn ConstructionScript
  (|CallParentFunction)
  (Variables|Default|SetStartLocation (Variables|/Script/Engine.SceneComponent|GetRelativeLocation (Variables|Default|GetBlockMesh)))
  (Rendering|Material|SetVectorParameterValueonMaterials (Variables|Default|GetBlockMesh) "ChangeColour" (Math|Random|RandomUnitVector))
  (bind _returnvalue (Actor|GetActorOfClass "/Game/Tech/Blueprints/Placeables/Triggerables/SnakeBridge/BP_SnakeBridgePath.BP_SnakeBridgePath_C"))
  (Variables|Default|SetPath%20ref _returnvalue)
  (CallFunction|MoveObject))