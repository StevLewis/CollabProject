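; Triggerable snake bridge path that spawns a chain of BP_SnakeBridgeBlock actors, starting automatically on BeginPlay.
; The first Start spawns a block at the spline's location, then SpawnSnake re-calls itself after a delay, filling the Blocks array up to MaximumBlocks.
; Later Start calls run MoveObject on the stored blocks.
; The trigger events are crossed: Trigger untriggers every block, while Untrigger calls Start.
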(event Custom|SpawnSnake
  ;[1 1 1] Spawns enough blocks for the snake based on an editable variable, then adds each block spawned to an array
  (Utilities|FlowControl|Delay (Variables|Default|GetSpawn%20Delay))
  (Math|Float|IncrementFloat (Variables|Default|GetBlocksTriggered)
    (:%20%20
      (if (< (Variables|Default|GetBlocksTriggered) (Variables|Default|GetMaximumBlocks))
        (bind _returnvalue (Game|SpawnActorfromClass "/Game/Tech/Blueprints/Placeables/Triggerables/SnakeBridge/BP_SnakeBridgeBlock.BP_SnakeBridgeBlock_C" (Math|Transform|MakeTransform "0, 0, 0" "0, 0, 0" "1,1,1") "AlwaysSpawn" 0 "0.000000,0.000000,-300.000000" (Variables|Default|GetTime%20to%20Complete%20%28in%20Seconds%29) 0))
        (Utilities|Array|Add (Variables|Default|GetBlocks) _returnvalue)
        (CallFunction|SpawnSnake)
        (else
          (Variables|Default|SetBlocksTriggered 0.0))))))

(event Custom|Start
  (bind _spline (Variables|Default|GetSpline))
  ;[1 1 1] Event trigger, spawns a block at the splines world location
  (if (Variables|Default|GetFirstTrigger?)
    (Variables|Default|SetTriggered? true)
    (Variables|Default|SetFirstTrigger? false)
    (bind _returnvalue (Game|SpawnActorfromClass "/Game/Tech/Blueprints/Placeables/Triggerables/SnakeBridge/BP_SnakeBridgeBlock.BP_SnakeBridgeBlock_C" (Math|Transform|MakeTransform (Transformation|GetWorldLocation _spline) (Variables|/Script/Engine.SceneComponent|GetRelativeRotation _spline) "1,1,1") "AlwaysSpawn" 0 "0.000000,0.000000,-300.000000" (Variables|Default|GetTime%20to%20Complete%20%28in%20Seconds%29) 0))
    (bind _output_get (Variables|Default|SetBlock%20ref _returnvalue)) ; Sets the block ref to\nthe spawned actor
    (Utilities|Array|Add (Variables|Default|GetBlocks) _output_get)
    (CallFunction|SpawnSnake)
    (else
      (for _array_element (Variables|Default|GetBlocks)
        (Default|MoveObject _array_element)))))

(event EventBeginPlay
  ;[1 1 1] Calls trigger
  (CallFunction|Start))

(event EventUntrigger
  (CallFunction|Start))

(event EventTrigger
  (Default|Untrigger (Variables|Default|GetBlocks)))

(fn ConstructionScript)