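; Base placeable trigger that sends trigger and untrigger messages to a list of Triggerables, with optional one-time interaction.
; Interact starts ToggleTransition, which here only marks it in use; separate Trigger and Untrigger events update Activated.
; Connected triggers can be required together for activation, and any active one blocks untriggering.
; Timers handle delays, auto-deactivation and cascades that fire Triggerables one by one.
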(event Custom|Trigger
  ;[1 1 1] Trigger
  (if (Variables|Default|GetSwapTriggerAndUntrigger?)
    (CallFunction|Untrigger)
    (else
      (Variables|Trigger|SetInUse? false)
      (Utilities|FlowControl|Sequence
        (:then_0
          (if (Variables|Untrigger|GetShouldAutoDeactivate?)
            (bind _returnvalue (Utilities|Time|SetTimerbyEvent (EventDispatchers|CreateEvent :!event Custom|Deactivate) (+ (Variables|Trigger|GetTriggerDelay) (Variables|Deactivate|GetDeactivateTime))))
            (Variables|Deactivate|SetDeactivateTH _returnvalue)))
        (:then_1
          (Variables|Trigger|SetActivated? true)
          (if (Variables|Trigger|GetRequireAllTriggers?)
            (bind _allactivated_ (CallFunction|CheckifOtherTriggersActivated?))
            (if _allactivated_
              (if (<= (Variables|Trigger|GetTriggerDelay) 0.0) :!label _label
                (CallFunction|TriggerAllTriggerables)
                (elif (Variables|Trigger|GetCascadeTrigger?)
                  (Variables|Untrigger|SetCurrentTriggerable 0)
                  (bind _returnvalue_2 (Utilities|Time|SetTimerbyEvent (EventDispatchers|CreateEvent :!event TriggerNextTriggerable) (Variables|Trigger|GetTriggerDelay) true))
                  (Variables|Trigger|SetCascadeTriggerTH _returnvalue_2)
                  (else
                    (Utilities|Time|SetTimerbyEvent (EventDispatchers|CreateEvent :!event TriggerAllTriggerables) (Variables|Trigger|GetTriggerDelay))))))
            (else
              (goto _label))))))))

(event Custom|Untrigger
  ;[1 1 1] Untrigger
  (Variables|Trigger|SetInUse? false)
  (if (Variables|Untrigger|GetShouldUntrigger?)
    (if (Variables|Trigger|GetActivated?)
      (Variables|Trigger|SetActivated? false))
    (bind _activated_ (CallFunction|CheckifAnyOtherTriggersActivated?))
    (if (not _activated_)
      (Variables|Trigger|SetActivated? false)
      (if (<= (Variables|Deactivate|GetDeactivateTime) 0.0)
        (CallFunction|UntriggerAllTriggerables :!label _label)
        (elif (Variables|Untrigger|GetShouldAutoDeactivate?)
          (goto _label)
          (else
            (Utilities|Time|SetTimerbyEvent (EventDispatchers|CreateEvent :!event UntriggerAllTriggerables) (Variables|Deactivate|GetDeactivateTime))))))))

(event Custom|ToggleTransition
  (params (Forward? :type Boolean))
  ;[1 1 1] Transition
  (Variables|Trigger|SetInUse? true))

(event Custom|Deactivate
  ;[1 1 1] Deactivate
  (if (Variables|Trigger|GetActivated?)
    (CallFunction|ToggleTransition false)))

(event Custom|ToggleTrigger
  (if (Variables|Trigger|GetActivated?)
    (CallFunction|Untrigger)
    (else
      (CallFunction|Trigger))))

(event EventInteract
  (params (Interactor :type Actor%20Object%20Reference))
  ;[1 1 1] On Interact
  (if (Variables|Trigger|GetOneTimeUse?)
    (if (and (Variables|Trigger|GetOneTimeUse?) (not (Variables|Trigger|GetOneTimeUsed?)))
      (Variables|Trigger|SetOneTimeUsed? true)
      (Variables|Transition|SetInteractable? false)
      (if (not (Variables|Trigger|GetInUse?)) :!label _label
        (CallFunction|ToggleTransition (not (Variables|Trigger|GetActivated?)))))
    (else
      (goto _label))))

(fn ConstructionScript)

(fn CheckOtherTriggers
  (for _array_element (Variables|Trigger|GetConnectedTriggers)
    (if (Variables|BP_BaseTrigger_C|GetActivated? _array_element)
      (return false)))
  (return true))

(fn TriggerTriggerables)

(fn TriggerAllTriggerables
  (for _array_element (Variables|Trigger|GetTriggerables)
    (Class|BPITrigger|Trigger(Message) _array_element)))

(fn TriggerNextTriggerable
  (bind _triggerables (Variables|Trigger|GetTriggerables))
  (bind _currenttriggerable (Variables|Untrigger|GetCurrentTriggerable))
  (bind _output (Utilities|Array|Get(acopy) _triggerables _currenttriggerable))
  (Utilities|IsValid _output
    (:Is%20Valid
      (Class|BPITrigger|Trigger(Message) _output)
      (Math|Integer|IncrementInt (Variables|Untrigger|GetCurrentTriggerable)))
    (:Is%20Not%20Valid
      (Utilities|Time|ClearandInvalidateTimerbyHandle (Variables|Trigger|GetCascadeTriggerTH)))))

(fn UntriggerAllTriggerables
  (for _array_element (Variables|Trigger|GetTriggerables)
    (Class|BPITrigger|Untrigger(Message) _array_element))
  (Utilities|Time|ClearandInvalidateTimerbyHandle (Variables|Deactivate|GetDeactivateTH)))

(fn CheckifOtherTriggersActivated?
  (for _array_element (Variables|Trigger|GetConnectedTriggers)
    (if (not (Variables|BP_BaseTrigger_C|GetActivated? _array_element))
      (return false)))
  (return true))

(fn CheckifAnyOtherTriggersActivated?
  (for _array_element (Variables|Trigger|GetConnectedTriggers)
    (if (Variables|BP_BaseTrigger_C|GetActivated? _array_element)
      (return true)))
  (return false))

(fn GetInteractable?
  (return (Variables|Transition|GetInteractable?)))