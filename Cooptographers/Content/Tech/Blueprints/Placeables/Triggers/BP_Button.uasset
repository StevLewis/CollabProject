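; BP_Button is a placeable trigger that animates a button press and release.
; A timeline lerps the Button component's relative location between two fixed points, playing forward on TriggerTransition and reversing on UntriggerTransition.
; Trigger fires once the press finishes, while Untrigger fires as soon as the release begins.
; Interactable is cleared during either transition and restored only after the release completes.
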(event EventTriggerTransition
  (Variables|Default|SetInTransition? true)
  (Variables|Default|SetInteractable? false)
  (bind (_direction _newtrack_0) (Timeline|ButtonMovement Play)
    (:Update
      (Transformation|SetRelativeLocation (Variables|Default|GetButton) (Math|Vector|Lerp(Vector) "-4.000000,8.000000, 0" "0.000000,-4.000000, 0" _newtrack_0) false false))
    (:Finished
      (Variables|Default|SetInTransition? false)
      (switch Utilities|FlowControl|Switch|SwitchonETimelineDirection _direction
        (:Forward
          (CallFunction|Trigger))
        (:Backward
          (Variables|Default|SetInteractable? true))))))

(event EventUntriggerTransition
  (Variables|Default|SetInTransition? true)
  (Variables|Default|SetInteractable? false)
  (CallFunction|Untrigger)
  (bind (_direction _newtrack_0) (Timeline|ButtonMovement Reverse)
    (:Update
      (Transformation|SetRelativeLocation (Variables|Default|GetButton) (Math|Vector|Lerp(Vector) "-4.000000,8.000000, 0" "0.000000,-4.000000, 0" _newtrack_0) false false))
    (:Finished
      (Variables|Default|SetInTransition? false)
      (switch Utilities|FlowControl|Switch|SwitchonETimelineDirection _direction
        (:Forward
          (CallFunction|Trigger))
        (:Backward
          (Variables|Default|SetInteractable? true))))))

(fn ConstructionScript
  (|CallParentFunction))