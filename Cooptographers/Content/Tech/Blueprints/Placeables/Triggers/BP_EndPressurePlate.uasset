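; BP_EndPressurePlate is a trigger plate that responds only to BP_BaseCharacter pawns whose Class matches its own (Mage or Scout).
; Matching overlaps drive the parent's ToggleTransition and a timeline that lowers or raises the plate.
; Completing the movement calls Trigger and turns the plate yellow, or Untrigger and restores its class colour from the construction script.
; UntriggerAllTriggerables also raises the plate.
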(event OnComponentEndOverlap(Collision)
  (params (OverlappedComponent :type Primitive%20Component%20Object%20Reference) (OtherActor :type Actor%20Object%20Reference) (OtherComp :type Primitive%20Component%20Object%20Reference) (OtherBodyIndex :type Integer))
  (bind _asbp_base_character (Utilities|Casting|CastToBP_BaseCharacter OtherActor))
  (if (Utilities|Enum|Equal(Enum) (Variables|/Game/Tech/Blueprints/Characters/BP_BaseCharacter.BP_BaseCharacter_C|GetClass _asbp_base_character) (Variables|Default|GetClass))
    (CallFunction|ToggleTransition false)))

(event OnComponentBeginOverlap(Collision)
  (params (OverlappedComponent :type Primitive%20Component%20Object%20Reference) (OtherActor :type Actor%20Object%20Reference) (OtherComp :type Primitive%20Component%20Object%20Reference) (OtherBodyIndex :type Integer) (bFromSweep :type Boolean) (SweepResult :type Hit%20Result%20Structure%20%28by%20ref%29))
  (bind _asbp_base_character (Utilities|Casting|CastToBP_BaseCharacter OtherActor))
  (if (Utilities|Enum|Equal(Enum) (Variables|/Game/Tech/Blueprints/Characters/BP_BaseCharacter.BP_BaseCharacter_C|GetClass _asbp_base_character) (Variables|Default|GetClass))
    (CallFunction|ToggleTransition true)))

(event Custom|PlateUp
  (bind _pressureplate (Variables|Default|GetPressurePlate))
  (bind (_direction _newtrack_0) (Timeline|Movement Reverse)
    (:Update
      (Transformation|SetRelativeLocation (Variables|Default|GetPressurePlate) (Math|Vector|Lerp(Vector) "0, 0, 0" "0, 0,-4.000000" _newtrack_0) false false))
    (:Finished
      (switch Utilities|FlowControl|Switch|SwitchonETimelineDirection _direction
        (:Forward
          (CallFunction|Trigger)
          (Rendering|Material|SetMaterial _pressureplate 0 "/Game/Tech/Materials/MI_Yellow.MI_Yellow"))
        (:Backward
          (CallFunction|Untrigger)
          (Rendering|Material|SetMaterial _pressureplate 0 (Variables|Default|GetMaterial)))))))

(event Custom|PlateDown
  (bind _pressureplate (Variables|Default|GetPressurePlate))
  (bind (_direction _newtrack_0) (Timeline|Movement Play)
    (:Update
      (Transformation|SetRelativeLocation (Variables|Default|GetPressurePlate) (Math|Vector|Lerp(Vector) "0, 0, 0" "0, 0,-4.000000" _newtrack_0) false false))
    (:Finished
      (switch Utilities|FlowControl|Switch|SwitchonETimelineDirection _direction
        (:Forward
          (CallFunction|Trigger)
          (Rendering|Material|SetMaterial _pressureplate 0 "/Game/Tech/Materials/MI_Yellow.MI_Yellow"))
        (:Backward
          (CallFunction|Untrigger)
          (Rendering|Material|SetMaterial _pressureplate 0 (Variables|Default|GetMaterial)))))))

(event EventToggleTransition
  (params (Forward? :type Boolean))
  (|CallParentFunction Forward?)
  (if Forward?
    (CallFunction|PlateDown)
    (else
      (CallFunction|PlateUp))))

(fn ConstructionScript
  (|CallParentFunction)
  (Rendering|Material|SetMaterial (Variables|Default|GetPressurePlate) 0 (Utilities|Select :Index (Variables|Default|GetClass) :NewEnumerator2 "/Game/Tech/Materials/M_Base.M_Base" :NewEnumerator1 "/Game/Tech/Materials/MI_Orange.MI_Orange" :NewEnumerator0 "/Game/Tech/Materials/MI_Green.MI_Green"))
  (Variables|Default|SetMaterial (Rendering|Material|GetMaterial (Variables|Default|GetPressurePlate) 0)))

(fn UntriggerAllTriggerables
  (CallFunction|PlateUp)
  (|CallParentFunction))