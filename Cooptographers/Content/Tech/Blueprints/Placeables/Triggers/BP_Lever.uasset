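; BP_Lever is an interactable trigger lever that fires its referenced traps on first activation.
; Interact alternates a timeline forward and in reverse to swing the handle, recording the interacting actor on forward pulls.
; The first pull triggers all traps immediately, or starts a non-looping timer if TrapDelay is positive.
; TriggerTrap steps through TrapRefs by index, though the timer's bound event is not shown.
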(event EventInteract
  (params (Interacting :type Actor%20Object%20Reference))
  (Utilities|FlowControl|FlipFlop
    (:A
      (if (not (Variables|Default|GetTriggered?))
        (if (<= (Variables|Default|GetTrapDelay) 0.0)
          (CallFunction|TriggerAllTraps)
          (else
            (bind _returnvalue (Utilities|Time|SetTimerbyEvent (EventDispatchers|CreateEvent :!event TriggerTrap) (Variables|Default|GetTrapDelay)))
            (Variables|Default|SetTimerDelayTH _returnvalue)))
        (Variables|Default|SetTriggered? true))
      (Utilities|Array|Add (Variables|Default|GetOverlappedActors) Interacting)
      (bind _newtrack_0 (Timeline|ChangeLever Play)
        (:Update
          (Transformation|SetRelativeRotation (Variables|Default|GetScene) (Math|Rotator|Lerp(Rotator) "0.000000,0.000000,40.000000" "0.000000,0.000000,-40.000000" _newtrack_0) false false))))
    (:B
      (Timeline|ChangeLever Reverse))))

(fn ConstructionScript
  (|CallParentFunction))

(fn TriggerAllTraps
  (for _array_element (Variables|Default|GetTrapRefs)
    (Class|BPITrigger|Trigger(Message) _array_element)))

(fn TriggerTrap
  (bind _traprefs (Variables|Default|GetTrapRefs))
  (bind _trapindex (Variables|Default|GetTrapIndex))
  (bind _output (Utilities|Array|Get(acopy) _traprefs _trapindex))
  (Utilities|IsValid _output
    (:Is%20Valid
      (Class|BPITrigger|Trigger(Message) _output)
      (Math|Integer|IncrementInt (Variables|Default|GetTrapIndex)))
    (:Is%20Not%20Valid
      (Utilities|Time|ClearandInvalidateTimerbyHandle (Variables|Default|GetTimerDelayTH)))))