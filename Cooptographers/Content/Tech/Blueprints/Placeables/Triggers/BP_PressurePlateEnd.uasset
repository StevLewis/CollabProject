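; BP_PressurePlateEnd is a placeable pressure plate trigger that responds only to a character of its assigned class, Mage or Scout.
; Overlap by a matching character plays a timeline that lowers the plate, calling Trigger once fully pressed.
; Ending that overlap calls Untrigger immediately and reverses the timeline to raise the plate.
; The construction script colors the plate with a red or green gem material according to the class.
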(event OnComponentBeginOverlap(Collision)
  (params (OverlappedComponent :type Primitive%20Component%20Object%20Reference) (OtherActor :type Actor%20Object%20Reference) (OtherComp :type Primitive%20Component%20Object%20Reference) (OtherBodyIndex :type Integer) (bFromSweep :type Boolean) (SweepResult :type Hit%20Result%20Structure%20%28by%20ref%29))
  (bind _asbp_base_character (Utilities|Casting|CastToBP_BaseCharacter OtherActor))
  (if (Utilities|Enum|Equal(Enum) (Variables|/Game/Tech/Blueprints/Characters/BP_BaseCharacter.BP_BaseCharacter_C|GetClass _asbp_base_character) (Variables|Default|GetClass))
    (CallFunction|TriggerTransition)))

(event OnComponentEndOverlap(Collision)
  (params (OverlappedComponent :type Primitive%20Component%20Object%20Reference) (OtherActor :type Actor%20Object%20Reference) (OtherComp :type Primitive%20Component%20Object%20Reference) (OtherBodyIndex :type Integer))
  (bind _asbp_base_character (Utilities|Casting|CastToBP_BaseCharacter OtherActor))
  (if (Utilities|Enum|Equal(Enum) (Variables|/Game/Tech/Blueprints/Characters/BP_BaseCharacter.BP_BaseCharacter_C|GetClass _asbp_base_character) (Variables|Default|GetClass))
    (CallFunction|UntriggerTransition)))

(event EventTriggerTransition
  (Variables|Default|SetInTransition? true)
  (bind (_direction _newtrack_0) (Timeline|PlateMovement Play)
    (:Update
      (Transformation|SetRelativeLocation (Variables|Default|GetPressurePlate) (Math|Vector|Lerp(Vector) "0.000000,0.000000,3.000000" "0.000000,0.000000,-1.000000" _newtrack_0) false false))
    (:Finished
      (Variables|Default|SetInTransition? false)
      (switch Utilities|FlowControl|Switch|SwitchonETimelineDirection _direction
        (:Forward
          (CallFunction|Trigger))))))

(event EventUntriggerTransition
  (Variables|Default|SetInTransition? true)
  (CallFunction|Untrigger)
  (bind (_direction _newtrack_0) (Timeline|PlateMovement Reverse)
    (:Update
      (Transformation|SetRelativeLocation (Variables|Default|GetPressurePlate) (Math|Vector|Lerp(Vector) "0.000000,0.000000,3.000000" "0.000000,0.000000,-1.000000" _newtrack_0) false false))
    (:Finished
      (Variables|Default|SetInTransition? false)
      (switch Utilities|FlowControl|Switch|SwitchonETimelineDirection _direction
        (:Forward
          (CallFunction|Trigger))))))

(fn ConstructionScript
  (|CallParentFunction)
  (Rendering|Material|SetMaterial (Variables|Default|GetPressurePlate) 0 (Utilities|Select :Index (Variables|Default|GetClass) :NewEnumerator2 0 :NewEnumerator1 "/Game/Art/EnvironmentArt/Materials/MI_GemRed.MI_GemRed" :NewEnumerator0 "/Game/Art/EnvironmentArt/Materials/MI_GemGreen.MI_GemGreen")))