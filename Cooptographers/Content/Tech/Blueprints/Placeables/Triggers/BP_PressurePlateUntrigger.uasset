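; Placeable pressure plate that calls Untrigger once it has been fully pressed down.
; Collision overlaps track occupants, optionally only characters; the first one starts the press, and the last one leaving raises the plate if CanCauseUntrigger is set.
; A timeline lerps the plate's height in both directions, calling Untrigger only when it finishes forward.
; OneTimeUse clears Interactable on the first press.
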(event OnComponentEndOverlap(Collision)
  (params (OverlappedComponent :type Primitive%20Component%20Object%20Reference) (OtherActor :type Actor%20Object%20Reference) (OtherComp :type Primitive%20Component%20Object%20Reference) (OtherBodyIndex :type Integer))
  (if (Variables|Default|GetOnlyByCharacter?)
    (bind _asbp_base_character (Utilities|Casting|CastToBP_BaseCharacter OtherActor))
    (Utilities|Array|RemoveItem (Variables|Default|GetOverlappedActors) _asbp_base_character)
    (else
      (Utilities|Array|RemoveItem (Variables|Default|GetOverlappedActors) OtherActor)))
  (if (not (Utilities|Array|IsValidIndex (Variables|Default|GetOverlappedActors)))
    (if (Variables|Default|GetCanCauseUntrigger?)
      (CallFunction|UntriggerTransition))))

(event OnComponentBeginOverlap(Collision)
  (params (OverlappedComponent :type Primitive%20Component%20Object%20Reference) (OtherActor :type Actor%20Object%20Reference) (OtherComp :type Primitive%20Component%20Object%20Reference) (OtherBodyIndex :type Integer) (bFromSweep :type Boolean) (SweepResult :type Hit%20Result%20Structure%20%28by%20ref%29))
  (if (Variables|Default|GetOnlyByCharacter?)
    (bind _asbp_base_character (Utilities|Casting|CastToBP_BaseCharacter OtherActor))
    (Utilities|Array|Add (Variables|Default|GetOverlappedActors) _asbp_base_character)
    (else
      (Utilities|Array|Add (Variables|Default|GetOverlappedActors) OtherActor)))
  (if (not (Utilities|Array|IsValidIndex (Variables|Default|GetOverlappedActors) 1))
    (if (Variables|Default|GetOneTimeUse?)
      (Utilities|FlowControl|DoOnce false
        (:Completed
          (Variables|Default|SetInteractable? false))))
    (CallFunction|TriggerTransition)))

(event EventTriggerTransition
  (Variables|Default|SetInTransition? true)
  (bind (_direction _newtrack_0) (Timeline|PlateMovement Play)
    (:Update
      (Transformation|SetRelativeLocation (Variables|Default|GetPressurePlate) (Math|Vector|Lerp(Vector) "0.000000,0.000000,3.000000" "0.000000,0.000000,-1.000000" _newtrack_0) false false))
    (:Finished
      (Variables|Default|SetInTransition? false)
      (switch Utilities|FlowControl|Switch|SwitchonETimelineDirection _direction
        (:Forward
          (CallFunction|Untrigger))))))

(event EventUntriggerTransition
  (Variables|Default|SetInTransition? true)
  (bind (_direction _newtrack_0) (Timeline|PlateMovement Reverse)
    (:Update
      (Transformation|SetRelativeLocation (Variables|Default|GetPressurePlate) (Math|Vector|Lerp(Vector) "0.000000,0.000000,3.000000" "0.000000,0.000000,-1.000000" _newtrack_0) false false))
    (:Finished
      (Variables|Default|SetInTransition? false)
      (switch Utilities|FlowControl|Switch|SwitchonETimelineDirection _direction
        (:Forward
          (CallFunction|Untrigger))))))

(fn ConstructionScript
  (|CallParentFunction))