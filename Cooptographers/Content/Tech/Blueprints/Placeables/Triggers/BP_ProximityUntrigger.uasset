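; Placeable proximity trigger that calls Untrigger when an actor enters its Collision volume.
; An OnlyByCharacter flag restricts it to BP_BaseCharacter actors; otherwise any overlapping actor counts.
; Entering actors are tracked in OverlappedActors, and Untrigger fires only while that list holds no second entry.
; Leaving actors are removed from the list without firing anything.
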(event OnComponentEndOverlap(Collision)
  (params (OverlappedComponent :type Primitive%20Component%20Object%20Reference) (OtherActor :type Actor%20Object%20Reference) (OtherComp :type Primitive%20Component%20Object%20Reference) (OtherBodyIndex :type Integer))
  (Utilities|Array|RemoveItem (Variables|Default|GetOverlappedActors) OtherActor))

(event OnComponentBeginOverlap(Collision)
  (params (OverlappedComponent :type Primitive%20Component%20Object%20Reference) (OtherActor :type Actor%20Object%20Reference) (OtherComp :type Primitive%20Component%20Object%20Reference) (OtherBodyIndex :type Integer) (bFromSweep :type Boolean) (SweepResult :type Hit%20Result%20Structure%20%28by%20ref%29))
  (if (Variables|Default|GetOnlyByCharacter?)
    (bind _asbp_base_character (Utilities|Casting|CastToBP_BaseCharacter OtherActor))
    (Utilities|Array|Add (Variables|Default|GetOverlappedActors) _asbp_base_character)
    (else
      (Utilities|Array|Add (Variables|Default|GetOverlappedActors) OtherActor)))
  (if (not (Utilities|Array|IsValidIndex (Variables|Default|GetOverlappedActors) 1))
    (CallFunction|Untrigger)))

(fn ConstructionScript
  (|CallParentFunction))