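; BP_WallLever is a placeable wall lever trigger that swings between two positions with a sound.
; Transition events drive the LeverMovement timeline forward or in reverse to rotate the Lever, blocking interaction until it finishes.
; Trigger fires only when the forward swing completes, while Untrigger fires as soon as the reverse swing starts.
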(event EventTriggerTransition
  (Audio|SpawnSoundAttached "/Game/Tech/Sounds/Cues/SC_Lever.SC_Lever" (Variables|Default|GetDefaultSceneRoot) "None" (Transformation|GetActorLocation) "0, 0, 0" "SnapToTarget" false 1.0 1.0 0.0 "/Game/Tech/Sounds/SA_DefaultAttentuation.SA_DefaultAttentuation" 0)
  (Variables|Default|SetInTransition? true)
  (Variables|Default|SetInteractable? false)
  (bind (_direction _newtrack_0) (Timeline|LeverMovement Play)
    (:Update
      (Transformation|SetRelativeRotation (Variables|Default|GetLever) (Math|Rotator|Lerp(Rotator) "0.000000,0.000000,-50.000000" "0.000000,0.000000,50.000000" _newtrack_0) false false))
    (:Finished
      (Variables|Default|SetInTransition? false)
      (Variables|Default|SetInteractable? true)
      (switch Utilities|FlowControl|Switch|SwitchonETimelineDirection _direction
        (:Forward
          (CallFunction|Trigger))))))

(event EventUntriggerTransition
  (Audio|SpawnSoundAttached "/Game/Tech/Sounds/Cues/SC_Lever.SC_Lever" (Variables|Default|GetDefaultSceneRoot) "None" (Transformation|GetActorLocation) "0, 0, 0" "SnapToTarget" false 1.0 1.0 0.0 "/Game/Tech/Sounds/SA_DefaultAttentuation.SA_DefaultAttentuation" 0)
  (Variables|Default|SetInTransition? true)
  (Variables|Default|SetInteractable? false)
  (CallFunction|Untrigger)
  (bind (_direction _newtrack_0) (Timeline|LeverMovement Reverse)
    (:Update
      (Transformation|SetRelativeRotation (Variables|Default|GetLever) (Math|Rotator|Lerp(Rotator) "0.000000,0.000000,-50.000000" "0.000000,0.000000,50.000000" _newtrack_0) false false))
    (:Finished
      (Variables|Default|SetInTransition? false)
      (Variables|Default|SetInteractable? true)
      (switch Utilities|FlowControl|Switch|SwitchonETimelineDirection _direction
        (:Forward
          (CallFunction|Trigger))))))

(fn ConstructionScript
  (|CallParentFunction))