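; BP_PushableBox is a work-in-progress box meant to be pushed by the player, with configurable mass and linear damping applied on BeginPlay.
; X and Y side triggers show an Info prompt and set one shared Overlapped flag for BP_BaseCharacter, with debug prints.
; Interact alternates PickupBlock and DropBlock through a FlipFlop while overlapped.
; Both functions currently do nothing, as their attach, detach, physics and rotation-lock logic is disconnected.
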(event OnComponentBeginOverlap(YCollision)
  (params (OverlappedComponent :type Primitive%20Component%20Object%20Reference) (OtherActor :type Actor%20Object%20Reference) (OtherComp :type Primitive%20Component%20Object%20Reference) (OtherBodyIndex :type Integer) (bFromSweep :type Boolean) (SweepResult :type Hit%20Result%20Structure%20%28by%20ref%29))
  ;[1 1 1] Makes the block pushable on Y when entering on the Y side of the block
  (Utilities|Casting|CastToBP_BaseCharacter OtherActor)
  (Rendering|SetVisibility (Variables|Default|GetInfo) true false)
  (bind _output_get (Variables|Default|SetOverlapped? true))
  (Development|PrintString "Pushable on Y, Overlapped")
  (Development|PrintString (Utilities|String|ToString(Boolean) _output_get)))

(event OnComponentEndOverlap(YCollision)
  (params (OverlappedComponent :type Primitive%20Component%20Object%20Reference) (OtherActor :type Actor%20Object%20Reference) (OtherComp :type Primitive%20Component%20Object%20Reference) (OtherBodyIndex :type Integer))
  ;[1 1 1] Makes the block pushable on Y when entering on the Y side of the block
  (Utilities|Casting|CastToBP_BaseCharacter OtherActor)
  (Rendering|SetVisibility (Variables|Default|GetInfo) false false)
  (bind _output_get (Variables|Default|SetOverlapped? false))
  (Development|PrintString "No longer pushable on Y, no longer overlapped")
  (Development|PrintString (Utilities|String|ToString(Boolean) _output_get)))

(event OnComponentBeginOverlap(XCollision)
  (params (OverlappedComponent :type Primitive%20Component%20Object%20Reference) (OtherActor :type Actor%20Object%20Reference) (OtherComp :type Primitive%20Component%20Object%20Reference) (OtherBodyIndex :type Integer) (bFromSweep :type Boolean) (SweepResult :type Hit%20Result%20Structure%20%28by%20ref%29))
  ;[1 1 1] Makes the block pushable on X when entering on the X side of the block
  (Utilities|Casting|CastToBP_BaseCharacter OtherActor)
  (Rendering|SetVisibility (Variables|Default|GetInfo) true false)
  (bind _output_get (Variables|Default|SetOverlapped? true))
  (Development|PrintString "Pushable on X, Overlapped")
  (Development|PrintString (Utilities|String|ToString(Boolean) _output_get)))

(event OnComponentEndOverlap(XCollision)
  (params (OverlappedComponent :type Primitive%20Component%20Object%20Reference) (OtherActor :type Actor%20Object%20Reference) (OtherComp :type Primitive%20Component%20Object%20Reference) (OtherBodyIndex :type Integer))
  ;[1 1 1] Makes the block pushable on X when entering on the X side of the block
  (Utilities|Casting|CastToBP_BaseCharacter OtherActor)
  (Rendering|SetVisibility (Variables|Default|GetInfo) false false)
  (bind _output_get (Variables|Default|SetOverlapped? false))
  (Development|PrintString "No longer pushable on X, no longer overlapped")
  (Development|PrintString (Utilities|String|ToString(Boolean) _output_get)))

(event Custom|Init
  (bind _box (Variables|Default|GetBox))
  ;[1 1 1] Init sets the weight and drag of the pushable object
  (Class|PrimitiveComponent|SetMassOverrideinKg _box "None" (Variables|Default|GetMassKG) true)
  (Class|PrimitiveComponent|SetLinearDamping _box (Variables|Default|GetDrag)))

(event EventBeginPlay
  ;[1 1 1] EventBeginPlay call init
  (CallFunction|Init))

(event EventInteract
  (params (Interacting :type Actor%20Object%20Reference))
  ;[1 1 1] WIP
  (if (Variables|Default|GetOverlapped?)
    (Utilities|FlowControl|FlipFlop
      (:A
        (CallFunction|PickupBlock Interacting))
      (:B
        (CallFunction|DropBlock Interacting)))))

(fn ConstructionScript)

(fn PickupBlock
  (params (Object :type Object%20Object%20Reference)))

(fn DropBlock
  (params (Object :type Object%20Object%20Reference)))