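; Pushable box placeable that a character grabs and releases through alternating Interact calls to push or pull it along one axis.
; Two side collision volumes track which axis the player overlaps and toggle the Info prompt.
; Grabbing enables physics, a plane constraint matching that side and the pull boundary collisions, plus a hold message on the interactor; releasing resets these.
; Construction applies mass and drag to the box.
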(event OnComponentBeginOverlap(YCollision)
  (params (OverlappedComponent :type Primitive%20Component%20Object%20Reference) (OtherActor :type Actor%20Object%20Reference) (OtherComp :type Primitive%20Component%20Object%20Reference) (OtherBodyIndex :type Integer) (bFromSweep :type Boolean) (SweepResult :type Hit%20Result%20Structure%20%28by%20ref%29))
  ;[1 1 1] Checks if player is overlapped in Y
  (Utilities|Casting|CastToBP_BaseCharacter OtherActor)
  (Rendering|SetVisibility (Variables|Default|GetInfo) true false)
  (Variables|Default|SetOverlapped%20in%20Y? true))

(event OnComponentEndOverlap(YCollision)
  (params (OverlappedComponent :type Primitive%20Component%20Object%20Reference) (OtherActor :type Actor%20Object%20Reference) (OtherComp :type Primitive%20Component%20Object%20Reference) (OtherBodyIndex :type Integer))
  ;[1 1 1] Checks if player is overlapped in Y
  (Utilities|Casting|CastToBP_BaseCharacter OtherActor)
  (Rendering|SetVisibility (Variables|Default|GetInfo) false false)
  (Variables|Default|SetOverlapped%20in%20Y? false))

(event OnComponentBeginOverlap(XCollision)
  (params (OverlappedComponent :type Primitive%20Component%20Object%20Reference) (OtherActor :type Actor%20Object%20Reference) (OtherComp :type Primitive%20Component%20Object%20Reference) (OtherBodyIndex :type Integer) (bFromSweep :type Boolean) (SweepResult :type Hit%20Result%20Structure%20%28by%20ref%29))
  ;[1 1 1] Checks if player is overlapped in X
  (Utilities|Casting|CastToBP_BaseCharacter OtherActor)
  (Rendering|SetVisibility (Variables|Default|GetInfo) true false)
  (Variables|Default|SetOverlapped%20in%20X? true))

(event OnComponentEndOverlap(XCollision)
  (params (OverlappedComponent :type Primitive%20Component%20Object%20Reference) (OtherActor :type Actor%20Object%20Reference) (OtherComp :type Primitive%20Component%20Object%20Reference) (OtherBodyIndex :type Integer))
  ;[1 1 1] Checks if player is overlapped in X
  (Utilities|Casting|CastToBP_BaseCharacter OtherActor)
  (Rendering|SetVisibility (Variables|Default|GetInfo) false false)
  (Variables|Default|SetOverlapped%20in%20X? false))

(event EventInteract
  (params (Interacting :type Actor%20Object%20Reference))
  ;[1 1 1] Interacting with the block on the X axis or Y axis will make the block pushable and pullable
  (bind _output_get (Variables|Default|SetInteracting Interacting))
  (Development|PrintString (Utilities|GetDisplayName _output_get))
  (Utilities|FlowControl|FlipFlop
    (:A
      (if (Variables|Default|GetOverlapped%20in%20Y?)
        (CallFunction|UpdateState "YZPlane" true true "QueryAndPhysics")
        (elif (Variables|Default|GetOverlapped%20in%20X?)
          (CallFunction|UpdateState "XZPlane" true true "QueryAndPhysics"))))
    (:B
      (if (Variables|Default|GetOverlapped%20in%20Y?)
        (CallFunction|UpdateState "SixDOF" false false "NoCollision" :!label _label)
        (elif (Variables|Default|GetOverlapped%20in%20X?)
          (goto _label))))))

(fn ConstructionScript
  (bind _box (Variables|Default|GetBox))
  (Class|PrimitiveComponent|SetMassOverrideinKg _box "None" (Variables|Default|GetMassKG) true)
  (Class|PrimitiveComponent|SetLinearDamping _box (Variables|Default|GetDrag)))

(fn UpdateState
  (params (ConstraintMode :type EDOFMode%20Enum :default "Default") (Interacted? :type Boolean) (bSimulate :type Boolean) (NewType :type ECollisionEnabled%20Enum :default "NoCollision"))
  (Physics|SetSimulatePhysics (Variables|Default|GetBox) bSimulate)
  (Class|PrimitiveComponent|SetConstraintMode (Variables|Default|GetBox) ConstraintMode)
  (Collision|SetCollisionEnabled (Variables|Default|GetPull%20Boundary) NewType)
  (bind _output_get (Variables|Default|SetInteracted? Interacted?))
  (if _output_get
    (Class|BPIHold|Hold(Message) (Variables|Default|GetInteracting) self)
    (else
      (Class|BPIHold|StopHold(Message) (Variables|Default|GetInteracting)))))