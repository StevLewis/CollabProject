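; Spinning spike hazard that extends spikes from both sides and damages actors that overlap them.
; The construction script feeds SpinningRate into a RotatingMovement component to set the spin.
; On BeginPlay, two timelines start, sliding the left and right scene components outward in opposite directions along local X.
; Overlap events on each side's damage box apply a fixed amount of damage to the overlapping actor.
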(event OnComponentBeginOverlap(LeftDamageBox)
  (params (OverlappedComponent :type Primitive%20Component%20Object%20Reference) (OtherActor :type Actor%20Object%20Reference) (OtherComp :type Primitive%20Component%20Object%20Reference) (OtherBodyIndex :type Integer) (bFromSweep :type Boolean) (SweepResult :type Hit%20Result%20Structure%20%28by%20ref%29))
  (Game|Damage|ApplyDamage OtherActor 1.0 0 0))

(event OnComponentBeginOverlap(RightDamageBox)
  (params (OverlappedComponent :type Primitive%20Component%20Object%20Reference) (OtherActor :type Actor%20Object%20Reference) (OtherComp :type Primitive%20Component%20Object%20Reference) (OtherBodyIndex :type Integer) (bFromSweep :type Boolean) (SweepResult :type Hit%20Result%20Structure%20%28by%20ref%29))
  (Game|Damage|ApplyDamage OtherActor 1.0 0 0))

(event Custom|SetOffRightSpikes
  ;[1 1 1] Makes Right Spikes go off
  (Components|Timeline|SetPlayRate (Variables|Default|GetSetOffRightSpike) 2.0)
  (bind _newtrack_0 (Timeline|SetOffRightSpike Play)
    (:Update
      (Transformation|SetRelativeLocation (Variables|Default|GetRightScene) (Math|Vector|Lerp(Vector) "0, 0, 0" "30.000000,0.000000,0.000000" _newtrack_0) false false))))

(event Custom|SetOffLeftSpikes
  ;[1 1 1] Makes the Left spikes go Off
  (Components|Timeline|SetPlayRate (Variables|Default|GetSetOffLeftSpike) (Variables|Default|GetNew%20Rate))
  (bind _newtrack_0 (Timeline|SetOffLeftSpike Play)
    (:Update
      (Transformation|SetRelativeLocation (Variables|Default|GetLeftScene) (Math|Vector|Lerp(Vector) "0, 0, 0" "-30.000000,0.000000,0.000000" _newtrack_0) false false))))

(event EventBeginPlay
  (CallFunction|SetOffLeftSpikes)
  (CallFunction|SetOffRightSpikes))

(fn ConstructionScript
  (Variables|/Script/Engine.RotatingMovementComponent|SetRotationRate (Variables|Default|GetRotatingMovement) (Math|Rotator|MakeRotator 0.0 0.0 (Variables|Default|GetSpinningRate))))