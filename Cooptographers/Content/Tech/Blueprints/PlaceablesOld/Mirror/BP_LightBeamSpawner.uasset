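; Light beam emitter for mirror placeables that casts a beam as a line trace and notifies reflective actors it hits.
; A looping timer starts at BeginPlay, apparently to repeat the SpawnLine1 trace at short intervals.
; The trace runs forward from the arrow component and passes its hit result to any actor implementing BPI_Reflect through ReflectMessage.
; The only beam visual here is the trace's debug draw.
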(event EventBeginPlay
  (Utilities|Time|SetTimerbyEvent (EventDispatchers|CreateEvent :!event SpawnLine1) 0.1 true))

(fn ConstructionScript)

(fn SpawnLine1
  (bind _arrow (Variables|Default|GetArrow))
  (bind _returnvalue (Transformation|GetWorldLocation _arrow))
  (bind (_outhit _returnvalue_2) (Collision|LineTraceForObjects _returnvalue (+ _returnvalue (* (Math|Vector|GetForwardVector (Variables|Default|GetLightBeamSpawner)) (Variables|Default|GetLine%20Trace%20Length))) (Utilities|Array|MakeArray "ObjectTypeQuery1" "ObjectTypeQuery2" "ObjectTypeQuery3" "ObjectTypeQuery4" "ObjectTypeQuery5" "ObjectTypeQuery6") false (Utilities|Array|MakeArray self) "ForDuration" true "(R=1.000000,G=0.000000,B=0.000000,A=1.000000)" "(R=0.000000,G=1.000000,B=0.000000,A=1.000000)" 0.2))
  (if _returnvalue_2
    (if (Utilities|DoesObjectImplementInterface (.HitActor (Collision|BreakHitResult _outhit)) "/Game/Tech/Blueprints/PlaceablesOld/Mirror/BPI_Reflect.BPI_Reflect_C")
      (Class|BPIReflect|Reflect(Message) (.HitActor (Collision|BreakHitResult _outhit)) _outhit))))