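; A placeable puzzle mirror that redirects a line-trace beam and turns in 90-degree yaw steps when triggered.
; Reflect checks which of two box colliders was hit and starts a short timer, unless one is already active.
; SpawnLine and SpawnLineReverse trace from either arrow, shown as debug lines, and pass hits to BPI_Reflect actors, so mirrors can chain.
; Trigger plays a timeline that lerps the rotation, then sets the next target.
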(event EventReflect
  (params (ActorHit :type Hit%20Result%20Structure))
  (bind _hitcomponent (Collision|BreakHitResult ActorHit))
  ;[1 1 1] Checks which collision is hit and spawns a line at the right angle based on that
  (if (== _hitcomponent (Variables|Default|GetArrow%201%20Box%20Collision))
    (if (not (Utilities|Time|IsTimerActivebyHandle (Variables|Default|GetBeamTH)))
      (bind _returnvalue (Utilities|Time|SetTimerbyEvent (EventDispatchers|CreateEvent :!event SpawnLine) 0.1))
      (Variables|Default|SetBeamTH _returnvalue))
    (elif (== _hitcomponent (Variables|Default|GetArrow%20Box%20Collision))
      (if (not (Utilities|Time|IsTimerActivebyHandle (Variables|Default|GetBeamTH)))
        (bind _returnvalue_2 (Utilities|Time|SetTimerbyEvent (EventDispatchers|CreateEvent :!event SpawnLineReverse) 0.1))
        (Variables|Default|SetBeamTH _returnvalue_2)))))

(event EventTrigger
  (bind _newtrack_0 (Timeline|Rotate%20Mirror PlayFromStart)
    (:Update
      (Transformation|SetWorldRotation (Variables|Default|GetScene) (Math|Rotator|Lerp(Rotator) (Variables|Default|GetStart%20Rotation) (Variables|Default|GetTarget%20Rotation) _newtrack_0) false false))
    (:Finished
      (Variables|Default|SetStart%20Rotation (Transformation|GetWorldRotation (Variables|Default|GetScene)))
      (if (> (+ (.yaw (Variables|Default|GetTarget%20Rotation)) 9e+01) 3.6e+02)
        (Variables|Default|SetStart%20Rotation "0, 0, 0")
        (Variables|Default|SetTarget%20Rotation "0,90.000000, 0")
        (else
          (Variables|Default|SetTarget%20Rotation (Math|Rotator|MakeRotator 0.0 0.0 (+ (.yaw (Variables|Default|GetTarget%20Rotation)) 9e+01))))))))

(fn ConstructionScript
  (if (Variables|Default|GetIsRotatable?)
    (Transformation|SetWorldRotation (Variables|Default|GetScene) "0,0.000000, 0" false false)
    (Variables|Default|SetStart%20Rotation (Transformation|GetWorldRotation (Variables|Default|GetScene)))))

(fn SpawnLine
  (bind _arrow (Variables|Default|GetArrow))
  (bind _returnvalue (Transformation|GetWorldLocation _arrow))
  (bind (_outhit _returnvalue_2) (Collision|LineTraceForObjects _returnvalue (+ _returnvalue (* (Math|Vector|GetForwardVector _arrow) (Variables|Default|GetLine%20Trace%20Length))) (Utilities|Array|MakeArray "ObjectTypeQuery1" "ObjectTypeQuery2" "ObjectTypeQuery3" "ObjectTypeQuery4" "ObjectTypeQuery5" "ObjectTypeQuery6") false (Utilities|Array|MakeArray self) "ForDuration" true "(R=1.000000,G=0.000000,B=0.000000,A=1.000000)" "(R=0.000000,G=1.000000,B=0.000000,A=1.000000)" 0.2))
  (if _returnvalue_2
    (if (Utilities|DoesObjectImplementInterface (.HitActor (Collision|BreakHitResult _outhit)) "/Game/Tech/Blueprints/PlaceablesOld/Mirror/BPI_Reflect.BPI_Reflect_C")
      (Class|BPIReflect|Reflect(Message) (.HitActor (Collision|BreakHitResult _outhit)) _outhit))))

(fn SpawnLineReverse
  (bind _arrow1 (Variables|Default|GetArrow1))
  (bind _returnvalue (Transformation|GetWorldLocation _arrow1))
  (bind (_outhit _returnvalue_2) (Collision|LineTraceForObjects _returnvalue (+ _returnvalue (* (Math|Vector|GetForwardVector _arrow1) (Variables|Default|GetLine%20Trace%20Length))) (Utilities|Array|MakeArray "ObjectTypeQuery1" "ObjectTypeQuery2" "ObjectTypeQuery3" "ObjectTypeQuery4" "ObjectTypeQuery5" "ObjectTypeQuery6") false (Utilities|Array|MakeArray self) "ForDuration" true "(R=1.000000,G=0.000000,B=0.000000,A=1.000000)" "(R=0.000000,G=1.000000,B=0.000000,A=1.000000)" 0.2))
  (if _returnvalue_2
    (if (Utilities|DoesObjectImplementInterface (.HitActor (Collision|BreakHitResult _outhit)) "/Game/Tech/Blueprints/PlaceablesOld/Mirror/BPI_Reflect.BPI_Reflect_C")
      (Class|BPIReflect|Reflect(Message) (.HitActor (Collision|BreakHitResult _outhit)) _outhit))))