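; BP_SpikeTrap is a placeable trap whose spike rises after a delay when triggered and damages what it hits.
; An overlap on SpikeTrigger calls Trigger if Triggerable is set, and a timeline lerps the spike's relative height at a configurable speed.
; When fully raised, a timer starts for the retract delay, and UnTrigger reverses the timeline at its own speed.
; A separate Box overlap applies damage independently of the spike's state.
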(event OnComponentBeginOverlap(SpikeTrigger)
  (params (OverlappedComponent :type Primitive%20Component%20Object%20Reference) (OtherActor :type Actor%20Object%20Reference) (OtherComp :type Primitive%20Component%20Object%20Reference) (OtherBodyIndex :type Integer) (bFromSweep :type Boolean) (SweepResult :type Hit%20Result%20Structure%20%28by%20ref%29))
  (if (Variables|Default|GetTriggerable?)
    (if (!= OtherActor self)
      (CallFunction|Trigger))))

(event OnComponentBeginOverlap(Box)
  (params (OverlappedComponent :type Primitive%20Component%20Object%20Reference) (OtherActor :type Actor%20Object%20Reference) (OtherComp :type Primitive%20Component%20Object%20Reference) (OtherBodyIndex :type Integer) (bFromSweep :type Boolean) (SweepResult :type Hit%20Result%20Structure%20%28by%20ref%29))
  (Game|Damage|ApplyDamage OtherActor 1.0 0 0))

(event EventTrigger
  (Components|Timeline|SetPlayRate (Variables|Default|GetSpikeGoUp) (Variables|Default|GetSpikeGoUpSpeed))
  (Utilities|FlowControl|Delay (Variables|Default|GetDelay))
  (bind (_direction _newtrack_0) (Timeline|SpikeGoUp PlayFromStart)
    (:Update
      (Transformation|SetRelativeLocation (Variables|Default|GetSpike) (Math|Vector|Lerp(Vector) "0, 0,-100.000000" "0.000000,0.000000,100.000000" _newtrack_0) false false))
    (:Finished
      (switch Utilities|FlowControl|Switch|SwitchonETimelineDirection _direction
        (:Forward
          (Utilities|Time|SetTimerbyEvent (EventDispatchers|CreateEvent :!event UnTrigger) (Variables|Default|GetRetractDelay)))))))

(event EventUnTrigger
  (Components|Timeline|SetPlayRate (Variables|Default|GetSpikeGoUp) (Variables|Default|GetSpikeGoDownSpeed))
  (bind (_direction _newtrack_0) (Timeline|SpikeGoUp Reverse)
    (:Update
      (Transformation|SetRelativeLocation (Variables|Default|GetSpike) (Math|Vector|Lerp(Vector) "0, 0,-100.000000" "0.000000,0.000000,100.000000" _newtrack_0) false false))
    (:Finished
      (switch Utilities|FlowControl|Switch|SwitchonETimelineDirection _direction
        (:Forward
          (Utilities|Time|SetTimerbyEvent (EventDispatchers|CreateEvent :!event UnTrigger) (Variables|Default|GetRetractDelay)))))))

(fn ConstructionScript
  (|CallParentFunction))