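; BP_CharacterSwitcher is a pressure plate trigger that requests a character switch when both the Mage and Scout stand on it.
; Box overlaps maintain an actor list, which CharactersCheck scans for both character classes.
; A timeline lowers or raises the plate, then on finishing sets it green or blue.
; If both characters are still present then, it calls SwitchCharactersMessage on the game mode.
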(event OnComponentBeginOverlap(Box)
  (params (OverlappedComponent :type Primitive%20Component%20Object%20Reference) (OtherActor :type Actor%20Object%20Reference) (OtherComp :type Primitive%20Component%20Object%20Reference) (OtherBodyIndex :type Integer) (bFromSweep :type Boolean) (SweepResult :type Hit%20Result%20Structure%20%28by%20ref%29))
  (bind _pressureplate (Variables|Default|GetPressurePlate))
  (Utilities|Array|Add (Variables|Default|GetOverlappedActors_0) OtherActor)
  (CallFunction|CharactersCheck)
  (if (Variables|Default|GetCharactersOn?)
    (Variables|Default|SetPlateDown? true)
    (bind _newtrack_0 (Timeline|PlateGoesUp Play)
      (:Update
        (Transformation|SetRelativeLocation (Variables|Default|GetPressurePlate) (Math|Vector|Lerp(Vector) "0, 0,10.000000" "0, 0,1.000000" _newtrack_0) false false))
      (:Finished
        (Utilities|FlowControl|Sequence
          (:then_0
            (if (Variables|Default|GetPlateDown?)
              (Rendering|Material|SetMaterial _pressureplate 0 "/Game/Tech/Materials/MI_Green.MI_Green")
              (else
                (Rendering|Material|SetMaterial _pressureplate 0 "/Game/Tech/Materials/MI_Blue.MI_Blue"))))
          (:then_1
            (if (Variables|Default|GetCharactersOn?)
              (Class|BPISwitch|SwitchCharacters(Message) (Game|GetGameMode)))))))
    (else
      (Variables|Default|SetPlateDown? false)
      (Timeline|PlateGoesUp Reverse))))

(event OnComponentEndOverlap(Box)
  (params (OverlappedComponent :type Primitive%20Component%20Object%20Reference) (OtherActor :type Actor%20Object%20Reference) (OtherComp :type Primitive%20Component%20Object%20Reference) (OtherBodyIndex :type Integer))
  (bind _pressureplate (Variables|Default|GetPressurePlate))
  (Utilities|Array|RemoveItem (Variables|Default|GetOverlappedActors_0) OtherActor)
  (CallFunction|CharactersCheck)
  (if (Variables|Default|GetCharactersOn?)
    (Variables|Default|SetPlateDown? true)
    (bind _newtrack_0 (Timeline|PlateGoesUp Play)
      (:Update
        (Transformation|SetRelativeLocation (Variables|Default|GetPressurePlate) (Math|Vector|Lerp(Vector) "0, 0,10.000000" "0, 0,1.000000" _newtrack_0) false false))
      (:Finished
        (Utilities|FlowControl|Sequence
          (:then_0
            (if (Variables|Default|GetPlateDown?)
              (Rendering|Material|SetMaterial _pressureplate 0 "/Game/Tech/Materials/MI_Green.MI_Green")
              (else
                (Rendering|Material|SetMaterial _pressureplate 0 "/Game/Tech/Materials/MI_Blue.MI_Blue"))))
          (:then_1
            (if (Variables|Default|GetCharactersOn?)
              (Class|BPISwitch|SwitchCharacters(Message) (Game|GetGameMode)))))))
    (else
      (Variables|Default|SetPlateDown? false)
      (Timeline|PlateGoesUp Reverse))))

(fn ConstructionScript
  (|CallParentFunction))

(fn CharactersCheck
  (Variables|Default|SetCharactersOn? false)
  (bind _array_element (Utilities|Array|ForEachLoopwithBreak (Variables|Default|GetOverlappedActors_0) :!label _label)
    (:LoopBody
      (if (== (Utilities|GetClass _array_element) "/Game/Tech/Blueprints/Characters/BP_Mage.BP_Mage_C")
        (Variables|Default|SetCharactersOn? true)
        (goto _label Break)))
    (:Completed
      (if (Variables|Default|GetCharactersOn?)
        (Variables|Default|SetCharactersOn? false)
        (bind _array_element_2 (Utilities|Array|ForEachLoopwithBreak (Variables|Default|GetOverlappedActors_0) :!label _label_2)
          (:LoopBody
            (if (== (Utilities|GetClass _array_element_2) "/Game/Tech/Blueprints/Characters/BP_Scout.BP_Scout_C")
              (Variables|Default|SetCharactersOn? true)
              (goto _label_2 Break))))))))