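; BP_InvisibleTrigger is a box trigger volume that activates and deactivates the traps it references.
; The first overlap sends TriggerMessage to every trap in TrapRefs and sets a Triggered flag, while each overlapping actor is tracked in an array.
; When an overlap ends, it sends UnTriggerMessage and clears the flag only if its array and that of a valid paired OtherTrigger hold no valid first actor.
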(event OnComponentBeginOverlap(Box)
  (params (OverlappedComponent :type Primitive%20Component%20Object%20Reference) (OtherActor :type Actor%20Object%20Reference) (OtherComp :type Primitive%20Component%20Object%20Reference) (OtherBodyIndex :type Integer) (bFromSweep :type Boolean) (SweepResult :type Hit%20Result%20Structure%20%28by%20ref%29))
  (if (not (Variables|Default|GetTriggered?))
    (for _array_element (Variables|Default|GetTrapRefs)
      (Class|BPITrigger|Trigger(Message) _array_element))
    (Variables|Default|SetTriggered? true))
  (Utilities|Array|Add (Variables|Default|GetOverlappedActors) OtherActor))

(event OnComponentEndOverlap(Box)
  (params (OverlappedComponent :type Primitive%20Component%20Object%20Reference) (OtherActor :type Actor%20Object%20Reference) (OtherComp :type Primitive%20Component%20Object%20Reference) (OtherBodyIndex :type Integer))
  (bind _othertrigger (Variables|Default|GetOtherTrigger))
  (Utilities|Array|RemoveItem (Variables|Default|GetOverlappedActors) OtherActor)
  (Utilities|IsValid (Utilities|Array|Get(acopy) (Variables|Default|GetOverlappedActors))
    (:Is%20Not%20Valid
      (Utilities|IsValid _othertrigger
        (:Is%20Valid
          (Utilities|IsValid (Utilities|Array|Get(acopy) (Variables|BP_InvisibleTrigger_C|GetOverlappedActors_0 _othertrigger))
            (:Is%20Not%20Valid
              (for _array_element (Variables|Default|GetTrapRefs)
                (Class|BPITrigger|UnTrigger(Message) _array_element))
              (Variables|Default|SetTriggered? false))))))))

(fn ConstructionScript
  (|CallParentFunction))