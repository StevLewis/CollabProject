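; BP_Lever is a lever trigger meant to fire linked traps via TriggerMessage, but its Interact event is empty and the main lever logic is disconnected.
; That unused FlipFlop logic fires all traps once, immediately or through a delay timer, and swings the lever with a timeline that reverses on alternate calls.
; Helper functions trigger every referenced trap at once or step through them by index, clearing the timer when none remains valid.
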(event EventInteract
  (params (Interactor :type Actor%20Object%20Reference)))

(fn ConstructionScript
  (|CallParentFunction))

(fn TriggerAllTraps
  (for _array_element (Variables|Default|GetTrapRefs)
    (Class|BPITrigger|Trigger(Message) _array_element)))

(fn TriggerTrap
  (bind _traprefs (Variables|Default|GetTrapRefs))
  (bind _trapindex (Variables|Default|GetTrapIndex))
  (bind _output (Utilities|Array|Get(acopy) _traprefs _trapindex))
  (Utilities|IsValid _output
    (:Is%20Valid
      (Class|BPITrigger|Trigger(Message) _output)
      (Math|Integer|IncrementInt (Variables|Default|GetTrapIndex)))
    (:Is%20Not%20Valid
      (Utilities|Time|ClearandInvalidateTimerbyHandle (Variables|Default|GetTimerDelayTH)))))