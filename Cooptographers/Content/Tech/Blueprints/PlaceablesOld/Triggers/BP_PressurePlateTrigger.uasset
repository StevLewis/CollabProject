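; Pressure plate that triggers linked traps when an actor overlaps its box.
; Traps receive trigger messages all at once, or sequentially on a looping timer when a delay is set.
; A timeline moves the plate and swaps its material between green and blue.
; When the last actor leaves, traps untrigger and the timer clears if linked triggers are empty, or immediately upon finding an invalid trigger reference.
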(event OnComponentBeginOverlap(Box)
  (params (OverlappedComponent :type Primitive%20Component%20Object%20Reference) (OtherActor :type Actor%20Object%20Reference) (OtherComp :type Primitive%20Component%20Object%20Reference) (OtherBodyIndex :type Integer) (bFromSweep :type Boolean) (SweepResult :type Hit%20Result%20Structure%20%28by%20ref%29))
  (bind _pressureplate (Variables|Default|GetPressurePlate))
  (if (not (Variables|Default|GetTriggered?))
    (if (<= (Variables|Default|GetTrapDelay) 0.0)
      (CallFunction|TriggerAllTraps)
      (else
        (bind _returnvalue (Utilities|Time|SetTimerbyEvent (EventDispatchers|CreateEvent :!event TriggerTrap) (Variables|Default|GetTrapDelay) true))
        (Variables|Default|SetTimerDelayTH _returnvalue)))
    (Variables|Default|SetTriggered? true))
  (Utilities|Array|Add (Variables|Default|GetOverlappedActors) OtherActor)
  (Variables|Default|SetPlateDown? true)
  (bind _newtrack_0 (Timeline|PlateGoesUp Play)
    (:Update
      (Transformation|SetRelativeLocation (Variables|Default|GetPressurePlate) (Math|Vector|Lerp(Vector) "0, 0,10.000000" "0, 0,1.000000" _newtrack_0) false false))
    (:Finished
      (if (Variables|Default|GetPlateDown?)
        (Rendering|Material|SetMaterial _pressureplate 0 "/Game/Tech/Materials/MI_Green.MI_Green")
        (else
          (Rendering|Material|SetMaterial _pressureplate 0 "/Game/Tech/Materials/MI_Blue.MI_Blue"))))))

(event OnComponentEndOverlap(Box)
  (params (OverlappedComponent :type Primitive%20Component%20Object%20Reference) (OtherActor :type Actor%20Object%20Reference) (OtherComp :type Primitive%20Component%20Object%20Reference) (OtherBodyIndex :type Integer))
  (bind _pressureplate (Variables|Default|GetPressurePlate))
  (Utilities|Array|RemoveItem (Variables|Default|GetOverlappedActors) OtherActor)
  (Utilities|IsValid (Utilities|Array|Get(acopy) (Variables|Default|GetOverlappedActors))
    (:Is%20Not%20Valid
      (Utilities|FlowControl|Sequence
        (:then_0
          (Variables|Default|SetPlateDown? false)
          (bind _newtrack_0 (Timeline|PlateGoesUp Reverse)
            (:Update
              (Transformation|SetRelativeLocation (Variables|Default|GetPressurePlate) (Math|Vector|Lerp(Vector) "0, 0,10.000000" "0, 0,1.000000" _newtrack_0) false false))
            (:Finished
              (if (Variables|Default|GetPlateDown?)
                (Rendering|Material|SetMaterial _pressureplate 0 "/Game/Tech/Materials/MI_Green.MI_Green")
                (else
                  (Rendering|Material|SetMaterial _pressureplate 0 "/Game/Tech/Materials/MI_Blue.MI_Blue"))))))
        (:then_1
          (Variables|Default|SetShouldUntrigger? true)
          (bind _array_element (Utilities|Array|ForEachLoopwithBreak (Variables|Default|GetOtherTriggerRefs) :!label _label)
            (:LoopBody
              (Utilities|IsValid _array_element
                (:Is%20Valid
                  (Utilities|IsValid (Utilities|Array|Get(acopy) (Variables|/Game/Tech/Blueprints/PlaceablesOld/Triggers/BP_BaseTrigger.BP_BaseTrigger_C|GetOverlappedActors _array_element))
                    (:Is%20Valid
                      (Variables|Default|SetShouldUntrigger? false)
                      (goto _label Break))
                    (:Is%20Not%20Valid
                      (Variables|Default|SetShouldUntrigger? true))))
                (:Is%20Not%20Valid
                  (for _array_element_2 (Variables|Default|GetTrapRefs) :!label _label_2
                    (Class|BPITrigger|UnTrigger(Message) _array_element_2))
                  (Variables|Default|SetTriggered? false)
                  (Variables|Default|SetTrapIndex 0)
                  (Utilities|Time|ClearandInvalidateTimerbyHandle (Variables|Default|GetTimerDelayTH)))))
            (:Completed
              (if (Variables|Default|GetShouldUntrigger?)
                (goto _label_2)))))))))

(fn ConstructionScript
  (|CallParentFunction))

(fn TriggerTrap
  (bind _traprefs (Variables|Default|GetTrapRefs))
  (bind _trapindex (Variables|Default|GetTrapIndex))
  (bind _output (Utilities|Array|Get(acopy) _traprefs _trapindex))
  (Utilities|IsValid _output
    (:Is%20Valid
      (Class|BPITrigger|Trigger(Message) _output)
      (Math|Integer|IncrementInt (Variables|Default|GetTrapIndex)))
    (:Is%20Not%20Valid
      (Utilities|Time|ClearandInvalidateTimerbyHandle (Variables|Default|GetTimerDelayTH)))))

(fn TriggerAllTraps
  (for _array_element (Variables|Default|GetTrapRefs)
    (Class|BPITrigger|Trigger(Message) _array_element)))