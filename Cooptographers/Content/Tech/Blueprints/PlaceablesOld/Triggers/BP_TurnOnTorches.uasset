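; BP_TurnOnTorches is a placeable trigger box that turns on a series of referenced torches one at a time.
; The first character overlap starts a looping timer, guarded by DoOnce, at the TorchDelay interval.
; TriggerTorches messages the torch at the current index and increments it, clearing the timer at the first invalid reference.
; The construction script sizes the collision box from the Size variable.
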(event OnComponentBeginOverlap(Collision)
  (params (OverlappedComponent :type Primitive%20Component%20Object%20Reference) (OtherActor :type Actor%20Object%20Reference) (OtherComp :type Primitive%20Component%20Object%20Reference) (OtherBodyIndex :type Integer) (bFromSweep :type Boolean) (SweepResult :type Hit%20Result%20Structure%20%28by%20ref%29))
  ;[1 1 1] When player enters the collision, will trigger the torches 1 at a time
  (Utilities|Casting|CastToBP_BaseCharacter OtherActor)
  (Utilities|FlowControl|DoOnce false
    (:Completed
      (bind _returnvalue (Utilities|Time|SetTimerbyEvent (EventDispatchers|CreateEvent :!event TriggerTorches) (Variables|Default|GetTorchDelay) true))
      (Variables|Default|SetTimerDelayTH _returnvalue))))

(fn ConstructionScript
  (|CallParentFunction)
  (Components|Box|SetBoxExtent (Variables|Default|GetCollision) (Variables|Default|GetSize) true))

(fn TriggerTorches
  (bind _torchrefs (Variables|Default|GetTorchRefs))
  (bind _trapindex (Variables|Default|GetTrapIndex))
  (bind _output (Utilities|Array|Get(acopy) _torchrefs _trapindex))
  (Utilities|IsValid _output
    (:Is%20Valid
      (Class|BPITrigger|Trigger(Message) _output)
      (Math|Integer|IncrementInt (Variables|Default|GetTrapIndex)))
    (:Is%20Not%20Valid
      (Utilities|Time|ClearandInvalidateTimerbyHandle (Variables|Default|GetTimerDelayTH)))))